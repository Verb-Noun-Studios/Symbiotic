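; GM_Generator4 is a generator Blueprint, apparently a game mode, that starts level streaming and switches the music near the final streamed level.
; BeginPlay calls LevelStreamBase and plays the gameplay score in 2D.
; Each Tick runs custom culling and checks the player's distance to the last entry in Levels.
; Within range, a DoOnce stops that score and plays the boss fight score at that level's location with Boss attenuation.
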(event EventBeginPlay
  (|CallParentFunction)
  (CallFunction|LevelStreamBase 1)
  (bind _returnvalue (Audio|SpawnSound2D "/Game/Audio/Score_Gameplay.Score_Gameplay" 1.0 1.0 0.0 0))
  (Variables|Default|SetAudio _returnvalue))

(event EventTick
  (params (DeltaSeconds :type Float%20%28single-precision%29))
  (bind _levels (Variables|Default|GetLevels))
  (bind _returnvalue (Utilities|Array|LastIndex _levels))
  (bind _output (Utilities|Array|Get(acopy) _levels _returnvalue))
  (bind _leveltransform (Variables|/Script/Engine.LevelStreaming|GetLevelTransform _output))
  (|CallParentFunction DeltaSeconds)
  (CallFunction|CustCulling)
  (if (< (Math|Vector|Distance(Vector) (.location (Transformation|GetActorTransform (Game|Player|GetPlayerPawn 0))) (.location _leveltransform)) 8e+03)
    (Utilities|FlowControl|DoOnce false
      (:Completed
        (Audio|Components|Audio|Stop (Variables|Default|GetAudio))
        (bind _returnvalue_2 (Audio|SpawnSoundatLocation "/Game/Audio/Score_Boss_Fight__1_.Score_Boss_Fight__1_" (.location _leveltransform) "0, 0, 0" 1.0 1.0 0.0 "/Game/Audio/Boss.Boss" 0))
        (Variables|Default|SetAudio _returnvalue_2)))))

(fn ConstructionScript
  (|CallParentFunction))