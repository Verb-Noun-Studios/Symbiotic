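; First-person player Blueprint that creates the HUD, handles pausing and interacts with beacons through a camera trace.
; Tick mirrors ammo and firing state from the Gun child actor, adds shake and rotation while firing, clamps camera pitch, and traces the ground below.
; The settings GameInstance supplies sensitivity and a left-hand toggle that selects controls and the interact key.
; Zero health or the Home key opens the 3D menu map.
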(event Custom|LockCamera
  (bind _firstpersoncameracomponent (Variables|Default|GetFirstPersonCameraComponent))
  (bind _returnvalue (Transformation|GetWorldRotation _firstpersoncameracomponent))
  (bind (_roll _pitch _yaw) (Math|Rotator|BreakRotator _returnvalue))
  (Transformation|SetWorldRotation _firstpersoncameracomponent (Math|Rotator|MakeRotator (Math|Float|Clamp(Float) _roll 0.0 0.0) (Math|Float|Clamp(Float) _pitch -5e+01 6e+01) _yaw) false false))

(event EventBeginPlay
  (bind _aswbp_settings_controller (Utilities|Casting|CastToWBP_SettingsController (Game|GetGameInstance)))
  (Class|FragPlayer|UpdateControls (not (Variables|/Game/Widgets/3D_Menu/WBP_SettingsController.WBP_SettingsController_C|GetLeftHandToggle _aswbp_settings_controller)))
  (CallFunction|SetGunValues)
  (Actor|Tick|SetActorTickEnabled true)
  ;[1 1 1] Set Player HUD Widget
  (bind _returnvalue (UserInterface|CreateWidget "/Game/Widgets/WBP_PlayerHud.WBP_PlayerHud_C" (Game|GetPlayerController 0)))
  (UserInterface|Viewport|AddtoViewport _returnvalue 0))

(event EventTick
  (params (DeltaSeconds :type Float%20%28single-precision%29))
  (bind _collider (Variables|Default|GetCollider))
  (bind _returnvalue (Transformation|GetWorldLocation _collider))
  (Utilities|FlowControl|Sequence
    (:then_0
      (if (<= (Variables|/Script/RLFPS.HealthComponent|GetcurrentHealth (Variables|Default|GetHealthComponent)) 0.0)
        (Game|OpenLevel(byObjectReference) "/Game/Maps/3D_MenuMap.3D_MenuMap")
        (else
          (CallFunction|SetGunValues)
          (if (Variables|Default|Getfiring)
            (Class|MatineeCameraShake|StartMatineeCameraShake (Game|GetPlayerCameraManager 0) "/Game/BPs/Player/BP_GunShake.BP_GunShake_C" 0.8 "CameraLocal" "0, 0, 0")
            (Class|FragPlayer|AddRotation))
          (bind _outhit (Collision|LineTraceByChannel _returnvalue (+ (* (Math|Vector|GetUpVector _collider) -1e+03) _returnvalue) "TraceTypeQuery1" false 0 "None"))
          (Variables|Default|SetLocationUnderPlayer (.ImpactPoint (Collision|BreakHitResult _outhit))))))
    (:then_1
      (bind _aswbp_settings_controller (Utilities|Casting|CastToWBP_SettingsController (Game|GetGameInstance)))
      (Variables|Default|SetMouseSensitivity (Variables|/Game/Widgets/3D_Menu/WBP_SettingsController.WBP_SettingsController_C|GetPlayerSensitivity _aswbp_settings_controller)))
    (:then_2
      (CallFunction|LockCamera))))

(event Input|KeyboardEvents|Home
  (params (Key :type Key%20Structure))
  (:Pressed
    (Game|OpenLevel(byName) "3D_MenuMap")))

(event Input|KeyboardEvents|P
  (params (Key :type Key%20Structure))
  (bind _returnvalue (Game|GetPlayerController 0))
  (:Pressed
    ;[1 1 1] Escape Pressed
    (Development|PrintString "Hello")
    (Utilities|IsValid (Variables|Default|GetPauseMenuRef)
      (:Is%20Valid
        _)
      (:Is%20Not%20Valid
        (bind _returnvalue_2 (UserInterface|CreateWidget "/Game/BPs/PauseMenu/WBP_PauseMenu.WBP_PauseMenu_C"))
        (Variables|Default|SetPauseMenuRef _returnvalue_2)))
    (if (Game|IsGamePaused)
      ;[1 1 1] If the game is paused, unpause it
      (Widget|RemovefromParent (Variables|Default|GetPauseMenuRef))
      (Game|SetGamePaused false)
      (Variables|/Script/Engine.PlayerController|SetbShowMouseCursor _returnvalue false)
      (Input|SetInputModeGameOnly _returnvalue)
      (else
        ;[1 1 1] If the game isn't paused, pause it
        (UserInterface|Viewport|AddtoViewport (Variables|Default|GetPauseMenuRef) 0)
        (Game|SetGamePaused true)
        (Variables|/Script/Engine.PlayerController|SetbShowMouseCursor _returnvalue true)
        (Input|SetInputModeGameandUI _returnvalue (Variables|Default|GetPauseMenuRef) "LockInFullscreen" false)))))

(event Input|KeyboardEvents|Escape
  (params (Key :type Key%20Structure))
  (bind _returnvalue (Game|GetPlayerController 0))
  (:Pressed
    ;[1 1 1] Escape Pressed
    (Development|PrintString "Hello")
    (Utilities|IsValid (Variables|Default|GetPauseMenuRef)
      (:Is%20Valid
        _)
      (:Is%20Not%20Valid
        (bind _returnvalue_2 (UserInterface|CreateWidget "/Game/BPs/PauseMenu/WBP_PauseMenu.WBP_PauseMenu_C"))
        (Variables|Default|SetPauseMenuRef _returnvalue_2)))
    (if (Game|IsGamePaused)
      ;[1 1 1] If the game is paused, unpause it
      (Widget|RemovefromParent (Variables|Default|GetPauseMenuRef))
      (Game|SetGamePaused false)
      (Variables|/Script/Engine.PlayerController|SetbShowMouseCursor _returnvalue false)
      (Input|SetInputModeGameOnly _returnvalue)
      (else
        ;[1 1 1] If the game isn't paused, pause it
        (UserInterface|Viewport|AddtoViewport (Variables|Default|GetPauseMenuRef) 0)
        (Game|SetGamePaused true)
        (Variables|/Script/Engine.PlayerController|SetbShowMouseCursor _returnvalue true)
        (Input|SetInputModeGameandUI _returnvalue (Variables|Default|GetPauseMenuRef) "LockInFullscreen" false)))))

(event Input|KeyboardEvents|F
  (params (Key :type Key%20Structure))
  (bind _firstpersoncameracomponent (Variables|Default|GetFirstPersonCameraComponent))
  (bind _returnvalue (Transformation|GetWorldLocation _firstpersoncameracomponent))
  ;[1 1 1] Interact
  (:Pressed
    (bind _aswbp_settings_controller (Utilities|Casting|CastToWBP_SettingsController (Game|GetGameInstance)))
    (if (not (Variables|/Game/Widgets/3D_Menu/WBP_SettingsController.WBP_SettingsController_C|GetLeftHandToggle _aswbp_settings_controller))
      (bind _outhit (Collision|LineTraceByChannel _returnvalue (+ _returnvalue (* (Math|Vector|GetForwardVector _firstpersoncameracomponent) 4e+02)) "TraceTypeQuery1" false 0 "None"))
      (bind _asbp_beacon (Utilities|Casting|CastToBP_Beacon (.HitActor (Collision|BreakHitResult _outhit))))
      (Class|BeaconActor|Use _asbp_beacon))))

(event Input|KeyboardEvents|Enter
  (params (Key :type Key%20Structure))
  (bind _firstpersoncameracomponent (Variables|Default|GetFirstPersonCameraComponent))
  (bind _returnvalue (Transformation|GetWorldLocation _firstpersoncameracomponent))
  ;[1 1 1] Interact
  (:Pressed
    (bind _aswbp_settings_controller (Utilities|Casting|CastToWBP_SettingsController (Game|GetGameInstance)))
    (if (Variables|/Game/Widgets/3D_Menu/WBP_SettingsController.WBP_SettingsController_C|GetLeftHandToggle _aswbp_settings_controller)
      (bind _outhit (Collision|LineTraceByChannel _returnvalue (+ _returnvalue (* (Math|Vector|GetForwardVector _firstpersoncameracomponent) 4e+02)) "TraceTypeQuery1" false 0 "None"))
      (bind _asbp_beacon (Utilities|Casting|CastToBP_Beacon (.HitActor (Collision|BreakHitResult _outhit))))
      (Class|BeaconActor|Use _asbp_beacon))))

(fn ConstructionScript)

(fn SetGunValues
  (bind _asgun (Utilities|Casting|CastToGun (Variables|/Script/Engine.ChildActorComponent|GetChildActor (Variables|Default|GetGun))))
  (Variables|Default|SetcurAmmoCount (Variables|/Script/RLFPS.Gun|GetammoRemaining _asgun))
  (Variables|Default|SetmaxAmmoCount (Variables|/Script/RLFPS.Gun|GetammoCount _asgun))
  (Variables|Default|Setreloading (Variables|/Script/RLFPS.Gun|Getreloading _asgun))
  (Variables|Default|Setfiring (Variables|/Script/RLFPS.Gun|Getfiring _asgun)))