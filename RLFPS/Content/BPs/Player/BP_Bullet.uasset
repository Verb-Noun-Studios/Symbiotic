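; BP_Bullet is a projectile with a colored Niagara trail spawned on BeginPlay.
; On overlap, bullets not spawned by enemies that hit a BP_Grunt call the player gun's OnHitCallback, apply that gun's damage and destroy themselves.
; They ignore beacons, voiceline triggers, bullets and guns, and otherwise self-destroy only on the player.
; Enemy-spawned bullets have no overlap response in this graph.
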(event OnComponentBeginOverlap(CollisionComponent)
  (params (OverlappedComponent :type Primitive%20Component%20Object%20Reference) (OtherActor :type Actor%20Object%20Reference) (OtherComp :type Primitive%20Component%20Object%20Reference) (OtherBodyIndex :type Integer) (bFromSweep :type Boolean) (SweepResult :type Hit%20Result%20Structure%20%28by%20ref%29))
  (if (not (Variables|Default|GetspawnedByEnemy))
    (bind _asgrunt (Utilities|Casting|CastToBP_Grunt OtherActor)
      (:then
        (bind _returnvalue (Actor|GetActorOfClass "/Game/BPs/Player/BP_FPS_Player.BP_FPS_Player_C"))
        (bind _asgun_bp (Utilities|Casting|CastToBP_Gun (Variables|/Script/Engine.ChildActorComponent|GetChildActor (Variables|/Game/BPs/Player/BP_FPS_Player.BP_FPS_Player_C|GetGun _returnvalue))))
        (Class|Gun|OnHitCallback _asgun_bp _asgrunt)
        (Game|Damage|ApplyDamage _asgrunt (Variables|/Script/RLFPS.Gun|GetDamage _asgun_bp) 0 0)
        (Actor|DestroyActor))
      (:CastFailed
        (Utilities|Casting|CastToBP_Beacon OtherActor
          (:CastFailed
            (Utilities|Casting|CastToBP_VoicelineTrigger OtherActor
              (:CastFailed
                (Utilities|Casting|CastToBP_Bullet OtherActor
                  (:CastFailed
                    (Utilities|Casting|CastToBP_Gun OtherActor
                      (:CastFailed
                        (Utilities|Casting|CastToBP_FPS_Player OtherActor)
                        (Actor|DestroyActor)))))))))))))

(event EventBeginPlay
  (bind _returnvalue (Niagara|SpawnSystemAttached "/Game/Art/FX/BulletTrail/NS_Trail.NS_Trail" (Variables|Default|GetStaticMesh) "None" "0, 0, 0" "0, 0, 0" "KeepRelativeOffset" true))
  ;[1 1 1] Set Trail Color
  (Niagara|SetNiagaraVariable(LinearColor) _returnvalue "trail_color" (Math|Conversions|ToLinearColor(Color) (Variables|Default|Getcolor)))
  ;[1 1 1] Set Trail Width
  (Niagara|SetNiagaraVariable(Float) _returnvalue "trail_width" 15.0)
  ;[1 1 1] Set Trail Lifetime
  (Niagara|SetNiagaraVariable(Float) _returnvalue "trail_lifetime" 0.1))

(event Collision|EventActorBeginOverlap
  (params (OtherActor :type Actor%20Object%20Reference)))

(event EventTick
  (params (DeltaSeconds :type Float%20%28single-precision%29)))

(fn ConstructionScript)