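; BP_HollowBones is a player mod that trades maximum health for an extra jump.
; When applied, it lowers the health component's DefaultHealth by the PercentHealthLost percentage and clamps CurrentHealth to the new maximum.
; It then raises the movement component's MaxJumps by one.
; The changes are written directly to the player's components, and the graph has no logic to revert them.
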(event EventOnApply
  (params (player :type Frag%20Player%20Object%20Reference))
  (bind _healthcomponent (Variables|/Script/RLFPS.FragPlayer|GetHealthComponent player))
  (bind _movementcomponent (Variables|/Script/RLFPS.FragPlayer|GetMovementComponent player))
  (bind _output_get (Variables|/Script/RLFPS.HealthComponent|SetDefaultHealth _healthcomponent (* (Variables|/Script/RLFPS.HealthComponent|GetDefaultHealth _healthcomponent) (- 1.0 (/ (Variables|Default|GetPercentHealthLost) 1e+02)))))
  (Variables|/Script/RLFPS.HealthComponent|SetcurrentHealth _healthcomponent (Math|Float|Clamp(Float) (Variables|/Script/RLFPS.HealthComponent|GetcurrentHealth _healthcomponent) 0.0 _output_get))
  (Variables|/Script/RLFPS.FragMovementComponent|SetMaxJumps _movementcomponent (+ (Variables|/Script/RLFPS.FragMovementComponent|GetMaxJumps _movementcomponent) 1)))