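; BP_Napalm is a timed fire hazard that damages grunt characters and the FPS player standing in it.
; On BeginPlay it spawns a fire particle system and sets its lifespan from the trail duration.
; Tick feeds a Delay that throttles damage to everything valid overlapping its Box.
; UpdateStats lets a caller override duration and damage, resetting the lifespan.
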(event EventBeginPlay
  (bind _self self)
  (bind _returnvalue (Transformation|GetActorTransform _self))
  (bind (_location _rotation) (Math|Transform|BreakTransform _returnvalue))
  (Niagara|SpawnSystemAttached "/Game/Art/FX/FireEffect/NE_FireParts_System.NE_FireParts_System" 0 "None" _location _rotation "KeepRelativeOffset" false)
  (Actor|SetLifeSpan (Variables|Default|GetTrailDuration)))

(event EventTick
  (params (DeltaSeconds :type Float%20%28single-precision%29))
  (bind _self self)
  (bind _traildamage (Variables|Default|GetTrailDamage))
  (Utilities|FlowControl|Delay (Variables|Default|GetDelayBetweenDamageTick))
  (for _array_element (Collision|GetOverlappingActors (Variables|Default|GetBox) 0 :!class /Script/Engine.PrimitiveComponent)
    (bind _asbp_grunt_character_base (Utilities|Casting|CastToBP_GruntCharacterBase _array_element)
      (:then
        (Game|Damage|ApplyDamage _asbp_grunt_character_base _traildamage 0 _self))
      (:CastFailed
        (bind _asbp_fpsplayer (Utilities|Casting|CastToBP_FPSPlayer _array_element))
        (Game|Damage|ApplyDamage _asbp_fpsplayer _traildamage 0 _self)))))

(fn ConstructionScript)

(fn UpdateStats
  (params (Dur :type Float%20%28single-precision%29) (Dmg :type Float%20%28single-precision%29))
  (bind _output_get (Variables|Default|SetTrailDuration Dur))
  (Actor|SetLifeSpan _output_get)
  (Variables|Default|SetTrailDamage Dmg))