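; Berserker mode mod that buffs BP_FPSPlayer's jump force, ground speed, default health and gun damage on low health.
; OnLowHealth caches the original stats, applies multipliers and refreshes the gun's core stats.
; A Used branch accumulates delta time to restore those values after Lifetime, but shares the activation's DoOnce, which has no reset, so repeat calls never reach it.
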(event EventOnLowHealth
  (params (deltatime :type Float%20%28single-precision%29))
  (Utilities|FlowControl|DoOnce false
    (:Completed
      (if (Variables|Default|GetUsed)
        (if (< (Variables|Default|GetElapsedTime) (Variables|Default|GetLifetime))
          (bind _output_get (Variables|Default|SetElapsedTime (+ (Variables|Default|GetElapsedTime) deltatime)))
          (Development|PrintString 0 (Utilities|String|ToString(Float) _output_get))
          (if (not (< (Variables|Default|GetElapsedTime) (Variables|Default|GetLifetime)))
            (bind _returnvalue (Class|ModBase|GetActorOfClassInternal "/Game/BPs/BP_FPSPlayer.BP_FPSPlayer_C"))
            (bind _asbp_fpsplayer (Utilities|Casting|CastToBP_FPSPlayer _returnvalue))
            (|UpdateWithOldVals _asbp_fpsplayer)
            (Development|PrintString 0 "Values Set to normal")))
        (else
          (Variables|Default|SetUsed true)
          (bind _returnvalue_2 (Class|ModBase|GetActorOfClassInternal "/Game/BPs/BP_FPSPlayer.BP_FPSPlayer_C"))
          (bind _asbp_fpsplayer_2 (Utilities|Casting|CastToBP_FPSPlayer _returnvalue_2))
          (|SetLocalValues _asbp_fpsplayer_2
            (:NewParam
              (|UpdateWithNewVals _asbp_fpsplayer_2)
              (Development|PrintString 0 "Values Updated" true true "(R=1.000000,G=0.010436,B=0.000000,A=1.000000)" 3e+01))))))))