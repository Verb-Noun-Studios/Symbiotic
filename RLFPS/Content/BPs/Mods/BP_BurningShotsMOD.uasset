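; Burning Shots mod that sets hit grunts on fire and turns on the fire visuals of bullets.
; On hit, it attaches a fire Niagara system to the GruntCharacter's capsule, then constructs and adds the configured Effect object.
; The chance check scales with stacks, but RandomFloat is unconnected, so it compares zero and passes whenever the chance is non-negative.
; The bullet VFX update activates FireVFX on BP_Bullet.
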(event EventOnHit
  (params (hitActor :type Actor%20Object%20Reference) (world :type World%20Object%20Reference))
  (if (<= (* 0.0 1e+02) (+ (* (Variables|Default|Getstacks) (Variables|Default|GetstackingChance)) (Variables|Default|GetbaseChance)))
    (bind _asgrunt_character (Utilities|Casting|CastToGruntCharacter hitActor))
    (Niagara|SpawnSystemAttached "/Game/Art/FX/FireEffect/NE_FireSingle_System.NE_FireSingle_System" (Variables|/Script/Engine.Character|GetCapsuleComponent _asgrunt_character) "None" "0, 0, 0" "0, 0, 0" "KeepRelativeOffset" false)
    (bind _returnvalue (Game|ConstructObjectfromClass (Variables|Default|GetEffect) _asgrunt_character))
    (Class|GruntCharacter|AddEffect _asgrunt_character _returnvalue)))

(event EventOnUpdateBulletVFX
  (params (bullet :type Bullet%20Object%20Reference))
  (bind _asbp_bullet (Utilities|Casting|CastToBP_Bullet bullet))
  (Components|Activation|Activate (Variables|/Game/BPs/BP_Bullet.BP_Bullet_C|GetFireVFX _asbp_bullet) false))