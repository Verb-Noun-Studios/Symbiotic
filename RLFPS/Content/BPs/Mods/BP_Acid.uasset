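; Acid pool hazard that applies a status effect to grunts and damages the player until its duration expires.
; On spawn, a downward trace ignoring grunts snaps it onto surfaces matched by actor name, or teleports it far away.
; Tick applies the effect to overlapping grunts and hurts an overlapping player, whose damage value updates after two seconds.
; Only the player branch re-arms both damage gates, after an interval.
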(event OnComponentBeginOverlap(BoxCollider)
  (params (OverlappedComponent :type Primitive%20Component%20Object%20Reference) (OtherActor :type Actor%20Object%20Reference) (OtherComp :type Primitive%20Component%20Object%20Reference) (OtherBodyIndex :type Integer) (bFromSweep :type Boolean) (SweepResult :type Hit%20Result%20Structure%20%28by%20ref%29)))

(event EventBeginPlay
  (bind _self self)
  (bind _returnvalue (Transformation|GetActorLocation _self))
  (bind (_x _y _z) (Math|Vector|BreakVector _returnvalue))
  (bind _outactors (Actor|GetAllActorsOfClass "/Script/RLFPS.GruntCharacter"))
  (bind _outhit (Collision|LineTraceByChannel _returnvalue (Math|Vector|MakeVector _x _y (- _z 2e+03)) "TraceTypeQuery2" false _outactors "ForDuration" true "(R=1.000000,G=0.000000,B=0.000000,A=1.000000)" "(R=0.000000,G=1.000000,B=0.000000,A=1.000000)" 2.0))
  (if (Math|Boolean|ORBoolean (Utilities|String|Contains (Utilities|GetObjectName (.HitActor (Collision|BreakHitResult _outhit))) "Floor") (Utilities|String|Contains (Utilities|GetObjectName (.HitActor (Collision|BreakHitResult _outhit))) "Wall") (Utilities|String|Contains (Utilities|GetObjectName (.HitActor (Collision|BreakHitResult _outhit))) "Stair") (Utilities|String|Contains (Utilities|GetObjectName (.HitActor (Collision|BreakHitResult _outhit))) "Platform") (Utilities|String|Contains (Utilities|GetObjectName (.HitActor (Collision|BreakHitResult _outhit))) "Rock") (Utilities|String|Contains (Utilities|GetObjectName (.HitActor (Collision|BreakHitResult _outhit))) "Center") (Utilities|String|Contains (Utilities|GetObjectName (.HitActor (Collision|BreakHitResult _outhit))) "Column"))
    (Transformation|SetActorLocation (+ (.ImpactPoint (Collision|BreakHitResult _outhit)) "0, 0,-2.000000") false true)
    (Audio|SpawnSoundAttached "/Game/Audio/GunSFX/Upgrades_SFX-20220419T053714Z-001/Upgrades_SFX/_ON_HIT_SPREADING_Acid_Shots__no_ticking_._ON_HIT_SPREADING_Acid_Shots__no_ticking_" (Variables|Transformation|GetRootComponent) "None" "0, 0, 0" "0, 0, 0" "KeepRelativeOffset" false 15.0 1.0 0.0 "/Game/Audio/BurnAtt.BurnAtt" 0)
    (else
      (Transformation|SetActorLocation "0.000000, 0,99999.000000" false true)))
  (Utilities|FlowControl|Delay 2.0)
  (Variables|AffectPlayer|SetDamageToPlayer (Variables|Default|Getdamage))
  (Utilities|FlowControl|Delay (- (Variables|Default|Getduration) 2.0))
  (Actor|DestroyActor))

(event EventDestroyed)

(event EventTick
  (params (DeltaSeconds :type Float%20%28single-precision%29))
  (bind _returnvalue (Game|Player|GetPlayerPawn 0))
  (if (Variables|Default|GetCanDamage)
    (for _array_element (Collision|GetOverlappingActors (Variables|Default|GetBoxCollider) "/Script/RLFPS.GruntCharacter" :!class /Script/Engine.PrimitiveComponent)
      (bind _asgrunt_character (Utilities|Casting|CastToGruntCharacter _array_element))
      (bind _returnvalue_2 (Game|ConstructObjectfromClass (Variables|Default|GetStatusEffect) _asgrunt_character))
      (Class|GruntCharacter|AddEffect _asgrunt_character _returnvalue_2))
    (Variables|Default|SetCanDamage false))
  (if (and (Collision|IsOverlappingActor _returnvalue :!class /Script/Engine.Actor) (Variables|AffectPlayer|GetCanDamagePlayer))
    (bind _asbp_fpsplayer (Utilities|Casting|CastToBP_FPSPlayer _returnvalue))
    (Game|Damage|ApplyDamage _asbp_fpsplayer (Variables|AffectPlayer|GetDamageToPlayer) 0 self)
    (Variables|AffectPlayer|SetCanDamagePlayer false)
    (Utilities|FlowControl|Delay (Variables|Default|Getinterval))
    (Variables|Default|SetCanDamage true)
    (Variables|AffectPlayer|SetCanDamagePlayer true)
    (Audio|PlaySoundatLocation "/Game/Audio/GunSFX/Upgrades_SFX-20220419T053714Z-001/Upgrades_SFX/Acid_Shot.Acid_Shot" (Transformation|GetActorLocation) "0, 0, 0" 1.0 1.0 0.0 "/Game/Audio/BurnAtt.BurnAtt" 0 0)))

(fn ConstructionScript)