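; BP_HealingOnHitMod is a stackable on-hit mod that gives hits a chance to spawn a healing beam.
; OnHit rolls a random percentage against HealChance plus StackingChance scaled by Stacks, and on success spawns BP_HealingBeam at the hit actor, which becomes its owner.
; It also looks up BP_FPSPlayer without visibly using the result.
; A debug print shows a separately rolled value, so it can differ from the roll tested.
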(event EventOnHit
  (params (hitActor :type Actor%20Object%20Reference) (world :type World%20Object%20Reference))
  (bind _returnvalue (Math|Random|RandomFloat))
  (bind _stackingchance (Variables|Default|GetStackingChance))
  (bind _healchance (Variables|Default|GetHealChance))
  (bind _stacks (Variables|Default|Getstacks))
  (bind _returnvalue_2 (Math|Conversions|ToFloat(Integer) _stacks))
  (bind _returnvalue_3 (* _returnvalue 1e+02))
  (bind _returnvalue_4 (* _stackingchance _returnvalue_2))
  (bind _returnvalue_5 (+ _healchance _returnvalue_4))
  (Development|PrintString world (Utilities|String|Append (Utilities|String|MakeLiteralString "Rand val: ") (Utilities|String|ToString(Float) _returnvalue_3) "   Chance:  " (Utilities|String|ToString(Float) _returnvalue_5)))
  (if (<= _returnvalue_3 _returnvalue_5)
    (Class|ModBase|GetActorOfClassInternal "/Game/BPs/BP_FPSPlayer.BP_FPSPlayer_C")
    (Class|ModBase|SpawnActorOfClassInternal hitActor "/Game/Art/FX/HealingShot/BP_HealingBeam.BP_HealingBeam_C" (Transformation|GetActorLocation hitActor) (Transformation|GetActorRotation hitActor))))