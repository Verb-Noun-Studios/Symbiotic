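; Bullet mod that adds napalm fire to shots, with duration growing per stack from a base value.
; On bullet spawn, it creates a BP_NapalmManager high above the world origin and passes it the bullet, duration, damage and spawn delay.
; On hit, it spawns a BP_Napalm at the hit actor's transform with the same stats.
; SpawnFireTrail is inert because its constant condition never passes.
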(event EventOnHit
  (params (hitActor :type Actor%20Object%20Reference) (world :type World%20Object%20Reference))
  (bind _returnvalue (Transformation|GetActorTransform hitActor))
  (bind (_location _rotation) (Math|Transform|BreakTransform _returnvalue))
  (bind _returnvalue_2 (Class|ModBase|SpawnActorOfClassInternal 0 "/Game/BPs/Mods/BP_Napalm.BP_Napalm_C" _location _rotation))
  (Transformation|SetActorScale3D _returnvalue_2 "1.000000,1.000000,1.000000")
  (bind _asbp_napalm (Utilities|Casting|CastToBP_Napalm _returnvalue_2))
  (Default|UpdateStats _asbp_napalm (+ (Variables|Default|GetTrailDurationBase) (* (Variables|Default|Getstacks) (Variables|Default|GetTrailDurationStackIncrease))) (Variables|Default|GetTrailDamage)))

(event EventOnSpawn
  (params (bullet :type Bullet%20Object%20Reference))
  (bind _returnvalue (Class|ModBase|SpawnActorOfClassInternal 0 "/Game/BPs/Mods/BP_NapalmManager.BP_NapalmManager_C" (Math|Vector|MakeVector 0.0 0.0 99999.0) (Math|Rotator|MakeRotator 0.0 0.0 0.0)))
  (bind _asbp_napalm_manager (Utilities|Casting|CastToBP_NapalmManager _returnvalue))
  (Default|SetStats _asbp_napalm_manager (+ (Variables|Default|GetTrailDurationBase) (* (Variables|Default|Getstacks) (Variables|Default|GetTrailDurationStackIncrease))) (Variables|Default|GetTrailDamage) bullet)
  (Variables|/Game/BPs/Mods/BP_NapalmManager.BP_NapalmManager_C|SetSpawnDelay _asbp_napalm_manager (Variables|Default|GetSpawnDelay)))

(fn SpawnFireTrail
  (bind _thebullet (Variables|Default|GetTheBullet))
  (bind _returnvalue (Transformation|GetActorTransform _thebullet))
  (bind (_location _rotation) (Math|Transform|BreakTransform _returnvalue))
  (if (not (>= 0 0))
    (bind _returnvalue_2 (Class|ModBase|SpawnActorOfClassInternal 0 "/Game/BPs/Mods/BP_Napalm.BP_Napalm_C" _location _rotation))
    (bind _asbp_napalm (Utilities|Casting|CastToBP_Napalm _returnvalue_2))
    (Variables|/Game/BPs/Mods/BP_Napalm.BP_Napalm_C|SetTrailDuration _asbp_napalm (+ (Variables|Default|GetTrailDurationBase) (* (Variables|Default|Getstacks) (Variables|Default|GetTrailDurationStackIncrease))))))