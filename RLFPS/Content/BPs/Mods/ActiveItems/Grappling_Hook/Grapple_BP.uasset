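; Grappling hook actor that anchors at an end point and pulls the FPS player toward it, with a cable attached to the gun.
; Player input is disabled while it exists and gravity drops on start, both restored as it ends.
; Tick sets player velocity toward the hook plus movement-input steering scaled by air sensitivity.
; It destroys itself when the player gets within break distance or overlaps its sphere, or something else touches the cable.
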(event OnComponentBeginOverlap(Sphere)
  (params (OverlappedComponent :type Primitive%20Component%20Object%20Reference) (OtherActor :type Actor%20Object%20Reference) (OtherComp :type Primitive%20Component%20Object%20Reference) (OtherBodyIndex :type Integer) (bFromSweep :type Boolean) (SweepResult :type Hit%20Result%20Structure%20%28by%20ref%29))
  (if (Variables|Default|Getstarted)
    (Utilities|Casting|CastToBP_FPSPlayer OtherActor)
    (Variables|Default|SetPlayerOverlapped true)
    (Development|PrintString "grapple finished")
    (CallFunction|OnDestroy)))

(event OnComponentBeginOverlap(Cable)
  (params (OverlappedComponent :type Primitive%20Component%20Object%20Reference) (OtherActor :type Actor%20Object%20Reference) (OtherComp :type Primitive%20Component%20Object%20Reference) (OtherBodyIndex :type Integer) (bFromSweep :type Boolean) (SweepResult :type Hit%20Result%20Structure%20%28by%20ref%29))
  (Utilities|Casting|CastToBP_FPSPlayer OtherActor
    (:CastFailed
      (Utilities|Casting|CastToBP_Gun OtherActor
        (:CastFailed
          (Development|PrintString "overlapping cable")
          (CallFunction|OnDestroy))))))

(event Custom|OnDestroy
  (Variables|/Script/RLFPS.FragMovementComponent|SetGravity (Variables|/Script/RLFPS.FragPlayer|GetMovementComponent (Variables|Default|GetPlayer)) 8e+02)
  (Actor|DestroyActor))

(event EventBeginPlay
  (bind _returnvalue (Actor|GetActorOfClass "/Game/BPs/BP_FPSPlayer.BP_FPSPlayer_C"))
  (bind _output_get (Variables|Default|SetPlayer _returnvalue))
  (Variables|Default|SetDirection (- (Variables|Default|GetendLoc) (Variables|Default|GetstartLoc)))
  (Input|DisableInput _output_get (Game|GetPlayerController 0)))

(event EventDestroyed
  (Input|EnableInput (Variables|Default|GetPlayer) (Game|GetPlayerController 0)))

(event EventTick
  (params (DeltaSeconds :type Float%20%28single-precision%29))
  (bind _returnvalue (Transformation|GetActorLocation))
  (bind _player (Variables|Default|GetPlayer))
  (bind _returnvalue_2 (Transformation|GetActorLocation _player))
  (bind _movementinput (Variables|/Script/RLFPS.FragPlayer|GetMovementInput _player))
  (bind _returnvalue_3 (- _returnvalue _returnvalue_2))
  (bind (_x _y) (Math|Vector2D|BreakVector2D _movementinput))
  (if (not (Variables|Default|GetPlayerOverlapped))
    (Class|FragPlayer|SetVelocity _player (+ (* (Math|Vector|MakeVector _x _y 0.0) (Variables|Default|GetaireSensitivity)) (* (Math|Vector|Normalize _returnvalue_3) (Variables|Default|GetSpeed))))
    (if (< (Math|Vector|VectorLength _returnvalue_3) (Variables|Default|GetbreakDistance))
      (CallFunction|OnDestroy))
    (else
      (Development|PrintString "FAILURE" true true "(R=0.000000,G=0.660000,B=1.000000,A=1.000000)" 2e+01))))

(event EventOnStart
  (params (gun :type Actor%20Object%20Reference))
  (Transformation|SetActorLocation (Variables|Default|GetendLoc) false false)
  (Class|CableComponent|SetAttachEndto (Variables|Default|GetCable) gun "None" "None")
  (Variables|Default|Setstarted true)
  (Variables|/Script/RLFPS.FragMovementComponent|SetGravity (Variables|/Script/RLFPS.FragPlayer|GetMovementComponent (Variables|Default|GetPlayer)) 9.0))

(fn ConstructionScript)