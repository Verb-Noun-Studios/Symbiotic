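; Active item mod that spawns a black hole in front of the gun when its ability triggers.
; OnActiveAbility spawns the BlackHole actor a short way along the gun's forward vector, matching its rotation and owned by the gun.
; It prints the current and required kill counts to screen, then resets the current count to zero.
; This graph does not compare the two counts itself.
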(event EventOnActiveAbility
  (params (gun :type Actor%20Object%20Reference))
  (Development|PrintString 0 (Utilities|String|ToString(Integer) (Variables|Default|GetcurrentKillCount)))
  (Development|PrintString 0 (Utilities|String|ToString(Integer) (Variables|Default|GetrequiredKillCount)))
  (Class|ActiveItem|SpawnActorOfClassInternal gun "/Game/BPs/Mods/ActiveItems/BlackHole/BlackHole.BlackHole_C" (+ (Transformation|GetActorLocation gun) (* (Transformation|GetActorForwardVector gun) 200)) (Transformation|GetActorRotation gun))
  (Variables|Default|SetcurrentKillCount 0))