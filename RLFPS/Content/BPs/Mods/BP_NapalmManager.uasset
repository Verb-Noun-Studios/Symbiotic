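; BP_NapalmManager is a mod actor that leaves a trail of napalm behind a bullet.
; SetStats stores the bullet along with the trail's duration and damage.
; Every Tick it spawns a BP_Napalm at the bullet's location and rotation and passes it those stats, destroying itself once the bullet is no longer valid.
; A SpawnDelay wait exists but never runs, so spawning is per frame.
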(event EventBeginPlay)

(event Collision|EventActorBeginOverlap
  (params (OtherActor :type Actor%20Object%20Reference)))

(event EventTick
  (params (DeltaSeconds :type Float%20%28single-precision%29))
  (bind _thebullet (Variables|Default|GetTheBullet))
  (bind _returnvalue (Transformation|GetActorTransform _thebullet))
  (bind (_location _rotation) (Math|Transform|BreakTransform _returnvalue))
  (if (Utilities|IsValid (Variables|Default|GetTheBullet))
    (bind _returnvalue_2 (Game|SpawnActorfromClass "/Game/BPs/Mods/BP_Napalm.BP_Napalm_C" (Math|Transform|MakeTransform _location _rotation) "Undefined" 0 0))
    (Default|UpdateStats _returnvalue_2 (Variables|Default|GetTrailDuration) (Variables|Default|GetTrailDamage))
    (else
      (Actor|DestroyActor))))

(fn ConstructionScript)

(fn SetStats
  (params (Dur :type Float%20%28single-precision%29) (Dmg :type Float%20%28single-precision%29) (Bullet :type Bullet%20Object%20Reference))
  (Variables|Default|SetTrailDuration Dur)
  (Variables|Default|SetTrailDamage Dmg)
  (Variables|Default|SetTheBullet Bullet))