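; BP_Armor is a player mod that trades movement speed for armor.
; On apply, it adds a per-stack damage block value to the HealthComponent's Armor.
; It also cuts the MovementComponent's ground and air max speeds by separate percentages, scaling the current values so repeated applications compound.
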(event EventOnApply
  (params (player :type Frag%20Player%20Object%20Reference))
  (bind _healthcomponent (Variables|/Script/RLFPS.FragPlayer|GetHealthComponent player))
  (bind _movementcomponent (Variables|/Script/RLFPS.FragPlayer|GetMovementComponent player))
  (Variables|/Script/RLFPS.HealthComponent|Setarmor _healthcomponent (+ (Variables|/Script/RLFPS.HealthComponent|Getarmor _healthcomponent) (Variables|Default|GetDamageBlockPerStack)))
  (Variables|/Script/RLFPS.FragMovementComponent|SetGroundMaxSpeed _movementcomponent (* (Variables|/Script/RLFPS.FragMovementComponent|GetGroundMaxSpeed _movementcomponent) (- 1.0 (/ (Variables|Default|GetGroundSpeedReductionPercentage) 1e+02))))
  (Variables|/Script/RLFPS.FragMovementComponent|SetAirMaxSpeed _movementcomponent (* (Variables|/Script/RLFPS.FragMovementComponent|GetAirMaxSpeed _movementcomponent) (- 1.0 (/ (Variables|Default|GetAirSpeedReductionPercentage) 1e+02)))))