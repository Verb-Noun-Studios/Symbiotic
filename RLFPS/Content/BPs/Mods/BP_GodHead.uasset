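; BP_GodHead is a mod actor that damages GruntCharacters inside its ColArea collision volume.
; An overlap starts a 0.01-second Delay loop that applies damage and calls OnHitCallback on the player's Gun child actor.
; A single InRadius flag controls the loop, so any grunt leaving clears it, even if others remain inside.
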(event OnComponentBeginOverlap(ColArea)
  (params (OverlappedComponent :type Primitive%20Component%20Object%20Reference) (OtherActor :type Actor%20Object%20Reference) (OtherComp :type Primitive%20Component%20Object%20Reference) (OtherBodyIndex :type Integer) (bFromSweep :type Boolean) (SweepResult :type Hit%20Result%20Structure%20%28by%20ref%29))
  (Utilities|Casting|CastToGruntCharacter OtherActor)
  (Variables|Default|SetinRadius true)
  (bind _returnvalue (Actor|GetActorOfClass "/Game/BPs/BP_FPSPlayer.BP_FPSPlayer_C" :!label _label))
  (bind _asgun (Utilities|Casting|CastToGun (Variables|/Script/Engine.ChildActorComponent|GetChildActor (Variables|/Game/BPs/BP_FPSPlayer.BP_FPSPlayer_C|GetGun _returnvalue))))
  (Class|Gun|OnHitCallback _asgun)
  (Game|Damage|ApplyDamage OtherActor 5.0 0 0)
  (Utilities|FlowControl|Delay 0.01)
  (if (Variables|Default|GetinRadius)
    (goto _label)))

(event OnComponentEndOverlap(ColArea)
  (params (OverlappedComponent :type Primitive%20Component%20Object%20Reference) (OtherActor :type Actor%20Object%20Reference) (OtherComp :type Primitive%20Component%20Object%20Reference) (OtherBodyIndex :type Integer))
  (Utilities|Casting|CastToGruntCharacter OtherActor)
  (Variables|Default|SetinRadius false))

(event EventBeginPlay)

(event EventTick
  (params (DeltaSeconds :type Float%20%28single-precision%29)))

(fn ConstructionScript)