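; BP_ShotgunMod is a gun mod that adds shotgun-style effects whenever its gun fires.
; On the fire event, it spawns a Niagara system offset from the gun along its forward vector by the muzzle location, using the gun's rotation.
; It passes the mod's stack count to the system's bullet count parameter.
; It also plays a symbiote explosion sound attached to the gun's root component.
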(event EventOnFire
  (params (gun :type Gun%20Object%20Reference))
  (bind _returnvalue (Class|ModBase|SpawnSystematLocationInternal (Variables|Default|GetniagaraVFX) (+ (* (Transformation|GetActorForwardVector gun) (Variables|/Script/RLFPS.Gun|GetMuzzleLocation gun)) (Transformation|GetActorLocation gun)) (Transformation|GetActorRotation gun) "1.000000,1.000000,1.000000"))
  (Class|NiagaraComponent|SetVariableInt _returnvalue "bulletCount" (Variables|Default|Getstacks))
  (bind _returnvalue_2 (Audio|SpawnSoundAttached "/Game/Audio/GunSFX/A_Symbiote_Explosion.A_Symbiote_Explosion" (Variables|/Script/Engine.Actor|GetRootComponent gun) "None" "0, 0, 0" "0, 0, 0" "KeepRelativeOffset" false 1.0 1.0 0.0 0 0))
  (Audio|Components|Audio|Play _returnvalue_2 0.0))