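; BP_AcidMod is a stackable acid mod for bullets, with this Blueprint handling its visual effect on the bullet trail.
; OnUpdateBulletVFX casts to BP_Bullet and rebuilds TrailColor with a clamped, stack-scaled amount added to the green channel.
; OnHit is an empty event marked as implemented in C++.
; A SetVariableLinearColor node for the trail color is left unconnected, so only the TrailColor variable changes here.
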(event EventOnHit
  (params (hitActor :type Actor%20Object%20Reference) (world :type World%20Object%20Reference))
  ;[1 1 1] Implemented in CPP. Don't edit.
)

(event EventOnUpdateBulletVFX
  (params (bullet :type Bullet%20Object%20Reference))
  (bind _asbp_bullet (Utilities|Casting|CastToBP_Bullet bullet))
  (Variables|/Game/BPs/BP_Bullet.BP_Bullet_C|Settrail_color _asbp_bullet (Math|Conversions|ToColor(LinearColor) (Utilities|Struct|MakeLinearColor (Math|Conversions|ToFloat(Byte) (.R (Math|Color|BreakColor (Variables|/Game/BPs/BP_Bullet.BP_Bullet_C|Gettrail_color _asbp_bullet)))) (+ (Math|Conversions|ToFloat(Byte) (.G (Math|Color|BreakColor (Variables|/Game/BPs/BP_Bullet.BP_Bullet_C|Gettrail_color _asbp_bullet)))) (Math|Float|Clamp(Float) (* (Variables|Default|Getstacks) 0.2))) (Math|Conversions|ToFloat(Byte) (.B (Math|Color|BreakColor (Variables|/Game/BPs/BP_Bullet.BP_Bullet_C|Gettrail_color _asbp_bullet)))) (Math|Conversions|ToFloat(Byte) (.A (Math|Color|BreakColor (Variables|/Game/BPs/BP_Bullet.BP_Bullet_C|Gettrail_color _asbp_bullet))))))))