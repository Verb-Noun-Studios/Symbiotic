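; BP_ExploadingShots is a stackable shot mod that sets off an explosion at the hit actor.
; OnHit spawns a Niagara effect and a radius-scaled trigger sphere to find overlapping GruntCharacters.
; Two identical loops each apply stack-scaled damage with distance falloff and push grunts outward by swept location offset.
; The stack-based chance is only debug-printed; the roll compares against 1000, so it always fires.
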(event EventOnHit
  (params (hitActor :type Actor%20Object%20Reference) (world :type World%20Object%20Reference))
  (bind _returnvalue (Transformation|GetActorTransform hitActor))
  (bind _returnvalue_2 (Math|Random|RandomFloat))
  (bind _damageradius (Variables|Default|GetDamageRadius))
  (bind (_location _rotation) (Math|Transform|BreakTransform _returnvalue))
  (bind _returnvalue_3 (* _returnvalue_2 1e+02))
  (Development|PrintString 0 (Utilities|String|Append (Utilities|String|MakeLiteralString "Rand val: ") (Utilities|String|ToString(Float) _returnvalue_3) "   Chance:  " (Utilities|String|ToString(Float) (+ (Variables|Default|GetBaseChance) (* (Variables|Default|GetStackingChance) (Math|Conversions|ToFloat(Integer) (Variables|Default|Getstacks)))))))
  (if (<= _returnvalue_3 1e+03)
    (Class|ModBase|SpawnSystematLocationInternal (Variables|Default|GetniagaraVFX) _location "0, 0, 0" "1.000000,1.000000,1.000000")
    (bind _returnvalue_4 (Class|ModBase|SpawnActorOfClassInternal 0 "/Script/Engine.TriggerSphere" _location _rotation))
    (Transformation|SetActorScale3D _returnvalue_4 (/ (Math|Vector|MakeVector _damageradius _damageradius _damageradius) 17.0))
    (for _array_element (Collision|GetOverlappingActors _returnvalue_4 "/Script/RLFPS.GruntCharacter" :!class /Script/Engine.Actor)
      (bind _asgrunt_character (Utilities|Casting|CastToGruntCharacter _array_element))
      (Game|Damage|ApplyDamage _asgrunt_character (* (- 1.0 (Math|Float|Absolute(Float) (/ (Math|Vector|Distance(Vector) (Transformation|GetActorLocation _array_element) _location) 1e+02))) (+ (* (- (Variables|Default|Getstacks) 1) (Variables|Default|GetStackingDamage)) (Variables|Default|GetBaseDamage))) 0 0)
      (Transformation|SetActorLocation _asgrunt_character (+ (Transformation|GetActorLocation _asgrunt_character) (* (Math|Vector|GetUnitDirection(Vector) _location (Transformation|GetActorLocation _array_element)) (Variables|Default|GetRepulsionForce))) true false))
    (for _array_element_2 (Collision|GetOverlappingActors _returnvalue_4 "/Script/RLFPS.GruntCharacter" :!class /Script/Engine.Actor)
      (bind _asgrunt_character_2 (Utilities|Casting|CastToGruntCharacter _array_element_2))
      (Game|Damage|ApplyDamage _asgrunt_character_2 (* (- 1.0 (Math|Float|Absolute(Float) (/ (Math|Vector|Distance(Vector) (Transformation|GetActorLocation _array_element_2) _location) 1e+02))) (+ (* (- (Variables|Default|Getstacks) 1) (Variables|Default|GetStackingDamage)) (Variables|Default|GetBaseDamage))) 0 0)
      (Transformation|SetActorLocation _asgrunt_character_2 (+ (Transformation|GetActorLocation _asgrunt_character_2) (* (Math|Vector|GetUnitDirection(Vector) _location (Transformation|GetActorLocation _array_element_2)) (Variables|Default|GetRepulsionForce))) true false))))