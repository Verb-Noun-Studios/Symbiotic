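; HealingOnHitModBP is a stackable mod that gives a chance to heal the player on hit.
; On each OnHit it rolls a random percentage against HealChance plus StackingChance times Stacks.
; A successful roll finds the FPS_Player actor by class and heals its HealthComponent by HPToGain.
; A debug print shows the chance and a roll, drawn separately from the one compared.
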(event EventOnHit
  (params (hitActor :type Actor%20Object%20Reference) (world :type World%20Object%20Reference))
  (bind _returnvalue (Math|Random|RandomFloat))
  (bind _stackingchance (Variables|Default|GetStackingChance))
  (bind _healchance (Variables|Default|GetHealChance))
  (bind _stacks (Variables|Default|Getstacks))
  (bind _returnvalue_2 (Math|Conversions|ToFloat(Integer) _stacks))
  (bind _returnvalue_3 (* _returnvalue 1e+02))
  (bind _returnvalue_4 (* _stackingchance _returnvalue_2))
  (bind _returnvalue_5 (+ _healchance _returnvalue_4))
  (Development|PrintString world (Utilities|String|Append (Utilities|String|MakeLiteralString "Rand val: ") (Utilities|String|ToString(Float) _returnvalue_3) "   Chance:  " (Utilities|String|ToString(Float) _returnvalue_5)))
  (if (<= _returnvalue_3 _returnvalue_5)
    (bind _returnvalue_6 (Class|ModBase|GetActorOfClassInternal "/Game/BPs/FPS_Player.FPS_Player_C"))
    (bind _asfps_player (Utilities|Casting|CastToFPS_Player _returnvalue_6))
    (Class|HealthComponent|Heal (Variables|/Script/RLFPS.FragPlayer|GetHealthComponent _asfps_player) (Variables|Default|GetHPToGain))))