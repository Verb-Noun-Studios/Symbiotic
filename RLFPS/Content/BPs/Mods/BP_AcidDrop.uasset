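; BP_AcidDrop is an acid drop actor that turns into a BP_Acid hazard on the surface below it.
; On overlap, it traces 1000 units down on the Camera channel, ignoring GruntCharacters and drawing debug lines.
; If the hit actor's name matches level-geometry keywords like Floor or Wall, it waits briefly and spawns BP_Acid at the impact point.
; It passes on its damage, duration and tick interval, then destroys itself.
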(event EventBeginPlay)

(event Collision|EventActorBeginOverlap
  (params (OtherActor :type Actor%20Object%20Reference))
  (bind _self self)
  (bind _returnvalue (Transformation|GetActorLocation _self))
  (bind (_x _y _z) (Math|Vector|BreakVector _returnvalue))
  (bind _outactors (Actor|GetAllActorsOfClass "/Script/RLFPS.GruntCharacter"))
  (bind _outhit (Collision|LineTraceByChannel _returnvalue (Math|Vector|MakeVector _x _y (- _z 1e+03)) "TraceTypeQuery2" false _outactors "ForDuration" true "(R=1.000000,G=0.000000,B=0.000000,A=1.000000)" "(R=0.000000,G=1.000000,B=0.000000,A=1.000000)" 2.0))
  (if (Math|Boolean|ORBoolean (Utilities|String|Contains (Utilities|GetObjectName (.HitActor (Collision|BreakHitResult _outhit))) "Floor") (Utilities|String|Contains (Utilities|GetObjectName (.HitActor (Collision|BreakHitResult _outhit))) "Wall") (Utilities|String|Contains (Utilities|GetObjectName (.HitActor (Collision|BreakHitResult _outhit))) "Stair") (Utilities|String|Contains (Utilities|GetObjectName (.HitActor (Collision|BreakHitResult _outhit))) "Platform") (Utilities|String|Contains (Utilities|GetObjectName (.HitActor (Collision|BreakHitResult _outhit))) "Rock") (Utilities|String|Contains (Utilities|GetObjectName (.HitActor (Collision|BreakHitResult _outhit))) "Center") (Utilities|String|Contains (Utilities|GetObjectName (.HitActor (Collision|BreakHitResult _outhit))) "Column"))
    (Utilities|FlowControl|Delay 0.2)
    (bind _returnvalue_2 (Game|SpawnActorfromClass "/Game/BPs/Mods/BP_Acid.BP_Acid_C" (Math|Conversions|ToTransform(Vector) (.ImpactPoint (Collision|BreakHitResult _outhit))) "Undefined" 0 0))
    (Variables|/Script/RLFPS.Acid|Setdamage _returnvalue_2 (Variables|Default|Getdamage))
    (Variables|/Game/BPs/Mods/BP_Acid.BP_Acid_C|SetDamageToPlayer _returnvalue_2 (Variables|Default|Getdamage))
    (Variables|/Script/RLFPS.Acid|Setduration _returnvalue_2 (Variables|Default|Getduration))
    (Variables|/Script/RLFPS.Acid|Setinterval _returnvalue_2 (Variables|Default|Getinterval))
    (Variables|/Game/BPs/Mods/BP_Acid.BP_Acid_C|SetTimeBetweenTicks _returnvalue_2 (Variables|Default|Getinterval))
    (Actor|DestroyActor)))

(fn ConstructionScript)