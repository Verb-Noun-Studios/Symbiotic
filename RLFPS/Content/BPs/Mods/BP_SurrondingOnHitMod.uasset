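; BP_SurrondingOnHitMod is an on-hit mod that spreads a gun hit to grunts surrounding the hit actor.
; OnHit scans all BP_Grunt actors and selects those within a base radius that grows with stack count.
; For each, it finds the BP_Gun and calls OnHitCallbackWithSkip with the mod's Name, apparently to avoid retriggering itself.
; It also prints each grunt's distance-to-radius ratio for debugging.
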(event EventOnHit
  (params (hitActor :type Actor%20Object%20Reference) (world :type World%20Object%20Reference))
  (bind _radius (Variables|Default|GetRadius))
  (bind _stackingradius (Variables|Default|GetStackingRadius))
  (bind _stacks (Variables|Default|Getstacks))
  (bind _returnvalue (* _stacks _stackingradius))
  (bind _returnvalue_2 (+ _returnvalue _radius))
  (bind _returnvalue_3 (Class|ModBase|GetActorsOfClassInternal "/Game/BPs/AI/Grunt/BP_Grunt.BP_Grunt_C"))
  (for _array_element _returnvalue_3
    (Development|PrintString world (Utilities|String|ToString(Float) (/ (Math|Vector|VectorLength (- (Transformation|GetActorLocation _array_element) (Transformation|GetActorLocation hitActor))) _returnvalue_2)))
    (if (< (Math|Vector|VectorLength (- (Transformation|GetActorLocation _array_element) (Transformation|GetActorLocation hitActor))) _returnvalue_2)
      (bind _returnvalue_4 (Class|ModBase|GetActorOfClassInternal "/Game/BPs/BP_Gun.BP_Gun_C"))
      (bind _asgun (Utilities|Casting|CastToGun _returnvalue_4))
      (Class|Gun|OnHitCallbackwithSkip _asgun _array_element (Variables|Default|Getname)))))