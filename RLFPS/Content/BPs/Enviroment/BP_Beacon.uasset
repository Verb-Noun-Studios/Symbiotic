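; BP_Beacon is an interactable beacon that rewards a weapon mod once its event is complete.
; A world widget shows the mod's name, rotates toward the player each tick and switches panels with event state.
; On use, a completed, activated beacon constructs the mod and replaces BP_Gun's active item; otherwise it plays horde-mode audio.
; An overlap with the gun plays a one-time first-discovery sound via GM_Sym, except on tutorial beacons.
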(event OnComponentBeginOverlap(Sphere)
  (params (OverlappedComponent :type Primitive%20Component%20Object%20Reference) (OtherActor :type Actor%20Object%20Reference) (OtherComp :type Primitive%20Component%20Object%20Reference) (OtherBodyIndex :type Integer) (bFromSweep :type Boolean) (SweepResult :type Hit%20Result%20Structure%20%28by%20ref%29))
  (Utilities|Casting|CastToBP_Gun OtherActor)
  (if (not (Variables|Default|GetisForTutorial))
    (bind _asgm_sym (Utilities|Casting|CastToGM_Sym (Game|GetGameMode)))
    (if (not (Variables|/Script/RLFPS.SymbioticGameMode|GetfirstBeaconFound _asgm_sym))
      (Variables|/Script/RLFPS.SymbioticGameMode|SetfirstBeaconFound _asgm_sym true)
      (Audio|PlaySound2D "/Game/Audio/FergusonVoiceLines/A_FirstBeacon.A_FirstBeacon" 1.0 1.0 0.0 0 0))))

(event EventBeginPlay
  (bind _aswbp_beacon_main (Utilities|Casting|CastToWBP_BeaconMain (UserInterface|GetWidget (Variables|Default|GetWidget))))
  (Appearance|SetBrushfromTexture (Variables|/Game/Widgets/Beacon/WBP_BeaconMain.WBP_BeaconMain_C|GetImage_61 _aswbp_beacon_main) 0 false)
  (Rendering|Components|TextRender|SetText (Variables|/Game/Widgets/Beacon/WBP_BeaconMain.WBP_BeaconMain_C|GetTextBlock_60 _aswbp_beacon_main) (Utilities|Text|ToText(String) (Utilities|String|ToString(Name) (.name (Utilities|GetClassDefaults (Variables|Default|GetnewMod)))))))

(event Collision|EventActorBeginOverlap
  (params (OtherActor :type Actor%20Object%20Reference)))

(event EventTick
  (params (DeltaSeconds :type Float%20%28single-precision%29))
  (bind _returnvalue (Actor|GetActorOfClass "/Game/BPs/BP_FPSPlayer.BP_FPSPlayer_C"))
  (Transformation|SetWorldRotation (Variables|Default|GetWidget) (Math|Rotator|FindLookatRotation (Transformation|GetActorLocation) (Transformation|GetActorLocation _returnvalue)) false false)
  (if (and (not (Variables|Default|GetmodCollected)) (Variables|Default|GeteventComplete))
    (bind _aswbp_beacon_main (Utilities|Casting|CastToWBP_BeaconMain (UserInterface|GetWidget (Variables|Default|GetWidget))))
    (if (!= (Class|WidgetSwitcher|GetActiveWidgetIndex (Variables|/Game/Widgets/Beacon/WBP_BeaconMain.WBP_BeaconMain_C|GetWidgetSwitcher_21 _aswbp_beacon_main)) 2)
      (Class|WidgetSwitcher|SetActiveWidgetIndex (Variables|/Game/Widgets/Beacon/WBP_BeaconMain.WBP_BeaconMain_C|GetWidgetSwitcher_21 _aswbp_beacon_main) 2))))

(event EventPlayActivationSound
  (Audio|PlaySound2D 0 1.0 1.0 0.0 0 0))

(event EventRecieveonUse
  (if (and (Variables|Default|GeteventComplete) (Variables|Default|Getactivated))
    (bind _returnvalue (Game|ConstructObjectfromClass (Variables|Default|GetnewMod) self))
    (bind _returnvalue_2 (Actor|GetActorOfClass "/Game/BPs/BP_Gun.BP_Gun_C"))
    (Class|Gun|ReplaceActiveItem _returnvalue_2 _returnvalue)
    (bind _aswbp_beacon_main (Utilities|Casting|CastToWBP_BeaconMain (UserInterface|GetWidget (Variables|Default|GetWidget))))
    (Class|WidgetSwitcher|SetActiveWidgetIndex (Variables|/Game/Widgets/Beacon/WBP_BeaconMain.WBP_BeaconMain_C|GetWidgetSwitcher_21 _aswbp_beacon_main))
    (Variables|Default|SetmodCollected true)
    (else
      (bind _aswbp_beacon_main_2 (Utilities|Casting|CastToWBP_BeaconMain (UserInterface|GetWidget (Variables|Default|GetWidget))))
      (Class|WidgetSwitcher|SetActiveWidgetIndex (Variables|/Game/Widgets/Beacon/WBP_BeaconMain.WBP_BeaconMain_C|GetWidgetSwitcher_21 _aswbp_beacon_main_2))
      (Audio|PlaySound2D "/Game/Audio/FergusonVoiceLines/A_HordeMode.A_HordeMode" 1.0 1.0 0.0 0 0))))

(fn ConstructionScript)