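; BP_RockDrip is an environment actor that repeatedly drops rock debris from its position.
; On BeginPlay it loops forever, calling Drip and then waiting a random delay between DelayMin and DelayMax.
; Each Drip spawns a BP_DebrisFull at the root transform, sets its rock scale and dust particle size, and sets its SpawnDebris flag to false.
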(event Custom|Drip
  (bind _returnvalue (Game|SpawnActorfromClass "/Game/Art/Meshes/LevelProps/BossRoom/Debris/BP_DebrisFull.BP_DebrisFull_C" (Transformation|GetWorldTransform (Variables|Default|GetDefaultSceneRoot)) "Undefined" 0 0))
  (Transformation|SetWorldScale3D (Variables|/Game/Art/Meshes/LevelProps/BossRoom/Debris/BP_DebrisFull.BP_DebrisFull_C|Getrock3 _returnvalue) (Variables|Default|GetrockScale))
  (Variables|/Game/Art/Meshes/LevelProps/BossRoom/Debris/BP_DebrisFull.BP_DebrisFull_C|SetpartScale _returnvalue (Variables|Default|GetdustSize))
  (Variables|/Game/Art/Meshes/LevelProps/BossRoom/Debris/BP_DebrisFull.BP_DebrisFull_C|SetspawnDebris _returnvalue false))

(event EventBeginPlay
  (CallFunction|Drip :!label _label)
  (Utilities|FlowControl|Delay (Math|Random|RandomFloatinRange (Variables|Default|GetdelayMin) (Variables|Default|GetdelayMax)))
  (goto _label))

(fn ConstructionScript)