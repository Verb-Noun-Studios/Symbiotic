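; BP_PortalEnd is a level exit portal that opens LevelToLoad when BP_FPSPlayer overlaps its box and no "Boss"-tagged actors remain.
; Each Tick, it checks whether the TriggerBox_Blueprint room has started and all bosses are gone.
; When both hold, a DoOnce, reset on BeginPlay, activates the Niagara effect and sets the escape title text if the player's health is nonzero.
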(event OnComponentBeginOverlap(Box)
  (params (OverlappedComponent :type Primitive%20Component%20Object%20Reference) (OtherActor :type Actor%20Object%20Reference) (OtherComp :type Primitive%20Component%20Object%20Reference) (OtherBodyIndex :type Integer) (bFromSweep :type Boolean) (SweepResult :type Hit%20Result%20Structure%20%28by%20ref%29))
  (Utilities|Casting|CastToBP_FPSPlayer OtherActor)
  (bind _outactors (Actor|GetAllActorswithTag "Boss"))
  (if (== (Utilities|Array|Length _outactors) 0)
    (Game|OpenLevel(byName) (Variables|Default|GetLevelToLoad))))

(event EventBeginPlay
  (Utilities|FlowControl|DoOnce false) ; enters at Reset
)

(event EventTick
  (params (DeltaSeconds :type Float%20%28single-precision%29))
  (bind _returnvalue (Actor|GetActorOfClass "/Game/Art/Meshes/LevelProps/BossRoom/TriggerBox_Blueprint.TriggerBox_Blueprint_C"))
  (if (Utilities|IsValid _returnvalue)
    (if (Variables|/Game/Art/Meshes/LevelProps/BossRoom/TriggerBox_Blueprint.TriggerBox_Blueprint_C|GetRoomStarted _returnvalue)
      (bind _outactors (Actor|GetAllActorswithTag "Boss"))
      (if (== (Utilities|Array|Length _outactors) 0)
        (Utilities|FlowControl|DoOnce false
          (:Completed
            (bind _returnvalue_2 (Actor|GetActorOfClass "/Game/BPs/BP_FPSPlayer.BP_FPSPlayer_C"))
            (if (!= (Variables|/Script/RLFPS.HealthComponent|GetcurrentHealth (Variables|/Script/RLFPS.FragPlayer|GetHealthComponent _returnvalue_2)) 0.0)
              (Components|Activation|SetActive (Variables|Default|GetNiagara) true false)
              (Rendering|Components|TextRender|SetText (Variables|Default|GetTitle) (Variables|Default|GetEscapeTxt)))))))))

(fn ConstructionScript)