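; BP_RemoveFloor is a tutorial floor tile that collapses when the player steps into its trigger box.
; On overlap by BP_FPSPlayer, it finds every BP_RemoveFloor with a matching SequenceNumber and calls Break, so grouped tiles fall together.
; Break swaps the intact floor mesh for a spawned BP_BrokenFloor at the same transform with impulse off and two pieces' velocity zeroed, then removes the trigger.
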(event OnComponentBeginOverlap(Box)
  (params (OverlappedComponent :type Primitive%20Component%20Object%20Reference) (OtherActor :type Actor%20Object%20Reference) (OtherComp :type Primitive%20Component%20Object%20Reference) (OtherBodyIndex :type Integer) (bFromSweep :type Boolean) (SweepResult :type Hit%20Result%20Structure%20%28by%20ref%29))
  (Utilities|Casting|CastToBP_FPSPlayer OtherActor)
  (bind _outactors (Actor|GetAllActorsOfClass "BP_RemoveFloor_C"))
  (for _array_element _outactors
    (if (== (Variables|Default|GetsequenceNumber) (Variables|BP_RemoveFloor_C|GetsequenceNumber _array_element))
      (CallFunction|Break _array_element))))

(event EventBeginPlay)

(event Collision|EventActorBeginOverlap
  (params (OtherActor :type Actor%20Object%20Reference)))

(event EventTick
  (params (DeltaSeconds :type Float%20%28single-precision%29)))

(fn ConstructionScript)

(fn Break
  (bind _s_floorpiece1_01 (Variables|Default|GetS_FloorPiece1_01))
  (Variables|Default|SetfloorTrans (Transformation|GetWorldTransform _s_floorpiece1_01))
  (Components|DestroyComponent _s_floorpiece1_01)
  (bind _returnvalue (Game|SpawnActorfromClass "/Game/Art/Meshes/NEWModularPieces/BrokenFloor/BP_BrokenFloor.BP_BrokenFloor_C" (Variables|Default|GetfloorTrans) "Undefined" 0 0))
  (Variables|/Game/Art/Meshes/NEWModularPieces/BrokenFloor/BP_BrokenFloor.BP_BrokenFloor_C|SetaddImpulse _returnvalue false)
  (Class|PrimitiveComponent|SetAllPhysicsLinearVelocity (Variables|/Game/Art/Meshes/NEWModularPieces/BrokenFloor/BP_BrokenFloor.BP_BrokenFloor_C|Getfloor_brocken_polySurface4 _returnvalue) "0, 0, 0" false)
  (Components|DestroyComponent (Variables|Default|GetBox)))