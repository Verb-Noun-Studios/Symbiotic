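; BP_Doorway is a tutorial environment door that opens when its Button component is shot by a BP_Bullet.
; On BeginPlay it stores its location as the start point and a point 700 units lower as the end point.
; A bullet overlap destroys the bullet and, only the first time, swaps the button material, removes the button's Niagara effect and plays a timeline that lerps the whole actor downward.
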(event OnComponentBeginOverlap(button)
  (params (OverlappedComponent :type Primitive%20Component%20Object%20Reference) (OtherActor :type Actor%20Object%20Reference) (OtherComp :type Primitive%20Component%20Object%20Reference) (OtherBodyIndex :type Integer) (bFromSweep :type Boolean) (SweepResult :type Hit%20Result%20Structure%20%28by%20ref%29))
  (Utilities|Casting|CastToBP_Bullet OtherActor)
  (Actor|DestroyActor OtherActor)
  (if (not (Variables|Default|Getactivated))
    (Variables|Default|Setactivated true)
    (Rendering|Material|SetMaterial (Variables|Default|Getbutton) 0 "/Game/Art/Meshes/TutorialProps/MI_PushedEmissive_Inst.MI_PushedEmissive_Inst")
    (Components|DestroyComponent (Variables|Default|Getns_button))
    (bind _alpha (Timeline|Timeline_0 Play)
      (:Update
        (Transformation|SetActorLocation (Math|Vector|Lerp(Vector) (Variables|Default|GetStartPoint) (Variables|Default|GetEndPoint) _alpha) false false)))))

(event EventBeginPlay
  (bind _returnvalue (Transformation|GetActorLocation))
  (Transformation|SetActorLocation (Transformation|GetActorLocation) false false)
  (Variables|Default|SetStartPoint (Transformation|GetActorLocation))
  (Variables|Default|SetEndPoint (Math|Vector|MakeVector (.x _returnvalue) (.y _returnvalue) (- (.z _returnvalue) 7e+02))))

(event Collision|EventActorBeginOverlap
  (params (OtherActor :type Actor%20Object%20Reference)))

(event EventTick
  (params (DeltaSeconds :type Float%20%28single-precision%29)))

(fn ConstructionScript)