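; Sliding double doorway that gates a spawner room as either an entrance or an exit.
; Box overlaps by the player or a Gun toggle ShouldbeOpen on entry, and player exit toggles it back.
; An entrance works only before its Spawner activates or clears, activating it when the player leaves the box; exits require RoomCleared.
; Tick offsets both panels oppositely by OpennessValue, which this graph never updates.
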(event OnComponentBeginOverlap(Box)
  (params (OverlappedComponent :type Primitive%20Component%20Object%20Reference) (OtherActor :type Actor%20Object%20Reference) (OtherComp :type Primitive%20Component%20Object%20Reference) (OtherBodyIndex :type Integer) (bFromSweep :type Boolean) (SweepResult :type Hit%20Result%20Structure%20%28by%20ref%29))
  (bind _spawner (Variables|Default|Getspawner))
  (bind _roomcleared (Variables|/Script/RLFPS.EnemySpawner|GetroomCleared _spawner))
  (if (not (Variables|Default|GetshouldbeOpen))
    (if (Variables|Default|GetEntrance)
      (if (not (Variables|/Script/RLFPS.EnemySpawner|Getactivated _spawner))
        (if (not _roomcleared)
          (Utilities|Casting|CastToGun OtherActor :!label _label
            (:then
              _)
            (:CastFailed
              (Utilities|Casting|CastToBP_FPSPlayer OtherActor)))
          (Variables|Default|SetshouldbeOpen (not (Variables|Default|GetshouldbeOpen)))
          (Development|PrintString (Utilities|GetDisplayName OtherActor))))
      (elif _roomcleared
        (goto _label)))))

(event OnComponentEndOverlap(Box)
  (params (OverlappedComponent :type Primitive%20Component%20Object%20Reference) (OtherActor :type Actor%20Object%20Reference) (OtherComp :type Primitive%20Component%20Object%20Reference) (OtherBodyIndex :type Integer))
  (bind _spawner (Variables|Default|Getspawner))
  (bind _roomcleared (Variables|/Script/RLFPS.EnemySpawner|GetroomCleared _spawner))
  (if (Variables|Default|GetEntrance)
    (if (and (not (Variables|/Script/RLFPS.EnemySpawner|Getactivated _spawner)) (not _roomcleared))
      (Utilities|Casting|CastToBP_FPSPlayer OtherActor)
      (Variables|Default|SetshouldbeOpen (not (Variables|Default|GetshouldbeOpen)))
      (Variables|/Script/RLFPS.EnemySpawner|Setactivated (Variables|Default|Getspawner) true))
    (elif _roomcleared
      (Utilities|Casting|CastToBP_FPSPlayer OtherActor)
      (Variables|Default|SetshouldbeOpen (not (Variables|Default|GetshouldbeOpen))))))

(event EventBeginPlay)

(event Collision|EventActorBeginOverlap
  (params (OtherActor :type Actor%20Object%20Reference)))

(event EventTick
  (params (DeltaSeconds :type Float%20%28single-precision%29))
  (Transformation|SetRelativeLocation (Variables|Default|GetRightSide) (+ (Math|Vector|MakeVector (* (Variables|Default|GetopennessValue) (Variables|Default|GetSlideOffset)) 0.0 0.0) "85.913055, 0, 0") false false)
  (Transformation|SetRelativeLocation (Variables|Default|GetLeftSide) (+ (Math|Vector|MakeVector (* (Variables|Default|GetopennessValue) (* (Variables|Default|GetSlideOffset) -1.0)) 0.0 0.0) "-85.913055, 0, 0") false false))

(fn ConstructionScript)