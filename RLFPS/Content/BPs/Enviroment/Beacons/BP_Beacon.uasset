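; BP_Beacon is an environment beacon that presents a mod through a widget.
; On BeginPlay it fills the WBP_BeaconMain widget with the image and name from the NewMod class defaults.
; When a BP_Gun overlaps its sphere on a non-tutorial beacon, it sets the GM_Sym first-found flag and plays a one-time discovery sound.
; A separate PlayActivationSound event plays a 2D sound, with no sound asset shown.
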(event OnComponentBeginOverlap(Sphere)
  (params (OverlappedComponent :type Primitive%20Component%20Object%20Reference) (OtherActor :type Actor%20Object%20Reference) (OtherComp :type Primitive%20Component%20Object%20Reference) (OtherBodyIndex :type Integer) (bFromSweep :type Boolean) (SweepResult :type Hit%20Result%20Structure%20%28by%20ref%29))
  (Utilities|Casting|CastToBP_Gun OtherActor)
  (if (not (Variables|Default|GetisForTutorial))
    (bind _asgm_sym (Utilities|Casting|CastToGM_Sym (Game|GetGameMode)))
    (if (not (Variables|/Script/RLFPS.SymbioticGameMode|GetfirstBeaconFound _asgm_sym))
      (Variables|/Script/RLFPS.SymbioticGameMode|SetfirstBeaconFound _asgm_sym true)
      (Audio|PlaySound2D "/Game/Audio/FergusonVoiceLines/A_FirstBeacon.A_FirstBeacon" 1.0 1.0 0.0 0 0))))

(event EventBeginPlay
  (bind _newmod (Variables|Default|GetnewMod))
  (bind (_name _type _image) (Utilities|GetClassDefaults _newmod))
  (bind _aswbp_beacon_main (Utilities|Casting|CastToWBP_BeaconMain (UserInterface|GetWidget (Variables|Default|GetWidget))))
  (Appearance|SetBrushfromTexture (Variables|/Game/Widgets/Beacon/WBP_BeaconMain.WBP_BeaconMain_C|GetImage_61 _aswbp_beacon_main) _image false)
  (Rendering|Components|TextRender|SetText (Variables|/Game/Widgets/Beacon/WBP_BeaconMain.WBP_BeaconMain_C|GetTextBlock_60 _aswbp_beacon_main) (Utilities|Text|ToText(String) (Utilities|String|ToString(Name) _name))))

(event EventPlayActivationSound
  (Audio|PlaySound2D 0 1.0 1.0 0.0 0 0))

(fn ConstructionScript)