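; Spawn beacon Blueprint that adds a Niagara effect to the activate and deactivate events inherited from its parent beacon.
; Activation calls the parent event, then spawns the active-beacon system at the bottom mesh's location and stores it.
; Deactivation also calls the parent's activate event, not a deactivate one, then deactivates the effect and destroys it after a short delay.
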(event EventBeginPlay)

(event Collision|EventActorBeginOverlap
  (params (OtherActor :type Actor%20Object%20Reference)))

(event EventOnBeaconActivate
  (|CallParentFunction)
  (bind _returnvalue (Niagara|SpawnSystematLocation "/Game/Art/FX/BeaconActive/NE_BeaconActive_System.NE_BeaconActive_System" (Transformation|GetWorldLocation (Variables|Default|GetMeshBottom))))
  (Variables|Default|Setfx _returnvalue))

(event EventOnBeaconDeactivate
  (bind _fx (Variables|Default|Getfx))
  (|CallParentFunction)
  (Components|Activation|Deactivate _fx)
  (Utilities|FlowControl|Delay 3.0)
  (Components|DestroyComponent _fx))

(fn ConstructionScript)