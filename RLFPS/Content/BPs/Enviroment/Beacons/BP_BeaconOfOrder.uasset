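; Beacon of Order is a usable beacon that rerolls the mods on the player's BP_Gun while preserving their count per rarity.
; Use tallies mod stacks by rarity, then repeatedly calls GetNewModOptions until the first option matches each needed rarity.
; It then clears the gun's mods, constructs and adds the collected classes, and resets its working data.
; Debug prints show per-rarity counts before and after.
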(event EventBeginPlay
  (|CallParentFunction) ; This node is disabled and will not be called.\nDrag off pins to build functionality.
)

(event Collision|EventActorBeginOverlap
  (params (OtherActor :type Actor%20Object%20Reference)))

(event EventTick
  (params (DeltaSeconds :type Float%20%28single-precision%29))
  (|CallParentFunction DeltaSeconds) ; This node is disabled and will not be called.\nDrag off pins to build functionality.
)

(event EventUse
  (if (stale _output_get)
    _
    (else
      _))
  (bind _output_get (Variables|Default|SetUsed true))
  (bind _returnvalue (Actor|GetActorOfClass "/Game/BPs/BP_Gun.BP_Gun_C"))
  (for _array_element (Variables|/Script/RLFPS.Gun|Getmods _returnvalue)
    (if (== (Variables|/Script/RLFPS.ModBase|Getrarity _array_element) 0)
      (Variables|Default|SetCommon (+ (Variables|Default|GetCommon) (Variables|/Script/RLFPS.ModBase|Getstacks _array_element)))
      (elif (== (Variables|/Script/RLFPS.ModBase|Getrarity _array_element) 1)
        (Variables|Default|SetUncommon (+ (Variables|Default|GetUncommon) (Variables|/Script/RLFPS.ModBase|Getstacks _array_element)))
        (elif (== (Variables|/Script/RLFPS.ModBase|Getrarity _array_element) 2)
          (Variables|Default|SetRare (+ (Variables|Default|GetRare) (Variables|/Script/RLFPS.ModBase|Getstacks _array_element)))
          (elif (== (Variables|/Script/RLFPS.ModBase|Getrarity _array_element) 3)
            (Variables|Default|SetMythic (+ (Variables|Default|GetMythic) (Variables|/Script/RLFPS.ModBase|Getstacks _array_element))))))))
  (Development|PrintString (Utilities|String|Append "Common: " (Utilities|String|ToString(Integer) (Variables|Default|GetCommon)) " Uncommon: " (Utilities|String|ToString(Integer) (Variables|Default|GetUncommon)) " Rare: " (Utilities|String|ToString(Integer) (Variables|Default|GetRare)) "Mythic" (Utilities|String|ToString(Integer) (Variables|Default|GetMythic))))
  (if (> (Variables|Default|GetCommon) 0)
    (for _index (range 0 (- (Variables|Default|GetCommon) 1))
      (while (not (Variables|Default|GetcorrectRarity))
        (bind _returnvalue_2 (Class|Gun|GetNewModOptions _returnvalue))
        (bind _output_get_2 (Variables|Default|SetMod (Utilities|Array|Get(acopy) _returnvalue_2)))
        (Variables|Default|SetcorrectRarity (== (Variables|/Script/RLFPS.ModBase|Getrarity _output_get_2) 0)))
      (Utilities|Array|Add (Variables|Default|GetMods%20Common) (Utilities|GetClass (Variables|Default|GetMod)))
      (Variables|Default|SetcorrectRarity false)))
  (if (> (Variables|Default|GetUncommon) 0)
    (for _index_2 (range 0 (- (Variables|Default|GetUncommon) 1))
      (while (not (Variables|Default|GetcorrectRarity))
        (bind _returnvalue_3 (Class|Gun|GetNewModOptions _returnvalue))
        (Variables|Default|SetMod (Utilities|Array|Get(acopy) _returnvalue_3))
        (Variables|Default|SetcorrectRarity (== (Variables|/Script/RLFPS.ModBase|Getrarity (Utilities|Array|Get(acopy) _returnvalue_3)) 1)))
      (Utilities|Array|Add (Variables|Default|GetMods%20Uncommon) (Utilities|GetClass (Variables|Default|GetMod)))
      (Variables|Default|SetcorrectRarity false)))
  (if (> (Variables|Default|GetRare) 0)
    (for _index_3 (range 0 (- (Variables|Default|GetRare) 1))
      (while (not (Variables|Default|GetcorrectRarity))
        (bind _returnvalue_4 (Class|Gun|GetNewModOptions _returnvalue))
        (Variables|Default|SetMod (Utilities|Array|Get(acopy) _returnvalue_4))
        (Variables|Default|SetcorrectRarity (== (Variables|/Script/RLFPS.ModBase|Getrarity (Utilities|Array|Get(acopy) _returnvalue_4)) 2)))
      (Utilities|Array|Add (Variables|Default|GetMods%20Rare) (Utilities|GetClass (Variables|Default|GetMod)))
      (Variables|Default|SetcorrectRarity false)))
  (if (> (Variables|Default|GetMythic) 0)
    (for _index_4 (range 0 (- (Variables|Default|GetMythic) 1))
      (while (not (Variables|Default|GetcorrectRarity))
        (bind _returnvalue_5 (Class|Gun|GetNewModOptions _returnvalue))
        (Variables|Default|SetMod (Utilities|Array|Get(acopy) _returnvalue_5))
        (Variables|Default|SetcorrectRarity (== (Variables|/Script/RLFPS.ModBase|Getrarity (Utilities|Array|Get(acopy) _returnvalue_5)) 3)))
      (Utilities|Array|Add (Variables|Default|GetMods%20Mythic) (Utilities|GetClass (Variables|Default|GetMod)))
      (Variables|Default|SetcorrectRarity false)))
  (Utilities|Array|Clear (Variables|/Script/RLFPS.Gun|Getmods _returnvalue))
  (for _array_element_2 (Variables|Default|GetMods%20Common)
    (bind _returnvalue_6 (Game|ConstructObjectfromClass _array_element_2 _returnvalue))
    (Class|Gun|AddMod _returnvalue _returnvalue_6))
  (for _array_element_3 (Variables|Default|GetMods%20Uncommon)
    (bind _returnvalue_7 (Game|ConstructObjectfromClass _array_element_3 _returnvalue))
    (Class|Gun|AddMod _returnvalue _returnvalue_7)
    (Variables|Default|SetNew%20Mods (+ (Variables|Default|GetNew%20Mods) 1)))
  (for _array_element_4 (Variables|Default|GetMods%20Rare)
    (bind _returnvalue_8 (Game|ConstructObjectfromClass _array_element_4 _returnvalue))
    (Class|Gun|AddMod _returnvalue _returnvalue_8)
    (Variables|Default|SetNew%20Mods (+ (Variables|Default|GetNew%20Mods) 1)))
  (for _array_element_5 (Variables|Default|GetMods%20Mythic)
    (bind _returnvalue_9 (Game|ConstructObjectfromClass _array_element_5 _returnvalue))
    (Class|Gun|AddMod _returnvalue _returnvalue_9))
  (Development|PrintString (Utilities|String|Append "Common: " (Utilities|String|ToString(Integer) (Utilities|Array|Length (Variables|Default|GetMods%20Common))) " Uncommon: " (Utilities|String|ToString(Integer) (Utilities|Array|Length (Variables|Default|GetMods%20Uncommon))) " Rare: " (Utilities|String|ToString(Integer) (Utilities|Array|Length (Variables|Default|GetMods%20Rare))) "Mythic" (Utilities|String|ToString(Integer) (Utilities|Array|Length (Variables|Default|GetMods%20Mythic)))))
  (Variables|Default|SetCommon 0)
  (Variables|Default|SetUncommon 0)
  (Variables|Default|SetRare 0)
  (Variables|Default|SetMythic 0)
  (Utilities|Array|Clear (Variables|Default|GetMods%20Common))
  (Utilities|Array|Clear (Variables|Default|GetMods%20Uncommon))
  (Utilities|Array|Clear (Variables|Default|GetMods%20Rare))
  (Utilities|Array|Clear (Variables|Default|GetMods%20Mythic)))

(fn ConstructionScript
  (|CallParentFunction))