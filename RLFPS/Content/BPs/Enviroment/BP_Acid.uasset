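; BP_Acid is an acid hazard that damages the FPS player while they are inside its Box volume.
; Box overlap begin stores the BP_FPSPlayer reference and applies damage immediately, and overlap end clears the reference.
; While the reference is valid, Tick applies DamagePerTick every frame without delta-time scaling, so the damage rate depends on frame rate.
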(event OnComponentBeginOverlap(Box)
  (params (OverlappedComponent :type Primitive%20Component%20Object%20Reference) (OtherActor :type Actor%20Object%20Reference) (OtherComp :type Primitive%20Component%20Object%20Reference) (OtherBodyIndex :type Integer) (bFromSweep :type Boolean) (SweepResult :type Hit%20Result%20Structure%20%28by%20ref%29))
  (bind _asbp_fpsplayer (Utilities|Casting|CastToBP_FPSPlayer OtherActor))
  (bind _output_get (Variables|Default|SetPlayer _asbp_fpsplayer))
  (Game|Damage|ApplyDamage _output_get (Variables|Default|GetdamagePerTick) 0 self))

(event OnComponentEndOverlap(Box)
  (params (OverlappedComponent :type Primitive%20Component%20Object%20Reference) (OtherActor :type Actor%20Object%20Reference) (OtherComp :type Primitive%20Component%20Object%20Reference) (OtherBodyIndex :type Integer))
  (Utilities|Casting|CastToBP_FPSPlayer OtherActor)
  (Variables|Default|SetPlayer 0))

(event EventBeginPlay)

(event EventTick
  (params (DeltaSeconds :type Float%20%28single-precision%29))
  (if (Utilities|IsValid (Variables|Default|GetPlayer))
    (Game|Damage|ApplyDamage (Variables|Default|GetPlayer) (Variables|Default|GetdamagePerTick) 0 self)))

(fn ConstructionScript)