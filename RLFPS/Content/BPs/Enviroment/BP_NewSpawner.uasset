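; Room enemy spawner that links itself to its Entrance and Exit doorways and marks the room cleared once the kill quota is met.
; While inactive, Tick recomputes that quota from FirstRoomKills plus the square root of the Gun's TotalEXP.
; SpawnEnemy spawns a random enemy type on navmesh within its box, gated by out-of-view or line-trace-hit tests.
; The random point is re-rolled between test and spawn, so the tested location differs.
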(event EventBeginPlay
  (bind _asbp_doorway (Utilities|Casting|CastToBP_Doorway (Variables|/Script/Engine.ChildActorComponent|GetChildActor (Variables|Default|GetExit_))))
  (Variables|/Script/RLFPS.Doorway|Setspawner _asbp_doorway self)
  (bind _asbp_doorway_2 (Utilities|Casting|CastToBP_Doorway (Variables|/Script/Engine.ChildActorComponent|GetChildActor (Variables|Default|GetEntrance))))
  (Variables|/Script/RLFPS.Doorway|Setspawner _asbp_doorway_2 self))

(event Collision|EventActorBeginOverlap
  (params (OtherActor :type Actor%20Object%20Reference)))

(event EventTick
  (params (DeltaSeconds :type Float%20%28single-precision%29))
  (if (>= (Variables|Default|GetemnemiesKilled) (Variables|Default|GetKillsRequired))
    (Variables|Default|Setactivated false)
    (Variables|Default|SetroomCleared true)
    (elif (not (Variables|Default|Getactivated))
      (bind _returnvalue (Actor|GetActorOfClass "/Script/RLFPS.Gun"))
      (if (<= (Variables|/Script/RLFPS.Gun|GettotalEXP _returnvalue) 0)
        (bind _output_get (Variables|Default|SetKillsRequired (Variables|Default|GetFirstRoomKills)))
        (Development|PrintString (Utilities|String|ToString(Integer) _output_get))
        (else
          (bind _output_get_2 (Variables|Default|SetKillsRequired (+ (Math|Conversions|ToInteger(Byte) (Class|KismetMathLibrary|FTrunc64 (Math|Float|Sqrt (Math|Conversions|ToFloat(Integer) (Variables|/Script/RLFPS.Gun|GettotalEXP _returnvalue))))) (Variables|Default|GetFirstRoomKills))))
          (Development|PrintString (Utilities|String|ToString(Integer) _output_get_2)))))))

(fn ConstructionScript)

(fn SpawnEnemy
  (bind _returnvalue (Transformation|GetActorLocation))
  (bind _boxsize (Variables|Default|GetBoxSize))
  (bind _enemytypes (Variables|Default|GetEnemyTypes))
  (bind _returnvalue_2 (Math|Random|RandomPointinBoundingBox _returnvalue _boxsize))
  (bind _randomlocation (Class|NavigationSystemV1|GetRandomPointinNavigableRadius _returnvalue_2 2e+01 0 0))
  (bind _returnvalue_3 (Actor|GetActorOfClass "/Game/BPs/BP_FPSPlayer.BP_FPSPlayer_C"))
  (Development|PrintString (Utilities|String|Append (Utilities|String|ToString(Float) (* (Math|Trig|Acos(Degrees) (/ (Math|Vector|DotProduct (Math|Vector|Normalize (Math|Vector|GetForwardVector (Variables|/Script/RLFPS.FragPlayer|GetFirstPersonCameraComponent _returnvalue_3))) (Math|Vector|Normalize (- _randomlocation (Transformation|GetWorldLocation (Variables|/Script/RLFPS.FragPlayer|GetFirstPersonCameraComponent _returnvalue_3))))) (* (Math|Vector|VectorLength (Math|Vector|Normalize (- _randomlocation (Transformation|GetWorldLocation (Variables|/Script/RLFPS.FragPlayer|GetFirstPersonCameraComponent _returnvalue_3))))) (Math|Vector|VectorLength (Math|Vector|Normalize (Math|Vector|GetForwardVector (Variables|/Script/RLFPS.FragPlayer|GetFirstPersonCameraComponent _returnvalue_3))))))) (/ 1.8e+02 3.14159))) "   >  " (Utilities|String|ToString(Float) (/ (+ (Variables|/Script/Engine.CameraComponent|GetFieldOfView (Variables|/Script/RLFPS.FragPlayer|GetFirstPersonCameraComponent _returnvalue_3)) 15.0) 2.0))))
  (if (> (* (Math|Trig|Acos(Degrees) (/ (Math|Vector|DotProduct (Math|Vector|Normalize (Math|Vector|GetForwardVector (Variables|/Script/RLFPS.FragPlayer|GetFirstPersonCameraComponent _returnvalue_3))) (Math|Vector|Normalize (- _randomlocation (Transformation|GetWorldLocation (Variables|/Script/RLFPS.FragPlayer|GetFirstPersonCameraComponent _returnvalue_3))))) (* (Math|Vector|VectorLength (Math|Vector|Normalize (- _randomlocation (Transformation|GetWorldLocation (Variables|/Script/RLFPS.FragPlayer|GetFirstPersonCameraComponent _returnvalue_3))))) (Math|Vector|VectorLength (Math|Vector|Normalize (Math|Vector|GetForwardVector (Variables|/Script/RLFPS.FragPlayer|GetFirstPersonCameraComponent _returnvalue_3))))))) (/ 1.8e+02 3.14159)) (/ (+ (Variables|/Script/Engine.CameraComponent|GetFieldOfView (Variables|/Script/RLFPS.FragPlayer|GetFirstPersonCameraComponent _returnvalue_3)) 15.0) 2.0))
    (bind _returnvalue_4 (Game|SpawnActorfromClass (Utilities|Array|Get(acopy) _enemytypes (Math|Random|RandomInteger (Utilities|Array|Length _enemytypes))) (Math|Transform|MakeTransform _randomlocation) "AdjustIfPossibleButAlwaysSpawn" 0 0 :!label _label))
    (if (Utilities|IsValid _returnvalue_4)
      (Variables|/Script/RLFPS.GruntCharacter|SetEnemySpawner _returnvalue_4 self))
    (return (Utilities|IsValid _returnvalue_4))
    (else
      (bind _returnvalue_5 (Collision|LineTraceForObjects (Transformation|GetWorldLocation (Variables|/Script/RLFPS.FragPlayer|GetFirstPersonCameraComponent _returnvalue_3)) _randomlocation (LocalVariables|GetNewLocalVar_0) false (Utilities|Array|MakeArray _returnvalue_3) "ForDuration" false))
      (if _returnvalue_5
        (goto _label)))))