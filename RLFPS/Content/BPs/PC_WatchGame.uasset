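; PC_WatchGame is a player controller that handles the pause menu toggle for the first-person player.
; On BeginPlay it casts the player pawn to BP_FPSPlayer and caches it.
; The PauseGame input flips that character's MenuOpen flag, switching the mouse cursor and input mode between game only and game and UI.
; It neither pauses the game nor creates a menu widget itself.
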(event EventBeginPlay
  (bind _asbp_fpsplayer (Utilities|Casting|CastToBP_FPSPlayer (Game|Player|GetPlayerPawn 0)))
  (Variables|Default|SetChar _asbp_fpsplayer))

(event EventTick
  (params (DeltaSeconds :type Float%20%28single-precision%29)))

(event Input|ActionEvents|InputActionPauseGame
  (params (Key :type Key%20Structure :default "None"))
  (bind _self self)
  (bind _char (Variables|Default|GetChar))
  (:Pressed
    (if (Variables|/Game/BPs/BP_FPSPlayer.BP_FPSPlayer_C|GetmenuOpen _char)
      (Variables|/Game/BPs/BP_FPSPlayer.BP_FPSPlayer_C|SetmenuOpen _char false)
      (Variables|Default|SetbShowMouseCursor false)
      (Input|SetInputModeGameOnly _self)
      (else
        (Variables|/Game/BPs/BP_FPSPlayer.BP_FPSPlayer_C|SetmenuOpen _char true)
        (Variables|Default|SetbShowMouseCursor true)
        (Input|SetInputModeGameandUI _self 0 "DoNotLock" true)))))

(fn ConstructionScript)