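; Game mode that runs a boss-meter countdown, then opens a portal when it expires.
; BeginPlay derives the duration from the boss EXP requirement and a time factor.
; StartTimer starts the countdown on Tick, which spawns BP_Portal once at the BP_PortalLocActor with a completion sound, while a parallel Delay deactivates all spawners.
; Debug prints remain, and a grunt-cleanup chain is left unconnected.
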(event EventBeginPlay
  ;[1 1 1] Set Timer for Boss Meter
  (Development|PrintString "Hello")
  (Variables|Default|SetbossTime (Math|Conversions|ToFloat(Integer) (/ (Variables|Default|GetEXPRequiredForBoss) (Variables|Default|GetBossTimeFactor)))))

(event EventTick
  (params (DeltaSeconds :type Float%20%28single-precision%29))
  (if (Variables|Default|GetbossActivated)
    (bind _output_get (Variables|Default|SetbossTime (- (Variables|Default|GetbossTime) DeltaSeconds)))
    (Development|PrintString (Utilities|String|ToString(Float) _output_get) true true "(R=0.000000,G=0.660000,B=1.000000,A=1.000000)" 0.0)
    (if (<= _output_get 0.0)
      (if (not (Variables|Default|GetportalSpawned))
        (bind _returnvalue (Actor|GetActorOfClass "/Game/BPs/Enviroment/BP_PortalLocActor.BP_PortalLocActor_C"))
        (Game|SpawnActorfromClass "/Game/BPs/Enviroment/BP_Portal.BP_Portal_C" (Transformation|GetActorTransform _returnvalue) "AdjustIfPossibleButAlwaysSpawn" self 0)
        (Variables|Default|SetportalSpawned true)
        (Audio|PlaySound2D "/Game/Audio/FergusonVoiceLines/A_CompletingBossMeter.A_CompletingBossMeter" 1.0 1.0 0.0 0 0)))))

(event EventStartTimer
  ;[1 1 1] Deactivate spawners after specified duration
  (Variables|Default|SetbossActivated true)
  (Utilities|FlowControl|Delay (Variables|Default|GetbossTime))
  (bind _outactors (Actor|GetAllActorsOfClass "/Game/BPs/Enviroment/BP_Spawner.BP_Spawner_C"))
  (for _array_element _outactors
    (Class|SpawningActor|Deactivate _array_element)))

(fn ConstructionScript)