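; Game mode that runs the boss meter countdown and provides functions for assembling a run from streamed levels.
; After StartTimer, Tick counts down an EXP-derived time, then spawns a portal once at BP_PortalLocActor, while a matching delay deactivates all spawners.
; LevelStream chains hidden corridor and arena level instances at increasing offsets, ending in a boss room.
; CustCulling shows only instances near the player; neither function is called here.
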(event EventBeginPlay
  ;[1 1 1] Set Timer for Boss Meter
  (Development|PrintString "Hello")
  (Variables|Default|SetbossTime (Math|Conversions|ToFloat(Integer) (/ (Variables|Default|GetEXPRequiredForBoss) (Variables|Default|GetBossTimeFactor)))))

(event EventTick
  (params (DeltaSeconds :type Float%20%28single-precision%29))
  (if (Variables|Default|GetbossActivated)
    (bind _output_get (Variables|Default|SetbossTime (- (Variables|Default|GetbossTime) DeltaSeconds)))
    (Development|PrintString (Utilities|String|ToString(Float) _output_get) true true "(R=0.000000,G=0.660000,B=1.000000,A=1.000000)" 0.0)
    (if (<= _output_get 0.0)
      (if (not (Variables|Default|GetportalSpawned))
        (bind _returnvalue (Actor|GetActorOfClass "/Game/BPs/Enviroment/BP_PortalLocActor.BP_PortalLocActor_C"))
        (Game|SpawnActorfromClass "/Game/BPs/Enviroment/BP_Portal.BP_Portal_C" (Transformation|GetActorTransform _returnvalue) "AdjustIfPossibleButAlwaysSpawn" self 0)
        (Variables|Default|SetportalSpawned true)
        (Audio|PlaySound2D "/Game/Audio/FergusonVoiceLines/A_CompletingBossMeter.A_CompletingBossMeter" 1.0 1.0 0.0 0 0)))))

(event EventStartTimer
  ;[1 1 1] Deactivate spawners after specified duration
  (Variables|Default|SetbossActivated true)
  (Utilities|FlowControl|Delay (Variables|Default|GetbossTime))
  (bind _outactors (Actor|GetAllActorsOfClass "/Game/BPs/Enviroment/BP_Spawner.BP_Spawner_C"))
  (for _array_element _outactors
    (Class|SpawningActor|Deactivate _array_element)))

(fn ConstructionScript)

(fn LevelStream
  (bind _levelstoloadcorridors (Variables|Default|GetLevelsToLoadCorridors))
  (bind _levelstoloadcorridors_2 (Variables|Default|GetLevelsToLoadCorridors))
  (bind _arenaoffset (Variables|Default|GetarenaOffset))
  (bind _levelstoloadtier1 (Variables|Default|GetLevelsToLoadTier1))
  (bind _roomtransform (Variables|Default|GetRoomTransform))
  (bind _bossroom (Variables|Default|GetBossRoom))
  (bind _output (Utilities|Array|Get(acopy) _levelstoloadcorridors))
  (bind _output_2 (Utilities|Array|Get(acopy) _levelstoloadtier1))
  (bind _output_3 (Utilities|Array|Get(acopy) _levelstoloadcorridors_2))
  (for _index (range 0 1)
    (CallFunction|LoadLevel (Class|GameplayStatics|GetStreamingLevel _output) (Utilities|String|Append (Utilities|String|ToString(Name) _output) "Level" (Utilities|String|ToString(Float) (Variables|Default|GetLastOffset))) (Math|Transform|MakeTransform (Math|Vector|MakeVector (* (Variables|Default|GetLastOffset) (.x (.location _roomtransform))) (.y (.location _roomtransform)) (.z (.location _roomtransform))) (.rotation _roomtransform) (.scale _roomtransform)))
    (Variables|Default|SetLastOffset (+ (Variables|Default|GetLastOffset) 1.0))
    (CallFunction|LoadLevel (Class|GameplayStatics|GetStreamingLevel _output_2) (Utilities|String|Append (Utilities|String|ToString(Name) _output_2) "Level" (Utilities|String|ToString(Float) (Variables|Default|GetLastOffset))) (Math|Transform|MakeTransform (Math|Vector|MakeVector (* (Variables|Default|GetLastOffset) (.x _arenaoffset)) (.y _arenaoffset) (.z _arenaoffset)) (.rotation _roomtransform) (.scale _roomtransform)))
    (Variables|Default|SetLastOffset (+ (Variables|Default|GetLastOffset) 1.0)))
  (CallFunction|LoadLevel (Class|GameplayStatics|GetStreamingLevel _output_3) (Utilities|String|Append (Utilities|String|ToString(Name) _output_3) "Level" (Utilities|String|ToString(Float) (Variables|Default|GetLastOffset))) (Math|Transform|MakeTransform (Math|Vector|MakeVector (* (Variables|Default|GetLastOffset) (.x (.location _roomtransform))) (.y (.location _roomtransform)) (.z (.location _roomtransform))) (.rotation _roomtransform) (.scale _roomtransform)))
  (Variables|Default|SetLastOffset (+ (Variables|Default|GetLastOffset) 1.0))
  (CallFunction|LoadLevel (Class|GameplayStatics|GetStreamingLevel _bossroom) (Utilities|String|Append (Utilities|String|ToString(Name) _bossroom) "Level" (Utilities|String|ToString(Float) (Variables|Default|GetLastOffset))) (Math|Transform|ComposeTransforms (Math|Transform|MakeTransform (Math|Vector|MakeVector (* (Variables|Default|GetLastOffset) (.x (.location _roomtransform))) (.y (.location _roomtransform)) (.z (.location _roomtransform))) (.rotation _roomtransform) (.scale _roomtransform)) (Math|Conversions|ToTransform(Vector) (Variables|Default|GetbossOffset)))))

(fn LoadLevel
  (params (LevelToStream :type Level%20Streaming%20Object%20Reference) (Name :type String) (OffsetAmount :type Transform))
  (bind _returnvalue (Class|LevelStreaming|CreateInstance LevelToStream Name))
  (Utilities|Array|Add (Variables|Default|GetLevels) _returnvalue)
  (Variables|/Script/Engine.LevelStreaming|SetbShouldBlockOnLoad _returnvalue true)
  (Variables|/Script/Engine.LevelStreaming|SetLevelTransform _returnvalue OffsetAmount)
  (Variables|/Script/Engine.LevelStreaming|SetbShouldBeLoaded _returnvalue true)
  (Variables|/Script/Engine.LevelStreaming|SetbShouldBeVisible _returnvalue false))

(fn CustCulling
  (for _array_element (Variables|Default|GetLevels)
    (if (< (Math|Vector|Distance(Vector) (.location (Variables|/Script/Engine.LevelStreaming|GetLevelTransform _array_element)) (.location (Transformation|GetActorTransform (Game|Player|GetPlayerPawn 0)))) 4e+03)
      (Variables|/Script/Engine.LevelStreaming|SetbShouldBeVisible _array_element true)
      (else
        (Variables|/Script/Engine.LevelStreaming|SetbShouldBeVisible _array_element false)))))