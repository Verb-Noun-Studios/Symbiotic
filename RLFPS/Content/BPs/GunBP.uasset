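; GunBP is a gun Blueprint that triggers the boss sequence once accumulated EXP is high enough.
; On BeginPlay it caches the FPS_Player's first-person camera and the SymGM game mode.
; Every Tick it compares TotalEXP with the game mode's EXPRequiredForBoss and calls StartBossSequence if the sequence has not started.
; The graph contains no firing or EXP-gain logic, and the cached camera is not used here.
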(event EventBeginPlay
  (bind _returnvalue (Actor|GetActorOfClass "/Game/BPs/FPS_Player.FPS_Player_C"))
  (Variables|Default|Setcamera (Variables|/Script/RLFPS.FragPlayer|GetFirstPersonCameraComponent _returnvalue))
  (bind _assym_gm (Utilities|Casting|CastToSymGM (Game|GetGameMode)))
  (Variables|Default|SetGameMode _assym_gm))

(event Collision|EventActorBeginOverlap
  (params (OtherActor :type Actor%20Object%20Reference)))

(event EventTick
  (params (DeltaSeconds :type Float%20%28single-precision%29))
  (bind _gamemode (Variables|Default|GetGameMode))
  (if (and (>= (Variables|Default|GettotalEXP) (Variables|/Script/RLFPS.SymbioticGameMode|GetEXPRequiredForBoss _gamemode)) (not (Variables|/Script/RLFPS.SymbioticGameMode|GetbossSequenceStarted _gamemode)))
    (Class|SymbioticGameMode|StartBossSequence (Variables|Default|GetGameMode))))

(fn ConstructionScript)