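; Crossbow gun Blueprint that shows level progress on the player's weapon and handles shot feedback.
; Construction creates a dynamic material and reads the left-handed setting; Tick applies the material to the player's ExpBar and updates its percent.
; Tick also starts the GM_Sym boss sequence once total EXP reaches the required threshold.
; Events play gunshot audio with optional Niagara muzzle flash, play a first-upgrade sound, and update handedness.
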(event Custom|UpdateControls
  (params (LeftHanded :type Boolean))
  (Variables|Default|SetLeftHanded LeftHanded))

(event EventBeginPlay
  (bind _returnvalue (Actor|GetActorOfClass "/Game/BPs/BP_FPSPlayer.BP_FPSPlayer_C"))
  (Variables|Default|Setcamera (Variables|/Script/RLFPS.FragPlayer|GetFirstPersonCameraComponent _returnvalue))
  (bind _asgm_sym (Utilities|Casting|CastToGM_Sym (Game|GetGameMode)))
  (Variables|Default|SetGameMode _asgm_sym))

(event Collision|EventActorBeginOverlap
  (params (OtherActor :type Actor%20Object%20Reference)))

(event EventTick
  (params (DeltaSeconds :type Float%20%28single-precision%29))
  (bind _gamemode (Variables|Default|GetGameMode))
  (bind _progressbarmaterial (Variables|Default|GetProgressBarMaterial))
  (bind _asbp_fpsplayer (Utilities|Casting|CastToBP_FPSPlayer (Game|Player|GetPlayerPawn 0)))
  (Rendering|Material|SetMaterial (Variables|/Game/BPs/BP_FPSPlayer.BP_FPSPlayer_C|GetExpBar _asbp_fpsplayer) 0 _progressbarmaterial)
  (bind _returnvalue (Class|Gun|GetLevelPercentage))
  (Rendering|Material|SetScalarParameterValue _progressbarmaterial "Percent" _returnvalue :!class /Script/Engine.MaterialInstanceDynamic)
  (if (and (>= (Variables|Default|GettotalEXP) (Variables|/Script/RLFPS.SymbioticGameMode|GetEXPRequiredForBoss _gamemode)) (not (Variables|/Script/RLFPS.SymbioticGameMode|GetbossSequenceStarted _gamemode)))
    (Class|SymbioticGameMode|StartBossSequence (Variables|Default|GetGameMode))))

(event EventOnFirstUpgrade
  (Audio|PlaySound2D "/Game/Audio/FergusonVoiceLines/A_FirstUpgrade.A_FirstUpgrade" 1.0 1.0 0.0 0 0))

(event EventPlayMuzzleFlashFX
  (params (playVFX :type Boolean))
  (Audio|PlaySound2D "/Game/Audio/GunSFX/A_Gunshot.A_Gunshot" 0.3 1.0 0.0 0 0)
  (if playVFX
    (Niagara|SpawnSystemAttached "/Game/Art/FX/MuzzleFlash/NS_MuzzleFlash.NS_MuzzleFlash" (Variables|Transformation|GetRootComponent) "point" (+ (* (Math|Vector|GetForwardVector (Transformation|GetActorRotation)) (Variables|Default|GetMuzzleLocation)) (Transformation|GetActorLocation)) (Transformation|GetActorRotation) "KeepWorldPosition" false)))

(fn ConstructionScript
  (bind _returnvalue (Rendering|Material|CreateDynamicMaterialInstance (Variables|Default|GetGun_v01_Muscle_low1) 0 "/Game/Art/Materials/Custom/LevelBarMat.LevelBarMat" "None" :!class /Script/Engine.PrimitiveComponent))
  (Variables|Default|SetProgressBarMaterial _returnvalue)
  (bind _aswbp_settings_controller (Utilities|Casting|CastToWBP_SettingsController (Game|GetGameInstance)))
  (Variables|Default|SetLeftHanded (Variables|/Game/Widgets/3D_Menu/WBP_SettingsController.WBP_SettingsController_C|GetLeftHandToggle _aswbp_settings_controller)))