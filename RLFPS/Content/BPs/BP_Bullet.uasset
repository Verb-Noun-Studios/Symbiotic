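; Projectile bullet with a tunable Niagara trail; overlap logic runs only for non-enemy shots.
; It damages grunts, bosses and head targets using the player gun's damage, and is destroyed by boss shields.
; Crystal instanced-mesh hits are swapped for B_Crystal actors, recolored by type.
; Explosive crystals apply radial knockback and damage through a spawned trigger sphere, while healing and acid crystals spawn their effect actors.
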(event OnComponentBeginOverlap(CollisionComponent)
  (params (OverlappedComponent :type Primitive%20Component%20Object%20Reference) (OtherActor :type Actor%20Object%20Reference) (OtherComp :type Primitive%20Component%20Object%20Reference) (OtherBodyIndex :type Integer) (bFromSweep :type Boolean) (SweepResult :type Hit%20Result%20Structure%20%28by%20ref%29))
  (bind _returnvalue (Transformation|GetActorLocation))
  (bind _returnvalue_2 (Transformation|GetActorLocation))
  (bind (_bblockinghit _binitialoverlap _time _distance _location _impactpoint _normal _impactnormal _physmat _hitactor _hitcomponent _hitbonename _hititem) (Collision|BreakHitResult SweepResult))
  (bind _explosionradis (Variables|Default|GetExplosionRadis))
  (bind _explosionradis_2 (Variables|Default|GetExplosionRadis))
  (bind _explosionradis_3 (Variables|Default|GetExplosionRadis))
  (if (not (Variables|Default|GetspawnedByEnemy))
    (bind _returnvalue_3 (Actor|GetActorOfClass "/Game/BPs/BP_FPSPlayer.BP_FPSPlayer_C"))
    (bind _asgun (Utilities|Casting|CastToGun (Variables|/Script/Engine.ChildActorComponent|GetChildActor (Variables|/Game/BPs/BP_FPSPlayer.BP_FPSPlayer_C|GetGun _returnvalue_3))))
    (Variables|Default|SetTheGun _asgun)
    (Utilities|Casting|CastToBP_Gun OtherActor
      (:CastFailed
        (bind _asgrunt_character (Utilities|Casting|CastToGruntCharacter OtherActor)
          (:then
            (Class|Gun|OnHitCallback (Variables|Default|GetTheGun) _asgrunt_character)
            (Game|Damage|ApplyDamage _asgrunt_character (Variables|/Script/RLFPS.Gun|GetDamage (Variables|Default|GetTheGun)) 0 0)
            (Actor|DestroyActor))
          (:CastFailed
            (bind _ashead_target_blueprint (Utilities|Casting|CastToheadTarget_Blueprint OtherActor)
              (:then
                (Default|ApplyDamage _ashead_target_blueprint (Variables|/Script/RLFPS.Gun|GetDamage (Variables|Default|GetTheGun))))
              (:CastFailed
                (Utilities|Casting|CastToBP_FPSPlayer OtherActor
                  (:then
                    (Actor|DestroyActor))
                  (:CastFailed
                    (bind _asboss_ai (Utilities|Casting|CastToBossAI OtherActor)
                      (:then
                        (Class|Gun|OnHitCallback (Variables|Default|GetTheGun) _asboss_ai)
                        (Game|Damage|ApplyDamage _asboss_ai (Variables|/Script/RLFPS.Gun|GetDamage (Variables|Default|GetTheGun)) 0 0)
                        (Actor|DestroyActor))
                      (:CastFailed
                        (Utilities|Casting|CastToBP_BossShield OtherActor
                          (:then
                            (Actor|DestroyActor))
                          (:CastFailed
                            (bind _asinstanced_static_mesh_component (Utilities|Casting|CastToInstancedStaticMeshComponent _hitcomponent))
                            (Variables|Default|SetInstanceIndex _hititem)
                            (bind _output_get (Variables|Default|SetComponent _asinstanced_static_mesh_component))
                            (Variables|Default|SetInstanceTransform (.OutInstanceTransform (Components|InstancedStaticMesh|GetInstanceTransform _output_get _hititem true)))
                            (if (== (Variables|/Script/Engine.StaticMeshComponent|GetStaticMesh (Variables|Default|GetComponent)) "/Game/Art/Meshes/NEWModularPieces/Crystals/crystal_regular.crystal_regular")
                              (Game|SpawnActorfromClass "/Game/Art/Meshes/NEWModularPieces/Crystals/B_Crystal.B_Crystal_C" (Variables|Default|GetInstanceTransform) "Undefined" 0 0)
                              (Class|InstancedStaticMeshComponent|RemoveInstance (Variables|Default|GetComponent) (Variables|Default|GetInstanceIndex))
                              (else
                                (bind _returnvalue_4 (Game|SpawnActorfromClass "/Game/Art/Meshes/NEWModularPieces/Crystals/B_Crystal.B_Crystal_C" (Variables|Default|GetInstanceTransform) "Undefined" 0 0))
                                (if (== (Variables|/Script/Engine.StaticMeshComponent|GetStaticMesh (Variables|Default|GetComponent)) "/Game/Art/Meshes/NEWModularPieces/Crystals/crystal_explosive.crystal_explosive")
                                  (Rendering|Material|SetMaterial (Variables|/Game/Art/Meshes/NEWModularPieces/Crystals/B_Crystal.B_Crystal_C|GetbrokenShard_shard3 _returnvalue_4) 0 "/Game/Art/Meshes/NEWModularPieces/Crystals/MI_CrystalGreen.MI_CrystalGreen")
                                  (Rendering|Material|SetMaterial (Variables|/Game/Art/Meshes/NEWModularPieces/Crystals/B_Crystal.B_Crystal_C|Getshard2 _returnvalue_4) 1 "/Game/Art/Meshes/NEWModularPieces/Crystals/MI_CrystalGreen.MI_CrystalGreen")
                                  (Niagara|SpawnSystematLocation "/Game/Art/FX/CrawlerExplosion/Explosion_V2/NE_ExplosionCentre_System.NE_ExplosionCentre_System" (Transformation|GetActorLocation))
                                  (Class|InstancedStaticMeshComponent|RemoveInstance (Variables|Default|GetComponent) (Variables|Default|GetInstanceIndex))
                                  (bind _returnvalue_5 (Game|SpawnActorfromClass "/Script/Engine.TriggerSphere" (Transformation|GetActorTransform) "Undefined" 0 0))
                                  (Transformation|SetActorScale3D _returnvalue_5 (/ (Math|Vector|MakeVector _explosionradis_2 _explosionradis_2 _explosionradis_2) 2e+01))
                                  (for _array_element (Collision|GetOverlappingActors _returnvalue_5 0 :!class /Script/Engine.Actor)
                                    (bind _asgrunt_character_2 (Utilities|Casting|CastToGruntCharacter _array_element)
                                      (:then
                                        (Variables|/Script/Engine.MovementComponent|SetVelocity (Variables|/Script/Engine.Character|GetCharacterMovement _asgrunt_character_2) (* (* (* (Math|Vector|GetUnitDirection(Vector) _returnvalue_2 (Transformation|GetActorLocation _asgrunt_character_2)) (Variables|Default|GetKnockbackRate)) (Math|Float|Clamp(Float) (- _explosionradis_3 (Math|Float|Absolute(Float) (Math|Vector|Distance(Vector) (Transformation|GetActorLocation _asgrunt_character_2) _returnvalue_2))) 0.1 _explosionradis_3)) (Variables|Default|GetForceMultiplier)))
                                        (Variables|/Script/RLFPS.HealthComponent|SetcurrentHealth (Variables|/Script/RLFPS.GruntCharacter|GetHealthComponent _asgrunt_character_2) (- (Variables|/Script/RLFPS.HealthComponent|GetcurrentHealth (Variables|/Script/RLFPS.GruntCharacter|GetHealthComponent _asgrunt_character_2)) (Variables|Default|GetDamageAmount))))
                                      (:CastFailed
                                        (bind _asbp_fpsplayer (Utilities|Casting|CastToBP_FPSPlayer _array_element))
                                        (Class|FragPlayer|SetVelocity _asbp_fpsplayer (* (* (* (Math|Vector|GetUnitDirection(Vector) _returnvalue (Transformation|GetActorLocation _asbp_fpsplayer)) (Variables|Default|GetKnockbackRate)) (Math|Float|Clamp(Float) (- _explosionradis (Math|Float|Absolute(Float) (Math|Vector|Distance(Vector) (Transformation|GetActorLocation _asbp_fpsplayer) _returnvalue))) 0.1 _explosionradis)) (Variables|Default|GetForceMultiplier)))
                                        (Game|Damage|ApplyDamage 0 (Variables|Default|GetDamageAmount) 0 self)))
                                    (Actor|DestroyActor))
                                  (for _array_element_2 (Class|Actor|GetOverlappingComponents _returnvalue_5)
                                    (Utilities|Casting|CastToInstancedStaticMeshComponent _array_element_2))
                                  (elif (== (Variables|/Script/Engine.StaticMeshComponent|GetStaticMesh (Variables|Default|GetComponent)) "/Game/Art/Meshes/NEWModularPieces/Crystals/crystal_regularBlue.crystal_regularBlue")
                                    (Rendering|Material|SetMaterial (Variables|/Game/Art/Meshes/NEWModularPieces/Crystals/B_Crystal.B_Crystal_C|GetbrokenShard_shard3 _returnvalue_4) 0 "/Game/Art/Meshes/NEWModularPieces/Crystals/MI_CrystalPurple.MI_CrystalPurple")
                                    (Rendering|Material|SetMaterial (Variables|/Game/Art/Meshes/NEWModularPieces/Crystals/B_Crystal.B_Crystal_C|GetbrokenShard_shard3 _returnvalue_4) 1 "/Game/Art/Meshes/NEWModularPieces/Crystals/MI_CrystalPurple.MI_CrystalPurple")
                                    (Class|InstancedStaticMeshComponent|RemoveInstance (Variables|Default|GetComponent) (Variables|Default|GetInstanceIndex))
                                    (elif (== (Variables|/Script/Engine.StaticMeshComponent|GetStaticMesh (Variables|Default|GetComponent)) "/Game/Art/Meshes/NEWModularPieces/Crystals/crystal_healing.crystal_healing")
                                      (Rendering|Material|SetMaterial (Variables|/Game/Art/Meshes/NEWModularPieces/Crystals/B_Crystal.B_Crystal_C|GetbrokenShard_shard3 _returnvalue_4) 0 "/Game/Art/Meshes/NEWModularPieces/Crystals/MI_CrystalWhite.MI_CrystalWhite")
                                      (Rendering|Material|SetMaterial (Variables|/Game/Art/Meshes/NEWModularPieces/Crystals/B_Crystal.B_Crystal_C|GetbrokenShard_shard3 _returnvalue_4) 1 "/Game/Art/Meshes/NEWModularPieces/Crystals/MI_CrystalWhite.MI_CrystalWhite")
                                      (Game|SpawnActorfromClass "/Game/Art/FX/HealingShot/BP_HealingBeam.BP_HealingBeam_C" (Math|Conversions|ToTransform(Vector) (Transformation|GetActorLocation)) "Undefined" 0 0)
                                      (Class|InstancedStaticMeshComponent|RemoveInstance (Variables|Default|GetComponent) (Variables|Default|GetInstanceIndex))
                                      (Actor|DestroyActor :!label _label)
                                      (elif (== (Variables|/Script/Engine.StaticMeshComponent|GetStaticMesh (Variables|Default|GetComponent)) "/Game/Art/Meshes/NEWModularPieces/Crystals/crystal_acid.crystal_acid")
                                        (Rendering|Material|SetMaterial (Variables|/Game/Art/Meshes/NEWModularPieces/Crystals/B_Crystal.B_Crystal_C|Get5 _returnvalue_4) 0 "/Game/Art/Meshes/NEWModularPieces/Crystals/MI_CrystalWhite.MI_CrystalWhite")
                                        (Rendering|Material|SetMaterial (Variables|/Game/Art/Meshes/NEWModularPieces/Crystals/B_Crystal.B_Crystal_C|Get5 _returnvalue_4) 1 "/Game/Art/Meshes/NEWModularPieces/Crystals/MI_CrystalWhite.MI_CrystalWhite")
                                        (Game|SpawnActorfromClass "/Game/BPs/Mods/BP_Acid.BP_Acid_C" (Math|Conversions|ToTransform(Vector) (Transformation|GetActorLocation)) "Undefined" 0 0)
                                        (Class|InstancedStaticMeshComponent|RemoveInstance (Variables|Default|GetComponent) (Variables|Default|GetInstanceIndex))
                                        (goto _label)))))))))))))))))))))

(event Custom|UpdateVelocity
  (params (Direction :type Vector))
  (Game|Components|ProjectileMovement|SetVelocityinLocalSpace (Variables|Default|GetProjectileMovementComponent) Direction))

(event EventBeginPlay
  (Niagara|SetNiagaraVariable(LinearColor) (Variables|Default|GetTrailFX) "trail_color" (Math|Conversions|ToLinearColor(Color) (Variables|VFX|Gettrail_color))))

(event Collision|EventActorBeginOverlap
  (params (OtherActor :type Actor%20Object%20Reference)))

(event EventTick
  (params (DeltaSeconds :type Float%20%28single-precision%29)))

(event EventUpdateVFX
  (Niagara|SetNiagaraVariable(LinearColor) (Variables|Default|GetTrailFX) "trail_color" (Math|Conversions|ToLinearColor(Color) (Variables|VFX|Getring_color)))
  (Niagara|SetNiagaraVariable(Float) (Variables|Default|GetTrailFX) "ring_lifetime" (Variables|VFX|Getring_lifetime))
  (Niagara|SetNiagaraVariable(Float) (Variables|Default|GetTrailFX) "ring_sizeScale" (Variables|VFX|Getring_sizeScale))
  (Niagara|SetNiagaraVariable(Float) (Variables|Default|GetTrailFX) "ring_spawnrate" (Variables|VFX|Getring_spawnRate))
  (Niagara|SetNiagaraVariable(LinearColor) (Variables|Default|GetTrailFX) "trail_color" (Math|Conversions|ToLinearColor(Color) (Variables|VFX|Gettrail_color)))
  (Niagara|SetNiagaraVariable(Float) (Variables|Default|GetTrailFX) "trail_lifetime" (Variables|VFX|Gettrail_lifetime))
  (Niagara|SetNiagaraVariable(Float) (Variables|Default|GetTrailFX) "trail_noiseStrength" (Variables|VFX|Gettrail_noiseStrength))
  (Niagara|SetNiagaraVariable(Float) (Variables|Default|GetTrailFX) "trail_width" (Variables|VFX|Gettrail_width)))

(fn ConstructionScript)

(fn SpawnHitEffect
  (Niagara|SpawnSystematLocation "/Game/Art/FX/BulletHit/NS_BulletHit.NS_BulletHit" (Transformation|GetWorldLocation (Variables|Default|GetStaticMesh))))

(fn CheckforMods
  (params (Gun :type Gun%20Object%20Reference) (SelfBullet :type Bullet%20Object%20Reference))
  (LocalVariables|SetThisBullet SelfBullet)
  (for _array_element (Variables|/Script/RLFPS.Gun|Getmods Gun)
    (if (Utilities|String|Contains (Utilities|String|ToString(Name) (Variables|/Script/RLFPS.ModBase|Getname _array_element)) "Shotgun")
      _)))