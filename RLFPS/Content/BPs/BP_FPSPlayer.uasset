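; First-person shooter player pawn that handles gun input, HUD, pause and upgrade menus, damage feedback and death.
; Tick triggers vaulting, copies gun state, shakes the camera while firing, refreshes sensitivity and watches health.
; Zero health invalidates save data and starts a post-process death timeline, then a physics tumble and paused lose screen.
; Beacon interaction uses a camera trace, with its key chosen by the left-hand setting.
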(event Custom|LockCamera)

(event Custom|Death%20Animation
  (bind _collider (Variables|Default|GetCollider))
  (Input|DisableInput (Game|GetPlayerController 0))
  (bind _outactors (Actor|GetAllActorsOfClass "/Script/RLFPS.GruntCharacter"))
  (for _array_element _outactors
    (Actor|DestroyActor _array_element))
  (bind _animation (Timeline|DeathTimeline Play)
    (:Update
      (Rendering|Material|SetScalarParameterValue (Variables|Default|GetDMI%20PP%20Death) "Dead" _animation :!class /Script/Engine.MaterialInstanceDynamic))
    (:Finished
      (Physics|SetSimulatePhysics _collider true)
      (Class|PrimitiveComponent|SetCenterOfMass _collider (Math|Vector|MakeVector (Math|Random|RandomFloatinRange -2e+02 2e+02) (Math|Random|RandomFloatinRange -2e+02 2e+02) (Math|Random|RandomFloatinRange -2e+02 2e+02)) "None")
      (Variables|/Script/Engine.CameraComponent|SetbUsePawnControlRotation (Variables|Default|GetFirstPersonCameraComponent) false)
      (Utilities|Time|SetTimerbyEvent (delegate Custom|ResetSimulatePhysics) 2.0))))

(event Custom|ResetSimulatePhysics
  (bind _returnvalue (Game|GetPlayerController 0))
  (Input|EnableInput (Game|GetPlayerController 0))
  (Physics|SetSimulatePhysics (Variables|Default|GetCollider) false)
  (bind _returnvalue_2 (UserInterface|CreateWidget "/Game/Widgets/WBP_LoseScreen.WBP_LoseScreen_C"))
  (UserInterface|Viewport|AddtoViewport _returnvalue_2 0)
  (Game|SetGamePaused true)
  (Input|SetInputModeGameandUI _returnvalue _returnvalue_2 "LockOnCapture" false)
  (Variables|/Script/Engine.PlayerController|SetbShowMouseCursor _returnvalue true))

(event EventBeginPlay
  (bind _aswbp_settings_controller (Utilities|Casting|CastToWBP_SettingsController (Game|GetGameInstance)))
  (Class|FragPlayer|UpdateControls (not (Variables|/Game/Widgets/3D_Menu/WBP_SettingsController.WBP_SettingsController_C|GetLeftHandToggle _aswbp_settings_controller)))
  (CallFunction|SetGunValues)
  (Actor|Tick|SetActorTickEnabled true)
  (bind _returnvalue (UserInterface|CreateWidget "/Game/Widgets/WBP_PlayerHud.WBP_PlayerHud_C" (Game|GetPlayerController 0)))
  (bind _output_get (Variables|Default|SetHUD_Widget _returnvalue))
  (UserInterface|Viewport|AddtoViewport _output_get 0)
  (bind _returnvalue_2 (Rendering|Material|CreateDynamicMaterialInstance "/Game/Art/Materials/MPPI_Death.MPPI_Death" "None" "None" :!class /Script/Engine.KismetMaterialLibrary))
  (Variables|Default|SetDMI%20PP%20Death _returnvalue_2))

(event Game|Damage|EventAnyDamage
  (params (Damage :type Float%20%28single-precision%29) (DamageType :type Damage%20Type%20Object%20Reference) (InstigatedBy :type Controller%20Object%20Reference) (DamageCauser :type Actor%20Object%20Reference))
  (bind _hud_widget (Variables|Default|GetHUD_Widget))
  (bind _bloodoverlay (Variables|/Game/Widgets/WBP_PlayerHud.WBP_PlayerHud_C|GetBloodOverlay _hud_widget))
  (Class|Image|SetBrushTintColor _bloodoverlay (Utilities|Struct|MakeSlateColor "(R=1.000000,G=1.000000,B=1.000000,A=1.000000)" "UseColor_Specified"))
  (bind _returnvalue (Actor|GetActorOfClass "/Game/BPs/BP_Gun.BP_Gun_C"))
  (if (Variables|/Script/RLFPS.Gun|GetreadyToLevelUp _returnvalue)
    (Widget|RemovefromParent (Variables|Default|GetHitIndicator))
    (else
      (bind _returnvalue_2 (UserInterface|CreateWidget "/Game/Widgets/WBP_HitIndicator.WBP_HitIndicator_C" 0 self DamageCauser))
      (bind _output_get (Variables|Default|SetHitIndicator _returnvalue_2))
      (UserInterface|Viewport|AddtoViewport _output_get 0)
      (Utilities|FlowControl|Delay 3.0)
      (Class|Image|SetBrushTintColor _bloodoverlay (Utilities|Struct|MakeSlateColor "(R=1.000000,G=0.000000,B=1.000000,A=0.000000)" "UseColor_Specified")))))

(event EventTick
  (params (DeltaSeconds :type Float%20%28single-precision%29))
  (bind _vaulting_comp (Variables|Default|GetVaulting_Comp))
  (bind _collider (Variables|Default|GetCollider))
  (bind _returnvalue (Transformation|GetWorldLocation _collider))
  ;[1 1 1] Vaulting Called
  (bind (_result _endlocation) (Default|CanVault (Variables|Default|GetVaulting_Comp)))
  (if (and _result (Utilities|Enum|Equal(Enum) (Default|GetVaultingState (Variables|Default|GetVaulting_Comp)) "NewEnumerator0"))
    (Default|SetEndPoint _vaulting_comp _endlocation)
    (Default|Vault _vaulting_comp))
  (Utilities|FlowControl|Sequence
    (:then_0
      (if (<= (Variables|/Script/RLFPS.HealthComponent|GetcurrentHealth (Variables|Default|GetHealthComponent)) 0.0)
        (Utilities|FlowControl|DoOnce false
          (:Completed
            (CallFunction|LoseScreen)
            (Class|SaveControllerSubsystem|InvalidateData (Subsystems|GetSaveControllerSubsystem))))
        (else
          (CallFunction|SetGunValues)
          (if (Variables|Default|Getfiring)
            (Class|MatineeCameraShake|StartMatineeCameraShake (Game|GetPlayerCameraManager 0) "/Game/BPs/BP_GunShake.BP_GunShake_C" 0.8 "CameraLocal" "0, 0, 0"))
          (bind _outhit (Collision|LineTraceByChannel _returnvalue (+ (* (Math|Vector|GetUpVector _collider) -1e+03) _returnvalue) "TraceTypeQuery1" false 0 "None"))
          (Variables|Default|SetLocationUnderPlayer (.ImpactPoint (Collision|BreakHitResult _outhit))))))
    (:then_1
      (bind _aswbp_settings_controller (Utilities|Casting|CastToWBP_SettingsController (Game|GetGameInstance)))
      (Variables|Default|SetMouseSensitivity (Variables|/Game/Widgets/3D_Menu/WBP_SettingsController.WBP_SettingsController_C|GetPlayerSensitivity _aswbp_settings_controller)))
    (:then_2
      (CallFunction|LockCamera))))

(event Input|KeyboardEvents|Home
  (params (Key :type Key%20Structure))
  (:Pressed
    (Game|OpenLevel(byName) "3D_MenuMap")))

(event Input|KeyboardEvents|P
  (params (Key :type Key%20Structure))
  ;[1 1 1] Escape Pressed
  (:Pressed
    (|Determineifdisplay
      (:true
        (Utilities|IsValid (Variables|Default|GetPauseMenuRef)
          (:Is%20Valid
            (|ShowPauseMenu))
          (:Is%20Not%20Valid
            (|BuildPauseMenu)))))))

(event Input|KeyboardEvents|Q
  (params (Key :type Key%20Structure))
  (:Pressed
    (Default|AddMods (Variables|/Game/Widgets/WBP_PlayerHud.WBP_PlayerHud_C|GetWBP_CurrMods (Variables|Default|GetHUD_Widget)) :!label _label))
  (:Released
    (goto _label)))

(event Input|MouseEvents|LeftMouseButton
  (params (Key :type Key%20Structure))
  (bind _gun (Variables|Default|GetGun))
  (bind _childactor (Variables|/Script/Engine.ChildActorComponent|GetChildActor _gun))
  (:Pressed
    (bind _asbp_gun (Utilities|Casting|CastToBP_Gun _childactor))
    (Variables|/Game/BPs/BP_Gun.BP_Gun_C|SetShooting _asbp_gun true))
  (:Released
    (bind _asbp_gun_2 (Utilities|Casting|CastToBP_Gun _childactor))
    (Variables|/Game/BPs/BP_Gun.BP_Gun_C|SetShooting _asbp_gun_2 false)))

(event Input|KeyboardEvents|Escape
  (params (Key :type Key%20Structure))
  ;[1 1 1] Escape Pressed
  (:Pressed
    (|Determineifdisplay
      (:true
        (Utilities|IsValid (Variables|Default|GetPauseMenuRef)
          (:Is%20Valid
            (|ShowPauseMenu))
          (:Is%20Not%20Valid
            (|BuildPauseMenu)))))))

(event Input|KeyboardEvents|E
  (params (Key :type Key%20Structure))
  (:Pressed
    (Default|AddMods (Variables|/Game/Widgets/WBP_PlayerHud.WBP_PlayerHud_C|GetWBP_CurrMods (Variables|Default|GetHUD_Widget)) :!label _label))
  (:Released
    (goto _label)))

(event Input|KeyboardEvents|F
  (params (Key :type Key%20Structure))
  (bind _firstpersoncameracomponent (Variables|Default|GetFirstPersonCameraComponent))
  (bind _returnvalue (Transformation|GetWorldLocation _firstpersoncameracomponent))
  ;[1 1 1] Interact
  (:Pressed
    (bind _aswbp_settings_controller (Utilities|Casting|CastToWBP_SettingsController (Game|GetGameInstance)))
    (if (not (Variables|/Game/Widgets/3D_Menu/WBP_SettingsController.WBP_SettingsController_C|GetLeftHandToggle _aswbp_settings_controller))
      (bind _outhit (Collision|LineTraceByChannel _returnvalue (+ _returnvalue (* (Math|Vector|GetForwardVector _firstpersoncameracomponent) 4e+02)) "TraceTypeQuery1" false 0 "None"))
      (bind _asbeacon_actor (Utilities|Casting|CastToBeaconActor (.HitActor (Collision|BreakHitResult _outhit))))
      (Class|InteractableInterface|Use(Message) _asbeacon_actor))))

(event Input|KeyboardEvents|Enter
  (params (Key :type Key%20Structure))
  (bind _firstpersoncameracomponent (Variables|Default|GetFirstPersonCameraComponent))
  (bind _returnvalue (Transformation|GetWorldLocation _firstpersoncameracomponent))
  ;[1 1 1] Interact
  (:Pressed
    (bind _aswbp_settings_controller (Utilities|Casting|CastToWBP_SettingsController (Game|GetGameInstance)))
    (if (Variables|/Game/Widgets/3D_Menu/WBP_SettingsController.WBP_SettingsController_C|GetLeftHandToggle _aswbp_settings_controller)
      (bind _outhit (Collision|LineTraceByChannel _returnvalue (+ _returnvalue (* (Math|Vector|GetForwardVector _firstpersoncameracomponent) 4e+02)) "TraceTypeQuery1" false 0 "None"))
      (bind _asbeacon_actor (Utilities|Casting|CastToBeaconActor (.HitActor (Collision|BreakHitResult _outhit))))
      (Class|InteractableInterface|Use(Message) _asbeacon_actor))))

(event Input|KeyboardEvents|7
  (params (Key :type Key%20Structure))
  (:Pressed
    (Default|AddMods (Variables|/Game/Widgets/WBP_PlayerHud.WBP_PlayerHud_C|GetWBP_CurrMods (Variables|Default|GetHUD_Widget)) :!label _label))
  (:Released
    (goto _label)))

(event Input|KeyboardEvents|Tab
  (params (Key :type Key%20Structure))
  (:Pressed
    (bind _returnvalue (Actor|GetActorOfClass "/Game/BPs/BP_Gun.BP_Gun_C"))
    (if (not (Variables|/Script/RLFPS.Gun|GetreadyToLevelUp _returnvalue))
      (|DetermineDisplay_2)
      (Utilities|IsValid (Variables|Default|GetPrevModsMenuRef)
        (:Is%20Valid
          (|Show/HideMenu))
        (:Is%20Not%20Valid
          (|BuildMenu))))))

(event Input|KeyboardEvents|9
  (params (Key :type Key%20Structure))
  (:Pressed
    (Default|AddMods (Variables|/Game/Widgets/WBP_PlayerHud.WBP_PlayerHud_C|GetWBP_CurrMods (Variables|Default|GetHUD_Widget)) :!label _label))
  (:Released
    (goto _label)))

(fn ConstructionScript)

(fn SetGunValues
  (bind _asgun (Utilities|Casting|CastToGun (Variables|/Script/Engine.ChildActorComponent|GetChildActor (Variables|Default|GetGun))))
  (Variables|Default|SetcurAmmoCount (Variables|/Script/RLFPS.Gun|GetammoRemaining _asgun))
  (Variables|Default|SetmaxAmmoCount (Variables|/Script/RLFPS.Gun|GetammoCount _asgun))
  (Variables|Default|Setreloading (Variables|/Script/RLFPS.Gun|Getreloading _asgun))
  (Variables|Default|Setfiring (Variables|/Script/RLFPS.Gun|Getfiring _asgun)))

(fn LoseScreen
  (Transformation|SetWorldLocation (Variables|Default|GetGun) "0, 0, 0" false true)
  (Viewport|RemoveAllWidgets)
  (Rendering|AddorUpdateBlendable (Variables|Default|GetFirstPersonCameraComponent) (Variables|Default|GetDMI%20PP%20Death) 1.0 :!class /Script/Engine.CameraComponent)
  (CallFunction|DeathAnimation))