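; BP_CrawlerMB_Goop is a damaging goop hazard for the Crawler miniboss that hurts the player standing in it.
; Each tick it checks whether its box collider overlaps the player pawn and applies damage, using a boolean gate and delay to space out damage ticks.
; StartEvent starts an optional lifetime: when the duration is positive, it waits, then removes the bubble particles and destroys the actor.
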(event Custom|StartEvent
  (if (> (Variables|Default|GetGoopDuration) 0.0)
    (Utilities|FlowControl|Delay (Variables|Default|GetGoopDuration))
    (Components|DestroyComponent (Variables|Default|GetPS_Bubbles))
    (Actor|DestroyActor)))

(event EventTick
  (params (DeltaSeconds :type Float%20%28single-precision%29))
  (bind _returnvalue (Game|Player|GetPlayerPawn 0))
  (if (and (Variables|Default|GetCanDamagePlayer) (Collision|IsOverlappingActor (Variables|Default|GetBoxCollider) _returnvalue :!class /Script/Engine.PrimitiveComponent))
    (bind _asbp_fpsplayer (Utilities|Casting|CastToBP_FPSPlayer _returnvalue))
    (Game|Damage|ApplyDamage _asbp_fpsplayer (Variables|Default|GetGoopDamage) 0 self)
    (Variables|Default|SetCanDamagePlayer false)
    (Utilities|FlowControl|Delay (Variables|Default|GetTimeBetweenDamageTicks))
    (Variables|Default|SetCanDamagePlayer true)))

(fn ConstructionScript)