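; Crawler enemy that explodes to damage and knock back (or optionally pull) the player and nearby GruntCharacters.
; BeginPlay scales health and damage using the player's gun, then starts BT_Crawler with blackboard tuning values.
; Tick updates player position and distance; at zero health it awards gun EXP, bumps the game mode's spawn count and detonates immediately.
; Also provides arced SmartJump launches, acid self-damage and blood decals spawned from particle collisions.
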(event Custom|On%20Colide%20Event
  (params (EventName :type Name) (EmitterTime :type Float%20%28single-precision%29) (ParticleTime :type Integer) (Location :type Vector) (Velocity :type Vector) (Direction :type Vector) (Normal :type Vector) (BoneName :type Name) (PhysMat :type Physical%20Material%20Object%20Reference))
  (bind _returnvalue (Rendering|Material|CreateDynamicMaterialInstance "/Game/Art/FX/BloodSplatter/m_Splatter_Decal.m_Splatter_Decal" "None" "None" :!class /Script/Engine.KismetMaterialLibrary))
  (Rendering|Material|SetScalarParameterValue _returnvalue "Frame" (Math|Conversions|ToFloat(Integer) (Math|Random|RandomInteger 11)) :!class /Script/Engine.MaterialInstanceDynamic)
  (Rendering|Decal|SpawnDecalatLocation _returnvalue (Math|Conversions|ToVector(Float) (Math|Random|RandomFloatinRange 25.0 1e+02)) Location (Math|Conversions|RotationFromXVector Normal) 2e+01))

(event Custom|ApplyAcidDamage
  (Game|Damage|ApplyDamage self (Variables|Default|GetAcidDamage) 0 0))

(event Custom|SmartJump
  (params (Destination :type Vector))
  (Pawn|Components|CharacterMovement|SetMovementMode (Variables|Character|GetCharacterMovement) "MOVE_Walking" 0)
  (bind _outlaunchvelocity (Game|SuggestProjectileVelocityCustomArc (Transformation|GetActorLocation) Destination 0.0 0.3))
  (Pawn|Components|CharacterMovement|SetMovementMode (Variables|Character|GetCharacterMovement) "MOVE_Flying" 0)
  (Character|LaunchCharacter self _outlaunchvelocity true true))

(event Custom|ExplosionEvent
  (params (Delay :type Float%20%28single-precision%29))
  (bind _returnvalue (Transformation|GetActorLocation))
  (bind _returnvalue_2 (Transformation|GetActorLocation))
  (bind _returnvalue_3 (Transformation|GetActorLocation))
  (bind _returnvalue_4 (Game|Player|GetPlayerPawn 0))
  (bind _forcemultiplier (Variables|Default|GetForceMultiplier))
  (bind _forcemultiplier_2 (Variables|Default|GetForceMultiplier))
  (bind _returnvalue_5 (Transformation|GetActorLocation _returnvalue_4))
  (bind (_x _y) (Math|Vector|BreakVector _returnvalue_3))
  (bind _returnvalue_6 (Math|Vector|MakeVector _x _y 0.0))
  (bind (_x_2 _y_2) (Math|Vector|BreakVector _returnvalue_5))
  (bind _ascrawler_anim (Utilities|Casting|CastToCrawlerAnim (Components|SkeletalMesh|GetAnimInstance (Variables|Character|GetMesh))))
  (Variables|/Game/Art/Meshes/Enemy/Crawler/CrawlerAnim.CrawlerAnim_C|SetGoingToExplode _ascrawler_anim true)
  (Variables|/Game/Art/Meshes/Enemy/Crawler/CrawlerAnim.CrawlerAnim_C|SetExplosionDelay _ascrawler_anim Delay)
  (Utilities|FlowControl|Delay Delay)
  (Niagara|SpawnSystematLocation "/Game/Art/FX/CrawlerExplosion/NS_CrawlerExplosion_System.NS_CrawlerExplosion_System" (Transformation|GetActorLocation self))
  (bind _outactors (Actor|GetAllActorsOfClass "/Script/RLFPS.GruntCharacter"))
  (if (> (Utilities|Array|Length _outactors) 0)
    (for _array_element _outactors
      ;[1 1 1] Grunt, Crawler, Flyer
      (if (<= (Math|Float|Absolute(Float) (Math|Vector|Distance(Vector) (Math|Vector|MakeVector (.X (Math|Vector|BreakVector (Transformation|GetActorLocation _array_element))) (.Y (Math|Vector|BreakVector (Transformation|GetActorLocation _array_element))) 0.0) _returnvalue_6)) (Variables|Default|GetExplosionRadius))
        (bind _asgrunt_character (Utilities|Casting|CastToGruntCharacter _array_element))
        (if (Variables|Default|GetShouldExplosionPull)
          (bind _result (Math|Float|NegateFloat _forcemultiplier)
            (:%20%20
              (Variables|/Script/Engine.MovementComponent|SetVelocity (Variables|/Script/Engine.Character|GetCharacterMovement _asgrunt_character) (/ (* (* (Math|Vector|GetUnitDirection(Vector) _returnvalue_2 (Transformation|GetActorLocation _asgrunt_character)) (Variables|Default|GetKnockbackRate)) (- (Variables|Default|GetExplosionRadius) (Math|Float|Absolute(Float) (Math|Vector|Distance(Vector) (Transformation|GetActorLocation _asgrunt_character) _returnvalue_2)))) _result))))
          (else
            (Variables|/Script/Engine.MovementComponent|SetVelocity (Variables|/Script/Engine.Character|GetCharacterMovement _asgrunt_character) (/ (* (* (Math|Vector|GetUnitDirection(Vector) _returnvalue_2 (Transformation|GetActorLocation _asgrunt_character)) (Variables|Default|GetKnockbackRate)) (- (Variables|Default|GetExplosionRadius) (Math|Float|Absolute(Float) (Math|Vector|Distance(Vector) (Transformation|GetActorLocation _asgrunt_character) _returnvalue_2)))) _forcemultiplier))))
        (Game|Damage|ApplyDamage _asgrunt_character (Variables|Default|GetDamageAmount) 0 self)
        (Actor|DestroyActor))))
  (if (<= (Math|Float|Absolute(Float) (Math|Vector|Distance(Vector) (Math|Vector|MakeVector _x_2 _y_2 0.0) _returnvalue_6)) (Variables|Default|GetExplosionRadius))
    ;[1 1 1] Player moved and takes damage
    (bind _asbp_fpsplayer (Utilities|Casting|CastToBP_FPSPlayer _returnvalue_4))
    (if (Variables|Default|GetShouldExplosionPull)
      (bind _result_2 (Math|Float|NegateFloat _forcemultiplier_2)
        (:%20%20
          (Class|FragPlayer|SetVelocity _asbp_fpsplayer (/ (* (* (Math|Vector|GetUnitDirection(Vector) _returnvalue (Transformation|GetActorLocation _asbp_fpsplayer)) (Variables|Default|GetKnockbackRate)) (- (Variables|Default|GetExplosionRadius) (Math|Float|Absolute(Float) (Math|Vector|Distance(Vector) (Transformation|GetActorLocation _asbp_fpsplayer) _returnvalue)))) _result_2))))
      (else
        (Class|FragPlayer|SetVelocity _asbp_fpsplayer (/ (* (* (Math|Vector|GetUnitDirection(Vector) _returnvalue (Transformation|GetActorLocation _asbp_fpsplayer)) (Variables|Default|GetKnockbackRate)) (- (Variables|Default|GetExplosionRadius) (Math|Float|Absolute(Float) (Math|Vector|Distance(Vector) (Transformation|GetActorLocation _asbp_fpsplayer) _returnvalue)))) _forcemultiplier_2))))
    (Game|Damage|ApplyDamage _asbp_fpsplayer (Variables|Default|GetDamageAmount) 0 self)
    (Actor|DestroyActor)))

(event Custom|OnTakeAnyDamage_Event_0
  (params (DamagedActor :type Actor%20Object%20Reference) (Damage :type Float%20%28single-precision%29) (DamageType :type Damage%20Type%20Object%20Reference) (InstigatedBy :type Controller%20Object%20Reference) (DamageCauser :type Actor%20Object%20Reference))
  (Variables|Default|SetHit true)
  (Utilities|FlowControl|Delay 1.1)
  (Variables|Default|SetHit false))

(event Custom|ManageExplosionVisual
  (params (Mesh :type Static%20Mesh%20Actor%20Object%20Reference))
  (bind _staticmeshcomponent (Variables|/Script/Engine.StaticMeshActor|GetStaticMeshComponent Mesh))
  (bind _explosionradius (Variables|Default|GetExplosionRadius))
  ;[1 1 1] Not actually used anymore
  (Rendering|Material|SetMaterial _staticmeshcomponent 0 "/Game/Art/Materials/Custom/CrawlerExplosion.CrawlerExplosion")
  (Transformation|SetMobility _staticmeshcomponent "Stationary")
  (Components|StaticMesh|SetStaticMesh _staticmeshcomponent "/Game/Art/Meshes/S_Sphere_01.S_Sphere_01")
  (Collision|SetCollisionEnabled _staticmeshcomponent "NoCollision")
  (Transformation|SetActorScale3D Mesh (/ (Math|Vector|MakeVector _explosionradius _explosionradius _explosionradius) 12.0))
  (Niagara|SpawnSystematLocation "/Game/Art/FX/CrawlerExplosion/NS_CrawlerExplosion_System.NS_CrawlerExplosion_System" (Transformation|GetWorldLocation (Variables|/Script/Engine.StaticMeshActor|GetStaticMeshComponent Mesh))))

(event Game|Damage|EventAnyDamage
  (params (Damage :type Float%20%28single-precision%29) (DamageType :type Damage%20Type%20Object%20Reference) (InstigatedBy :type Controller%20Object%20Reference) (DamageCauser :type Actor%20Object%20Reference))
  (bind _capsulecomponent (Variables|Default|GetCapsuleComponent))
  (bind _returnvalue (Transformation|GetWorldLocation _capsulecomponent))
  (bind _returnvalue_2 (Effects|SpawnEmitteratLocation "/Game/Art/FX/BloodSplatter/splatter_P.splatter_P" _returnvalue))
  (Niagara|SpawnSystematLocation "/Game/Art/FX/EnemyDeath/NE_EnemyDeath_System.NE_EnemyDeath_System" _returnvalue)
  (EventDispatchers|BindEventtoOnParticleCollide _returnvalue_2 (delegate Custom|On%20Colide%20Event))
  (Class|GruntCharacter|UpdateStatusWidget))

(event EventBeginPlay
  (bind _self self)
  (bind _healthcomponent (Variables|Default|GetHealthComponent))
  (bind _returnvalue (AI|GetBlackboard _self))
  (|CallParentFunction)
  (Variables|Default|SetGoingToExplode false)
  (bind _asbp_fpsplayer (Utilities|Casting|CastToBP_FPSPlayer (Game|Player|GetPlayerPawn 0)))
  (bind _asbp_gun (Utilities|Casting|CastToBP_Gun (Variables|/Script/Engine.ChildActorComponent|GetChildActor (Variables|/Game/BPs/BP_FPSPlayer.BP_FPSPlayer_C|GetGun _asbp_fpsplayer))))
  (bind (_newhealth _newdamage) (CallFunction|UpdateStats 1.0 (Variables|/Script/RLFPS.HealthComponent|GetcurrentHealth _healthcomponent) (Variables|Default|GetDamageAmount) _asbp_gun))
  (Variables|/Script/RLFPS.HealthComponent|SetcurrentHealth _healthcomponent _newhealth)
  (Variables|Default|SetDamageAmount _newdamage)
  (EventDispatchers|AssignOnTakeAnyDamage (delegate Custom|OnTakeAnyDamage_Event_0))
  (Class|SkeletalMeshComponent|SetAnimClass (Variables|Character|GetMesh) "/Game/Art/Meshes/Enemy/Crawler/CrawlerAnim.CrawlerAnim_C")
  (AI|RunBehaviorTree (AI|GetAIController self) "/Game/BPs/AI/Crawler/BT_Crawler.BT_Crawler")
  ;[1 1 1] Default values for the AI
  (AI|Components|Blackboard|SetValueasBool _returnvalue (Utilities|String|StringToName "True") true) ; Just leave this set as true
  (AI|Components|Blackboard|SetValueasFloat _returnvalue (Utilities|String|StringToName "AttackRange") (Variables|Default|GetAttackRange)) ; Range for the player to be considered in range
  (AI|Components|Blackboard|SetValueasFloat _returnvalue (Utilities|String|StringToName "ExplosionRadius") (Variables|Default|GetExplosionRadius)) ; How large the explosion radius is
  (AI|Components|Blackboard|SetValueasFloat _returnvalue (Utilities|String|StringToName "ExplosionDamage") (Variables|Default|GetDamageAmount)) ; How much damage does the explosion do to the player and nearby enemies
  (AI|Components|Blackboard|SetValueasFloat _returnvalue (Utilities|String|StringToName "TimeBeforeExplode") (Variables|Default|GetExplosionDelay)) ; Time delay before exploding once player is within range
  (AI|Components|Blackboard|SetValueasVector _returnvalue (Utilities|String|StringToName "Knockback Rate") (Variables|Default|GetKnockbackRate)) ; Percentage of the distance is applied as force to entites caught in the explosion
  (bind _asbp_fpsplayer_2 (Utilities|Casting|CastToBP_FPSPlayer (Game|Player|GetPlayerPawn 0)))
  (bind _returnvalue_2 (Class|FragPlayer|GetPosition _asbp_fpsplayer_2))
  (AI|Components|Blackboard|SetValueasVector (AI|GetBlackboard self) (Utilities|Name|MakeLiteralName "TargetDestination") _returnvalue_2)
  (AI|Components|Blackboard|SetValueasFloat (AI|GetBlackboard self) (Utilities|Name|MakeLiteralName "DistanceFromPlayer") (Transformation|GetDistanceTo (Game|Player|GetPlayerPawn 0)))
  (if (<= (Variables|/Script/RLFPS.HealthComponent|GetcurrentHealth (Variables|Default|GetHealthComponent)) 0.0)
    (bind _asbp_fpsplayer_3 (Utilities|Casting|CastToBP_FPSPlayer (Game|Player|GetPlayerPawn 0)))
    (bind _asbp_gun_2 (Utilities|Casting|CastToBP_Gun (Variables|/Script/Engine.ChildActorComponent|GetChildActor (Variables|/Game/BPs/BP_FPSPlayer.BP_FPSPlayer_C|GetGun _asbp_fpsplayer_3))))
    (Class|Gun|GainEXP _asbp_gun_2 2)
    (bind _asgm_sym (Utilities|Casting|CastToGM_Sym (Game|GetGameMode)))
    (Variables|/Script/RLFPS.SymbioticGameMode|SetenemiesLeftToSpawn _asgm_sym (+ (Variables|/Script/RLFPS.SymbioticGameMode|GetenemiesLeftToSpawn _asgm_sym) 1))
    (Class|GruntCharacter|OnDeath)
    (CallFunction|PlayDeathSound)
    (CallFunction|ExplosionEvent 0.0)))

(event EventTick
  (params (DeltaSeconds :type Float%20%28single-precision%29))
  (bind _ascrawler_anim (Utilities|Casting|CastToCrawlerAnim (Components|SkeletalMesh|GetAnimInstance (Variables|Character|GetMesh))))
  (Variables|/Game/Art/Meshes/Enemy/Crawler/CrawlerAnim.CrawlerAnim_C|SetHit _ascrawler_anim (Variables|Default|GetHit))
  (bind _asbp_fpsplayer (Utilities|Casting|CastToBP_FPSPlayer (Game|Player|GetPlayerPawn 0)))
  (bind _returnvalue (Class|FragPlayer|GetPosition _asbp_fpsplayer))
  (AI|Components|Blackboard|SetValueasVector (AI|GetBlackboard self) (Utilities|Name|MakeLiteralName "TargetDestination") _returnvalue)
  (AI|Components|Blackboard|SetValueasFloat (AI|GetBlackboard self) (Utilities|Name|MakeLiteralName "DistanceFromPlayer") (Transformation|GetDistanceTo (Game|Player|GetPlayerPawn 0)))
  (if (<= (Variables|/Script/RLFPS.HealthComponent|GetcurrentHealth (Variables|Default|GetHealthComponent)) 0.0)
    (bind _asbp_fpsplayer_2 (Utilities|Casting|CastToBP_FPSPlayer (Game|Player|GetPlayerPawn 0)))
    (bind _asbp_gun (Utilities|Casting|CastToBP_Gun (Variables|/Script/Engine.ChildActorComponent|GetChildActor (Variables|/Game/BPs/BP_FPSPlayer.BP_FPSPlayer_C|GetGun _asbp_fpsplayer_2))))
    (Class|Gun|GainEXP _asbp_gun 2)
    (bind _asgm_sym (Utilities|Casting|CastToGM_Sym (Game|GetGameMode)))
    (Variables|/Script/RLFPS.SymbioticGameMode|SetenemiesLeftToSpawn _asgm_sym (+ (Variables|/Script/RLFPS.SymbioticGameMode|GetenemiesLeftToSpawn _asgm_sym) 1))
    (Class|GruntCharacter|OnDeath)
    (CallFunction|PlayDeathSound)
    (CallFunction|ExplosionEvent 0.0)))

(fn ConstructionScript)

(fn PlayDeathSound
  (bind _returnvalue (Math|Random|RandomInteger 2))
  (switch int _returnvalue
    (:0
      (Audio|PlaySoundatLocation "/Game/Audio/AlienSFX/A_E1_Idle_Death.A_E1_Idle_Death" "0, 0, 0" "0, 0, 0" 1.0 1.0 0.0 0 0 0))
    (:1
      (Audio|PlaySoundatLocation "/Game/Audio/AlienSFX/A_E2_Agressive_Idle_Death.A_E2_Agressive_Idle_Death" "0, 0, 0" "0, 0, 0" 1.0 1.0 0.0 0 0 0))
    (:2
      (Audio|PlaySoundatLocation "/Game/Audio/AlienSFX/A_E4_Death.A_E4_Death" "0, 0, 0" "0, 0, 0" 1.0 1.0 0.0 0 0 0)))
  (Development|PrintString (Utilities|String|ToString(Integer) _returnvalue)))