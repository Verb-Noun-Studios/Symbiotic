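; BP_SwiperMB is the Swiper miniboss enemy, with gun-scaled health and damage, arced jump launches and projectile shots.
; BeginPlay starts BT_SwiperMB, seeding melee range and grunt-spawn limits into its blackboard.
; Tick feeds player location and distance to the blackboard, combat flags to GruntAnimation, and handles death, rewarding gun EXP and kills and incrementing EnemiesLeftToSpawn.
; Damage flashes the material and spawns particles whose collisions leave random splatter decals.
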(event Custom|On%20Colide%20Event
  (params (EventName :type Name) (EmitterTime :type Float%20%28single-precision%29) (ParticleTime :type Integer) (Location :type Vector) (Velocity :type Vector) (Direction :type Vector) (Normal :type Vector) (BoneName :type Name) (PhysMat :type Physical%20Material%20Object%20Reference))
  (bind _returnvalue (Rendering|Material|CreateDynamicMaterialInstance "/Game/Art/FX/BloodSplatter/m_Splatter_Decal.m_Splatter_Decal" "None" "None" :!class /Script/Engine.KismetMaterialLibrary))
  (Rendering|Material|SetScalarParameterValue _returnvalue "Frame" (Math|Conversions|ToFloat(Integer) (Math|Random|RandomInteger 11)) :!class /Script/Engine.MaterialInstanceDynamic)
  (Rendering|Decal|SpawnDecalatLocation _returnvalue (Math|Conversions|ToVector(Float) (Math|Random|RandomFloatinRange 25.0 1e+02)) Location (Math|Conversions|RotationFromXVector Normal) 2e+01))

(event Custom|SmartJump
  (params (Destination :type Vector))
  (Pawn|Components|CharacterMovement|SetMovementMode (Variables|Character|GetCharacterMovement) "MOVE_Walking" 0)
  (bind _outlaunchvelocity (Game|SuggestProjectileVelocityCustomArc (Transformation|GetActorLocation) Destination 0.0 0.3))
  (Pawn|Components|CharacterMovement|SetMovementMode (Variables|Character|GetCharacterMovement) "MOVE_Flying" 0)
  (Character|LaunchCharacter self _outlaunchvelocity true true))

(event Custom|Shoot
  (params (Player :type BP%20FPS%20Player%20Object%20Reference))
  (bind _returnvalue (Transformation|GetActorTransform))
  (bind _self self)
  (bind (_location _rotation _scale) (Math|Transform|BreakTransform _returnvalue))
  (bind _returnvalue_2 (Game|SpawnActorfromClass "/Game/BPs/AI/Grunt/BP_GruntShot.BP_GruntShot_C" (Math|Transform|MakeTransform (+ _location "0, 0,10.000000") _rotation _scale) "AlwaysSpawn" _self 2.0 _self))
  (Class|Bullet|SetInitialDirection _returnvalue_2 (Math|Vector|Normalize (- (Transformation|GetActorLocation Player) (Transformation|GetActorLocation))))
  (Class|Bullet|SetInitialSpeed _returnvalue_2 0.0))

(event Custom|OnTakeAnyDamage_Event_0
  (params (DamagedActor :type Actor%20Object%20Reference) (Damage :type Float%20%28single-precision%29) (DamageType :type Damage%20Type%20Object%20Reference) (InstigatedBy :type Controller%20Object%20Reference) (DamageCauser :type Actor%20Object%20Reference))
  (Variables|Default|SetHit true)
  (Utilities|FlowControl|Delay 1.1)
  (Variables|Default|SetHit false))

(event Game|Damage|EventAnyDamage
  (params (Damage :type Float%20%28single-precision%29) (DamageType :type Damage%20Type%20Object%20Reference) (InstigatedBy :type Controller%20Object%20Reference) (DamageCauser :type Actor%20Object%20Reference))
  (bind _mesh (Variables|Character|GetMesh))
  (bind _capsulecomponent (Variables|Default|GetCapsuleComponent))
  (bind _returnvalue (Transformation|GetWorldLocation _capsulecomponent))
  (bind _returnvalue_2 (Effects|SpawnEmitteratLocation "/Game/Art/FX/BloodSplatter/splatter_P.splatter_P" _returnvalue))
  (Niagara|SpawnSystematLocation "/Game/Art/FX/EnemyDeath/NE_EnemyDeath_System.NE_EnemyDeath_System" _returnvalue)
  (EventDispatchers|BindEventtoOnParticleCollide _returnvalue_2 (delegate Custom|On%20Colide%20Event))
  (Class|GruntCharacter|UpdateStatusWidget)
  (Rendering|Material|SetMaterial _mesh 0 (Variables|Default|GetHitMaterial))
  (Utilities|FlowControl|Delay 0.05)
  (Rendering|Material|SetMaterial _mesh 0 (Variables|Default|GetMaterial)))

(event EventBeginPlay
  (bind _self self)
  (bind _healthcomponent (Variables|Default|GetHealthComponent))
  (bind _returnvalue (AI|GetBlackboard _self))
  (bind _asbp_fpsplayer (Utilities|Casting|CastToBP_FPSPlayer (Game|Player|GetPlayerPawn 0)))
  (bind _asbp_gun (Utilities|Casting|CastToBP_Gun (Variables|/Script/Engine.ChildActorComponent|GetChildActor (Variables|/Game/BPs/BP_FPSPlayer.BP_FPSPlayer_C|GetGun _asbp_fpsplayer))))
  (bind (_newhealth _newdamage) (CallFunction|UpdateStats 1.0 (Variables|/Script/RLFPS.HealthComponent|GetcurrentHealth _healthcomponent) (Variables|Default|GetDamageAmount) _asbp_gun))
  (Variables|/Script/RLFPS.HealthComponent|SetcurrentHealth _healthcomponent _newhealth)
  (Variables|Default|SetDamageAmount _newdamage)
  (|CallParentFunction)
  (EventDispatchers|AssignOnTakeAnyDamage (delegate Custom|OnTakeAnyDamage_Event_0))
  (Class|SkeletalMeshComponent|SetAnimClass (Variables|Character|GetMesh) "/Game/Art/Meshes/Enemy/EnemyWithRig/GruntAnimation.GruntAnimation_C")
  (AI|RunBehaviorTree (AI|GetAIController self) "/Game/BPs/AI/Grunt/SwiperMiniboss/BT_SwiperMB.BT_SwiperMB")
  (Class|BlackboardComponent|SetValueasInt _returnvalue (Utilities|String|StringToName "MinGruntsToSpawn") (Variables|Default|GetMinGruntsToSpawn))
  (Class|BlackboardComponent|SetValueasInt _returnvalue (Utilities|String|StringToName "MaxGruntsToSpawn") (Variables|Default|GetMaxGruntsToSpawn))
  (AI|Components|Blackboard|SetValueasFloat _returnvalue (Utilities|String|StringToName "MeleeAttackRange") (Variables|Default|GetMeleeRange))
  (bind _asbp_fpsplayer_2 (Utilities|Casting|CastToBP_FPSPlayer (Game|Player|GetPlayerPawn 0)))
  (AI|Components|Blackboard|SetValueasVector (AI|GetBlackboard self) (Utilities|Name|MakeLiteralName "TargetDestination") (Variables|/Game/BPs/BP_FPSPlayer.BP_FPSPlayer_C|GetLocationUnderPlayer _asbp_fpsplayer_2))
  (AI|Components|Blackboard|SetValueasFloat (AI|GetBlackboard self) (Utilities|Name|MakeLiteralName "DistanceFromPlayer") (Transformation|GetDistanceTo (Game|Player|GetPlayerPawn 0)))
  (if (<= (Variables|/Script/RLFPS.HealthComponent|GetcurrentHealth (Variables|Default|GetHealthComponent)) 0.0)
    (bind _asbp_fpsplayer_3 (Utilities|Casting|CastToBP_FPSPlayer (Game|Player|GetPlayerPawn 0)))
    (bind _asbp_gun_2 (Utilities|Casting|CastToBP_Gun (Variables|/Script/Engine.ChildActorComponent|GetChildActor (Variables|/Game/BPs/BP_FPSPlayer.BP_FPSPlayer_C|GetGun _asbp_fpsplayer_3))))
    (Class|Gun|GainEXP _asbp_gun_2 2)
    (Default|IncrementKills _asbp_gun_2)
    (bind _asgm_sym (Utilities|Casting|CastToGM_Sym (Game|GetGameMode)))
    (Variables|/Script/RLFPS.SymbioticGameMode|SetenemiesLeftToSpawn _asgm_sym (+ (Variables|/Script/RLFPS.SymbioticGameMode|GetenemiesLeftToSpawn _asgm_sym) 1))
    (Class|GruntCharacter|OnDeath)
    (CallFunction|PlayDeathSound)
    (Actor|DestroyActor)
    (else
      (bind _returnvalue_2 (Actor|GetActorOfClass "/Game/BPs/BP_FPSPlayer.BP_FPSPlayer_C"))
      (Transformation|SetWorldRotation (Variables|Default|GetWidget) (Math|Rotator|FindLookatRotation (Transformation|GetActorLocation) (Transformation|GetActorLocation _returnvalue_2)) false false))))

(event EventTick
  (params (DeltaSeconds :type Float%20%28single-precision%29))
  (bind _asgrunt_animation (Utilities|Casting|CastToGruntAnimation (Components|SkeletalMesh|GetAnimInstance (Variables|Character|GetMesh))))
  (Variables|/Game/Art/Meshes/Enemy/EnemyWithRig/GruntAnimation.GruntAnimation_C|SetHit _asgrunt_animation (Variables|Default|GetHit))
  (Variables|/Game/Art/Meshes/Enemy/EnemyWithRig/GruntAnimation.GruntAnimation_C|SetMeleeAttack _asgrunt_animation (Variables|Default|GetMeleeAttack))
  (Variables|/Game/Art/Meshes/Enemy/EnemyWithRig/GruntAnimation.GruntAnimation_C|SetRangedAttack _asgrunt_animation (Variables|Default|GetRangedAttack))
  (AI|Components|Blackboard|SetValueasVector (AI|GetBlackboard self) (Utilities|Name|MakeLiteralName "TargetDestination") (Variables|/Game/BPs/BP_FPSPlayer.BP_FPSPlayer_C|GetLocationUnderPlayer (stale EventBeginPlay _asbp_fpsplayer_2)))
  (AI|Components|Blackboard|SetValueasFloat (AI|GetBlackboard self) (Utilities|Name|MakeLiteralName "DistanceFromPlayer") (Transformation|GetDistanceTo (Game|Player|GetPlayerPawn 0)))
  (if (<= (Variables|/Script/RLFPS.HealthComponent|GetcurrentHealth (Variables|Default|GetHealthComponent)) 0.0)
    (bind _asbp_fpsplayer (Utilities|Casting|CastToBP_FPSPlayer (Game|Player|GetPlayerPawn 0)))
    (bind _asbp_gun (Utilities|Casting|CastToBP_Gun (Variables|/Script/Engine.ChildActorComponent|GetChildActor (Variables|/Game/BPs/BP_FPSPlayer.BP_FPSPlayer_C|GetGun _asbp_fpsplayer))))
    (Class|Gun|GainEXP _asbp_gun 2)
    (Default|IncrementKills _asbp_gun)
    (bind _asgm_sym (Utilities|Casting|CastToGM_Sym (Game|GetGameMode)))
    (Variables|/Script/RLFPS.SymbioticGameMode|SetenemiesLeftToSpawn _asgm_sym (+ (Variables|/Script/RLFPS.SymbioticGameMode|GetenemiesLeftToSpawn _asgm_sym) 1))
    (Class|GruntCharacter|OnDeath)
    (CallFunction|PlayDeathSound)
    (Actor|DestroyActor)
    (else
      (bind _returnvalue (Actor|GetActorOfClass "/Game/BPs/BP_FPSPlayer.BP_FPSPlayer_C"))
      (Transformation|SetWorldRotation (Variables|Default|GetWidget) (Math|Rotator|FindLookatRotation (Transformation|GetActorLocation) (Transformation|GetActorLocation _returnvalue)) false false))))

(fn ConstructionScript)

(fn PlayDeathSound
  (bind _returnvalue (Math|Random|RandomInteger 2))
  (switch int _returnvalue
    (:0
      (Audio|PlaySoundatLocation "/Game/Audio/AlienSFX/A_E1_Idle_Death.A_E1_Idle_Death" "0, 0, 0" "0, 0, 0" 1.0 1.0 0.0 0 0 0))
    (:1
      (Audio|PlaySoundatLocation "/Game/Audio/AlienSFX/A_E2_Agressive_Idle_Death.A_E2_Agressive_Idle_Death" "0, 0, 0" "0, 0, 0" 1.0 1.0 0.0 0 0 0))
    (:2
      (Audio|PlaySoundatLocation "/Game/Audio/AlienSFX/A_E4_Death.A_E4_Death" "0, 0, 0" "0, 0, 0" 1.0 1.0 0.0 0 0 0)))
  (Development|PrintString (Utilities|String|ToString(Integer) _returnvalue)))