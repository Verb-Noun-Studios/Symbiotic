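; Base Blueprint for grunt AI characters that connects the character to its enemy status bar widget.
; On BeginPlay it assigns itself as the Entity of the EnemyStatusBar held by its Widget.
; UpdateStatusWidget resets the bar's lifetime to its default, and UpdateStatusEffects refreshes the displayed effects, then triggers that same reset.
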(event EventBeginPlay
  (bind _asenemy_status_bar (Utilities|Casting|CastToEnemyStatusBar (UserInterface|GetWidget (Variables|Default|GetWidget))))
  (Variables|/Game/Widgets/Enemies/EnemyStatusBar.EnemyStatusBar_C|SetEntity _asenemy_status_bar self))

(event Collision|EventActorBeginOverlap
  (params (OtherActor :type Actor%20Object%20Reference)))

(event EventTick
  (params (DeltaSeconds :type Float%20%28single-precision%29)))

(event EventUpdateStatusWidget
  (bind _asenemy_status_bar (Utilities|Casting|CastToEnemyStatusBar (UserInterface|GetWidget (Variables|Default|GetWidget))))
  (Variables|/Game/Widgets/Enemies/EnemyStatusBar.EnemyStatusBar_C|Setlifetime _asenemy_status_bar (Variables|/Game/Widgets/Enemies/EnemyStatusBar.EnemyStatusBar_C|GetdefaultLifetime _asenemy_status_bar)))

(event EventUpdateStatusEffects
  (bind _asenemy_status_bar (Utilities|Casting|CastToEnemyStatusBar (UserInterface|GetWidget (Variables|Default|GetWidget))))
  (Default|UpdateStatusEffects _asenemy_status_bar)
  (Class|GruntCharacter|UpdateStatusWidget))

(fn ConstructionScript)

(fn CustomEvent1)