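; BP_UpdateAIStats computes scaled health and damage for AI as the kill count grows.
; UpdateStats adds the gun's KilledEnemies, times a fixed rate and a strength factor, to the initial values, with health rising faster than damage.
; It reads EasyMode from the game instance, cast to WBP_SettingsController, and multiplies both results by EasyModeScaling when enabled.
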(fn UpdateStats
  (params (ScaleStrength :type Float%20%28single-precision%29) (InitialHealth :type Float%20%28single-precision%29) (InitialDamage :type Float%20%28single-precision%29) (Gun :type BP%20Gun%20Object%20Reference))
  (bind _easymodescaling (LocalVariables|GetEasyModeScaling))
  (LocalVariables|SetScaleStr ScaleStrength)
  (LocalVariables|SetHealth InitialHealth)
  (LocalVariables|SetDamage InitialDamage)
  (bind _output_get (LocalVariables|SetTheGun Gun))
  (bind _aswbp_settings_controller (Utilities|Casting|CastToWBP_SettingsController (Game|GetGameInstance)))
  (if (Variables|/Game/Widgets/3D_Menu/WBP_SettingsController.WBP_SettingsController_C|GetEasyMode _aswbp_settings_controller)
    (return (* (+ (* (* (Variables|/Game/BPs/BP_Gun.BP_Gun_C|GetKilledEnemies _output_get) 0.1) (LocalVariables|GetScaleStr)) (LocalVariables|GetHealth)) _easymodescaling) (* (+ (* (* (Variables|/Game/BPs/BP_Gun.BP_Gun_C|GetKilledEnemies _output_get) 0.08) (LocalVariables|GetScaleStr)) (LocalVariables|GetDamage)) _easymodescaling))
    (else
      (return (+ (* (* (Variables|/Game/BPs/BP_Gun.BP_Gun_C|GetKilledEnemies _output_get) 0.1) (LocalVariables|GetScaleStr)) (LocalVariables|GetHealth)) (+ (* (* (Variables|/Game/BPs/BP_Gun.BP_Gun_C|GetKilledEnemies _output_get) 0.08) (LocalVariables|GetScaleStr)) (LocalVariables|GetDamage))))))