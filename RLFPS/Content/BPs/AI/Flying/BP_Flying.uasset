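; Flying enemy that hunts the player and fires BP_GruntShot projectiles, with a chance of charge shots.
; BeginPlay scales stats using the player's gun, randomizes height and attack range, then runs BT_Flying.
; Tick drives FlierAnim and feeds ceiling/floor traces and player position to the blackboard.
; Damage triggers hit flashes and splatter decals; zero health, polled in Tick, grants gun EXP, updates GM_Sym's spawn count and may drop healing.
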(event Custom|On%20Colide%20Event
  (params (EventName :type Name) (EmitterTime :type Float%20%28single-precision%29) (ParticleTime :type Integer) (Location :type Vector) (Velocity :type Vector) (Direction :type Vector) (Normal :type Vector) (BoneName :type Name) (PhysMat :type Physical%20Material%20Object%20Reference))
  (bind _returnvalue (Rendering|Material|CreateDynamicMaterialInstance "/Game/Art/FX/BloodSplatter/m_Splatter_Decal.m_Splatter_Decal" "None" "None" :!class /Script/Engine.KismetMaterialLibrary))
  (Rendering|Material|SetScalarParameterValue _returnvalue "Frame" (Math|Conversions|ToFloat(Integer) (Math|Random|RandomInteger 11)) :!class /Script/Engine.MaterialInstanceDynamic)
  (Rendering|Decal|SpawnDecalatLocation _returnvalue (Math|Conversions|ToVector(Float) (Math|Random|RandomFloatinRange 25.0 1e+02)) Location (Math|Conversions|RotationFromXVector Normal) 2e+01))

(event Custom|ApplyAcidDamage
  (Game|Damage|ApplyDamage self (Variables|Default|GetAcidDamage) 0 0))

(event Custom|FlyingShoot
  (params (TargetPos :type Vector) (DamageMult :type Float%20%28single-precision%29))
  (bind _returnvalue (Transformation|GetActorTransform))
  (bind _self self)
  (bind (_location _rotation _scale) (Math|Transform|BreakTransform _returnvalue))
  (bind _returnvalue_2 (Game|SpawnActorfromClass "/Game/BPs/AI/Grunt/BP_GruntShot.BP_GruntShot_C" (Math|Transform|MakeTransform (+ _location "0, 0,10.000000") _rotation _scale) "AlwaysSpawn" _self (* DamageMult (Variables|Default|GetRangedAttackDamage)) _self))
  (Class|Bullet|SetInitialDirection _returnvalue_2 (Math|Vector|Normalize (- TargetPos (Transformation|GetActorLocation))))
  (Class|Bullet|SetInitialSpeed _returnvalue_2 1.0)
  (Variables|/Game/BPs/AI/Grunt/BP_GruntShot.BP_GruntShot_C|SetAttacker _returnvalue_2 self))

(event Custom|OnTakeAnyDamage_Event_0
  (params (DamagedActor :type Actor%20Object%20Reference) (Damage :type Float%20%28single-precision%29) (DamageType :type Damage%20Type%20Object%20Reference) (InstigatedBy :type Controller%20Object%20Reference) (DamageCauser :type Actor%20Object%20Reference))
  (Variables|Default|SetHit true)
  (Utilities|FlowControl|Delay 1.1)
  (Variables|Default|SetHit false))

(event Game|Damage|EventAnyDamage
  (params (Damage :type Float%20%28single-precision%29) (DamageType :type Damage%20Type%20Object%20Reference) (InstigatedBy :type Controller%20Object%20Reference) (DamageCauser :type Actor%20Object%20Reference))
  (bind _mesh (Variables|Character|GetMesh))
  (bind _capsulecomponent (Variables|Default|GetCapsuleComponent))
  (bind _returnvalue (Transformation|GetWorldLocation _capsulecomponent))
  (bind _returnvalue_2 (Effects|SpawnEmitteratLocation "/Game/Art/FX/BloodSplatter/splatter_P.splatter_P" _returnvalue))
  (Niagara|SpawnSystematLocation "/Game/Art/FX/EnemyDeath/NE_EnemyDeath_System.NE_EnemyDeath_System" _returnvalue)
  (EventDispatchers|BindEventtoOnParticleCollide _returnvalue_2 (delegate Custom|On%20Colide%20Event))
  (Class|GruntCharacter|UpdateStatusWidget)
  (Rendering|Material|SetMaterial _mesh 0 "/Game/BPs/AI/M_EnemyHit.M_EnemyHit")
  (Utilities|FlowControl|Delay 0.05)
  (Rendering|Material|SetMaterial _mesh 0 "/Game/Art/Materials/DisitegrationEffect/M_EnenmyDesidigration_FlyingVersion.M_EnenmyDesidigration_FlyingVersion"))

(event EventBeginPlay
  (bind _self self)
  (bind _self_2 self)
  (bind _attackrangevariation (Variables|Default|GetAttackRangeVariation))
  (bind _healthcomponent (Variables|Default|GetHealthComponent))
  (bind _returnvalue (AI|GetBlackboard _self_2))
  (bind _returnvalue_2 (Transformation|GetActorLocation _self))
  (|CallParentFunction)
  (bind _asbp_fpsplayer (Utilities|Casting|CastToBP_FPSPlayer (Game|Player|GetPlayerPawn 0)))
  (bind _asbp_gun (Utilities|Casting|CastToBP_Gun (Variables|/Script/Engine.ChildActorComponent|GetChildActor (Variables|/Game/BPs/BP_FPSPlayer.BP_FPSPlayer_C|GetGun _asbp_fpsplayer))))
  (bind (_newhealth _newdamage) (CallFunction|UpdateStats 1.0 (Variables|/Script/RLFPS.HealthComponent|GetcurrentHealth _healthcomponent) (Variables|Default|GetRangedAttackDamage) _asbp_gun))
  (Variables|/Script/RLFPS.HealthComponent|SetcurrentHealth _healthcomponent _newhealth)
  (Variables|Default|SetRangedAttackDamage _newdamage)
  (Variables|Default|SetDoesChargeShot (<= (Math|Random|RandomIntegerinRange 0 100) (Variables|Default|GetChanceForChargeShot)))
  (Variables|/Script/Engine.CharacterMovementComponent|SetGravityScale (Variables|/Script/Engine.Character|GetCharacterMovement _self) 0.0)
  (Transformation|SetActorLocation _self (Math|Vector|MakeVector (.x _returnvalue_2) (.y _returnvalue_2) (Math|Random|RandomFloatinRange (Variables|Default|GetMinHeightAbovePlayer) (Variables|Default|GetMaxHeightAbovePlayer))) false true)
  (EventDispatchers|AssignOnTakeAnyDamage (delegate Custom|OnTakeAnyDamage_Event_0))
  (Class|SkeletalMeshComponent|SetAnimClass (Variables|Character|GetMesh) "/Game/Art/Meshes/Enemy/Flier/FlierAnim.FlierAnim_C")
  (AI|RunBehaviorTree (AI|GetAIController self) "/Game/BPs/AI/Flying/BT_Flying.BT_Flying")
  (AI|Components|Blackboard|SetValueasFloat _returnvalue (Utilities|String|StringToName "FlySpeed") (Variables|Default|GetFlySpeed))
  (AI|Components|Blackboard|SetValueasBool _returnvalue (Utilities|String|StringToName "DoesChargeShot") (Variables|Default|GetDoesChargeShot))
  (AI|Components|Blackboard|SetValueasFloat (AI|GetBlackboard self) (Utilities|String|StringToName "RangeToAttack") (+ (Variables|Default|GetBaseAttackRange) (Math|Random|RandomFloatinRange (* -1 _attackrangevariation) _attackrangevariation)))
  (bind _asbp_fpsplayer_2 (Utilities|Casting|CastToBP_FPSPlayer (Game|Player|GetPlayerPawn 0)))
  (AI|Components|Blackboard|SetValueasVector (AI|GetBlackboard self) (Utilities|Name|MakeLiteralName "TargetDestination") (Math|Vector|MakeVector (.X (Math|Vector|BreakVector (Transformation|GetActorLocation _asbp_fpsplayer_2))) (.Y (Math|Vector|BreakVector (Transformation|GetActorLocation _asbp_fpsplayer_2))) (+ (.Z (Math|Vector|BreakVector (Transformation|GetActorLocation _asbp_fpsplayer_2))) 15.0)))
  (AI|Components|Blackboard|SetValueasFloat (AI|GetBlackboard self) (Utilities|Name|MakeLiteralName "DistanceFromPlayer") (Transformation|GetDistanceTo (Game|Player|GetPlayerPawn 0)))
  (if (<= (Variables|/Script/RLFPS.HealthComponent|GetcurrentHealth (Variables|Default|GetHealthComponent)) 0.0)
    (bind _asbp_fpsplayer_3 (Utilities|Casting|CastToBP_FPSPlayer (Game|Player|GetPlayerPawn 0)))
    (bind _asbp_gun_2 (Utilities|Casting|CastToBP_Gun (Variables|/Script/Engine.ChildActorComponent|GetChildActor (Variables|/Game/BPs/BP_FPSPlayer.BP_FPSPlayer_C|GetGun _asbp_fpsplayer_3))))
    (Class|Gun|GainEXP _asbp_gun_2 2)
    (bind _asgm_sym (Utilities|Casting|CastToGM_Sym (Game|GetGameMode)))
    (Variables|/Script/RLFPS.SymbioticGameMode|SetenemiesLeftToSpawn _asgm_sym (+ (Variables|/Script/RLFPS.SymbioticGameMode|GetenemiesLeftToSpawn _asgm_sym) 1))
    (Class|GruntCharacter|OnDeath)
    (CallFunction|PlayDeathSound)
    (if (<= (Math|Random|RandomInteger 100) (Variables|Default|GetPercentHealthDrop))
      (Game|SpawnActorfromClass "/Game/Art/FX/HealingShot/BP_HealingBeam.BP_HealingBeam_C" (Math|Conversions|ToTransform(Vector) (Transformation|GetActorLocation)) "Undefined" 0 0))
    (Actor|DestroyActor)))

(event EventTick
  (params (DeltaSeconds :type Float%20%28single-precision%29))
  (bind _returnvalue (Game|Player|GetPlayerPawn 0))
  (bind _returnvalue_2 (Game|Player|GetPlayerPawn 0))
  (bind _self self)
  (bind _self_2 self)
  (bind _maxheightaboveplayer (Variables|Default|GetMaxHeightAbovePlayer))
  (bind _minheightaboveplayer (Variables|Default|GetMinHeightAbovePlayer))
  (bind _returnvalue_3 (Transformation|GetActorLocation _self))
  (bind _returnvalue_4 (Transformation|GetActorLocation _returnvalue))
  (bind _returnvalue_5 (Transformation|GetActorLocation _returnvalue_2))
  (bind _returnvalue_6 (Transformation|GetActorLocation _self_2))
  (bind _z (Math|Vector|BreakVector _returnvalue_4))
  (bind _z_2 (Math|Vector|BreakVector _returnvalue_5))
  (bind _returnvalue_7 (+ _minheightaboveplayer _z))
  (bind _returnvalue_8 (+ _maxheightaboveplayer _z_2))
  (bind _asflier_anim (Utilities|Casting|CastToFlierAnim (Components|SkeletalMesh|GetAnimInstance (Variables|Character|GetMesh)))
    (:then
      (Variables|/Game/Art/Meshes/Enemy/Flier/FlierAnim.FlierAnim_C|SetHit _asflier_anim (Variables|Default|GetHit))
      (Variables|/Game/Art/Meshes/Enemy/Flier/FlierAnim.FlierAnim_C|SetMoving _asflier_anim (Math|Vector|NotEqual(Vector) (Transformation|GetVelocity) "0, 0, 0" 0.01)))
    (:CastFailed
      _))
  (bind (_outhit _returnvalue_9) (Collision|LineTraceByChannel (+ _returnvalue_3 "0, 0,5.000000") (+ _returnvalue_3 (Math|Vector|MakeVector 0.0 0.0 (Variables|Default|GetMaxHeightAbovePlayer))) "TraceTypeQuery2" false 0 "None" true "(R=1.000000,G=0.000000,B=0.000000,A=0.000000)" "(R=0.000000,G=1.000000,B=0.000000,A=0.000000)" 0.0))
  (if _returnvalue_9
    (AI|Components|Blackboard|SetValueasFloat (AI|GetBlackboard self) (Utilities|String|StringToName "CeilingDist") (Math|Float|Min(Float) (.Distance (Collision|BreakHitResult _outhit)) _returnvalue_8))
    (else
      (AI|Components|Blackboard|SetValueasFloat (AI|GetBlackboard self) (Utilities|String|StringToName "CeilingDist") _returnvalue_8)))
  (bind (_outhit_2 _returnvalue_10) (Collision|LineTraceByChannel (+ _returnvalue_6 "0, 0,-5.000000") (+ _returnvalue_6 (Math|Vector|MakeVector 0.0 0.0 (* (Variables|Default|GetMinHeightAbovePlayer) -1.0))) "TraceTypeQuery2" false 0 "None" true "(R=1.000000,G=0.000000,B=0.000000,A=0.000000)" "(R=0.000000,G=1.000000,B=0.000000,A=0.000000)" 0.0))
  (if _returnvalue_10
    (AI|Components|Blackboard|SetValueasFloat (AI|GetBlackboard self) (Utilities|String|StringToName "FloorDist") (Math|Float|Max(Float) (.Distance (Collision|BreakHitResult _outhit_2)) _returnvalue_7))
    (else
      (AI|Components|Blackboard|SetValueasFloat (AI|GetBlackboard self) (Utilities|String|StringToName "FloorDist") _returnvalue_7)))
  (bind _asbp_fpsplayer (Utilities|Casting|CastToBP_FPSPlayer (Game|Player|GetPlayerPawn 0)))
  (AI|Components|Blackboard|SetValueasVector (AI|GetBlackboard self) (Utilities|Name|MakeLiteralName "TargetDestination") (Math|Vector|MakeVector (.X (Math|Vector|BreakVector (Transformation|GetActorLocation _asbp_fpsplayer))) (.Y (Math|Vector|BreakVector (Transformation|GetActorLocation _asbp_fpsplayer))) (+ (.Z (Math|Vector|BreakVector (Transformation|GetActorLocation _asbp_fpsplayer))) 15.0)))
  (AI|Components|Blackboard|SetValueasFloat (AI|GetBlackboard self) (Utilities|Name|MakeLiteralName "DistanceFromPlayer") (Transformation|GetDistanceTo (Game|Player|GetPlayerPawn 0)))
  (if (<= (Variables|/Script/RLFPS.HealthComponent|GetcurrentHealth (Variables|Default|GetHealthComponent)) 0.0)
    (bind _asbp_fpsplayer_2 (Utilities|Casting|CastToBP_FPSPlayer (Game|Player|GetPlayerPawn 0)))
    (bind _asbp_gun (Utilities|Casting|CastToBP_Gun (Variables|/Script/Engine.ChildActorComponent|GetChildActor (Variables|/Game/BPs/BP_FPSPlayer.BP_FPSPlayer_C|GetGun _asbp_fpsplayer_2))))
    (Class|Gun|GainEXP _asbp_gun 2)
    (bind _asgm_sym (Utilities|Casting|CastToGM_Sym (Game|GetGameMode)))
    (Variables|/Script/RLFPS.SymbioticGameMode|SetenemiesLeftToSpawn _asgm_sym (+ (Variables|/Script/RLFPS.SymbioticGameMode|GetenemiesLeftToSpawn _asgm_sym) 1))
    (Class|GruntCharacter|OnDeath)
    (CallFunction|PlayDeathSound)
    (if (<= (Math|Random|RandomInteger 100) (Variables|Default|GetPercentHealthDrop))
      (Game|SpawnActorfromClass "/Game/Art/FX/HealingShot/BP_HealingBeam.BP_HealingBeam_C" (Math|Conversions|ToTransform(Vector) (Transformation|GetActorLocation)) "Undefined" 0 0))
    (Actor|DestroyActor)))

(fn ConstructionScript)

(fn PlayDeathSound
  (bind _returnvalue (Math|Random|RandomInteger 2))
  (switch int _returnvalue
    (:0
      (Audio|PlaySoundatLocation "/Game/Audio/AlienSFX/A_E1_Idle_Death.A_E1_Idle_Death" "0, 0, 0" "0, 0, 0" 1.0 1.0 0.0 0 0 0))
    (:1
      (Audio|PlaySoundatLocation "/Game/Audio/AlienSFX/A_E2_Agressive_Idle_Death.A_E2_Agressive_Idle_Death" "0, 0, 0" "0, 0, 0" 1.0 1.0 0.0 0 0 0))
    (:2
      (Audio|PlaySoundatLocation "/Game/Audio/AlienSFX/A_E4_Death.A_E4_Death" "0, 0, 0" "0, 0, 0" 1.0 1.0 0.0 0 0 0)))
  (Development|PrintString (Utilities|String|ToString(Integer) _returnvalue)))