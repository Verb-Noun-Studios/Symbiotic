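; Explosive projectile for the flying miniboss, configured through SetBaseStats and destroyed after ten seconds.
; Overlapping anything but its attacker spawns an explosion effect, then directly damages the player or shakes the camera otherwise.
; If the player is within the horizontal blast radius, it applies explosion damage and knockback scaled by 3D proximity.
; Only that in-radius branch destroys the effect and shot immediately on overlap.
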(event Custom|SetBaseStats
  (params (Attacker :type BP%20Flying%20Miniboss%20Object%20Reference) (ExplosionRadius :type Float%20%28single-precision%29) (ExplosionDamage :type Float%20%28single-precision%29) (KnockbackRate :type Vector) (ForceMult :type Float%20%28single-precision%29))
  (Variables|Default|SetAttacker Attacker)
  (Variables|Default|SetExplosionRadius ExplosionRadius)
  (Variables|Default|SetExplosionDamage ExplosionDamage)
  (Variables|Default|SetKnockbackRate KnockbackRate)
  (Variables|Default|SetForceMult ForceMult))

(event EventBeginPlay
  (Utilities|FlowControl|Delay 1e+01)
  (Actor|DestroyActor))

(event Collision|EventActorBeginOverlap
  (params (OtherActor :type Actor%20Object%20Reference))
  (bind _returnvalue (Transformation|GetActorLocation))
  (bind _returnvalue_2 (Transformation|GetActorLocation))
  (bind _returnvalue_3 (Game|Player|GetPlayerPawn 0))
  (bind _returnvalue_4 (Transformation|GetActorLocation _returnvalue_3))
  (bind (_x _y) (Math|Vector|BreakVector _returnvalue_2))
  (bind (_x_2 _y_2) (Math|Vector|BreakVector _returnvalue_4))
  (if (!= OtherActor (Variables|Default|GetAttacker))
    (bind _returnvalue_5 (Niagara|SpawnSystematLocation "/Game/Art/FX/CrawlerExplosion/Explosion_V2/NE_ExplosionCentre_System.NE_ExplosionCentre_System" (Transformation|GetActorLocation self) "0, 0, 0" "0.600000,0.600000,0.600000" false true "AutoRelease"))
    (bind _asbp_fpsplayer (Utilities|Casting|CastToBP_FPSPlayer OtherActor)
      (:then
        (Game|Damage|ApplyDamage _asbp_fpsplayer (Variables|Default|GetDamage) 0 (Variables|Default|GetAttacker)))
      (:CastFailed
        (Class|MatineeCameraShake|StartMatineeCameraShake (Game|GetPlayerCameraManager 0) "/Game/BPs/CameraShake/BossFightCamShake.BossFightCamShake_C" 0.07 "CameraLocal" "0, 0, 0")))
    (if (<= (Math|Float|Absolute(Float) (Math|Vector|Distance(Vector) (Math|Vector|MakeVector _x_2 _y_2 0.0) (Math|Vector|MakeVector _x _y 0.0))) (Variables|Default|GetExplosionRadius))
      ;[1 1 1] Player moved and takes damage
      (bind _asbp_fpsplayer_2 (Utilities|Casting|CastToBP_FPSPlayer _returnvalue_3))
      (Class|FragPlayer|SetVelocity _asbp_fpsplayer_2 (+ (Transformation|GetVelocity _asbp_fpsplayer_2) (* (* (* (Math|Vector|GetUnitDirection(Vector) _returnvalue (Transformation|GetActorLocation _asbp_fpsplayer_2)) (Variables|Default|GetKnockbackRate)) (- (Variables|Default|GetExplosionRadius) (Math|Float|Absolute(Float) (Math|Vector|Distance(Vector) (Transformation|GetActorLocation _asbp_fpsplayer_2) _returnvalue)))) (Variables|Default|GetForceMult))))
      (Game|Damage|ApplyDamage _asbp_fpsplayer_2 (Variables|Default|GetExplosionDamage) 0 (Variables|Default|GetAttacker))
      (Components|DestroyComponent _returnvalue_5)
      (Actor|DestroyActor))))

(fn ConstructionScript)