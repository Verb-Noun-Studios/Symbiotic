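; Flying miniboss enemy that hovers in a height band relative to the player and fires explosive charge shots.
; BeginPlay scales stats from the player's gun and easy mode, then runs BT_FlyingMiniboss.
; Tick traces up and down to feed ceiling, floor and player target to the blackboard, and on zero health grants gun EXP, updates the spawn count and destroys itself.
; Damage triggers blood decals, a material flash and a hit animation.
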(event Custom|On%20Colide%20Event
  (params (EventName :type Name) (EmitterTime :type Float%20%28single-precision%29) (ParticleTime :type Integer) (Location :type Vector) (Velocity :type Vector) (Direction :type Vector) (Normal :type Vector) (BoneName :type Name) (PhysMat :type Physical%20Material%20Object%20Reference))
  (bind _returnvalue (Rendering|Material|CreateDynamicMaterialInstance "/Game/Art/FX/BloodSplatter/m_Splatter_Decal.m_Splatter_Decal" "None" "None" :!class /Script/Engine.KismetMaterialLibrary))
  (Rendering|Material|SetScalarParameterValue _returnvalue "Frame" (Math|Conversions|ToFloat(Integer) (Math|Random|RandomInteger 11)) :!class /Script/Engine.MaterialInstanceDynamic)
  (Rendering|Decal|SpawnDecalatLocation _returnvalue (Math|Conversions|ToVector(Float) (Math|Random|RandomFloatinRange 25.0 1e+02)) Location (Math|Conversions|RotationFromXVector Normal) 2e+01))

(event Custom|ApplyAcidDamage
  (Game|Damage|ApplyDamage self (Variables|Default|GetAcidDamage) 0 0))

(event Custom|FlyingShoot
  (params (Target%20Position :type Vector) (DamageMult :type Float%20%28single-precision%29))
  (bind _returnvalue (Transformation|GetActorTransform))
  (bind _self self)
  (bind (_location _rotation _scale) (Math|Transform|BreakTransform _returnvalue))
  (bind _returnvalue_2 (Game|SpawnActorfromClass "/Game/BPs/AI/Flying/FlyingMiniboss/BP_FlyingMinibossShot.BP_FlyingMinibossShot_C" (Math|Transform|MakeTransform (+ _location "0.000000, 0,-200.000000") _rotation _scale) "AlwaysSpawn" _self (* DamageMult (Variables|Default|GetRangedAttackDamage)) _self))
  (Default|SetBaseStats _returnvalue_2 self (Variables|Default|GetExplosionRadius) (Variables|Default|GetExplosionDamage) (Variables|Default|GetKnockbackRate) (Variables|Default|GetForceMultiplier))
  (Class|Bullet|SetInitialDirection _returnvalue_2 (Math|Vector|Normalize (- Target%20Position (Transformation|GetActorLocation))))
  (Class|Bullet|SetInitialSpeed _returnvalue_2 (Variables|Default|GetShotSpeed)))

(event Custom|OnTakeAnyDamage_Event_0
  (params (DamagedActor :type Actor%20Object%20Reference) (Damage :type Float%20%28single-precision%29) (DamageType :type Damage%20Type%20Object%20Reference) (InstigatedBy :type Controller%20Object%20Reference) (DamageCauser :type Actor%20Object%20Reference))
  (Variables|Default|SetHit true)
  (Utilities|FlowControl|Delay 1.1)
  (Variables|Default|SetHit false))

(event Game|Damage|EventAnyDamage
  (params (Damage :type Float%20%28single-precision%29) (DamageType :type Damage%20Type%20Object%20Reference) (InstigatedBy :type Controller%20Object%20Reference) (DamageCauser :type Actor%20Object%20Reference))
  (bind _mesh (Variables|Character|GetMesh))
  (bind _capsulecomponent (Variables|Default|GetCapsuleComponent))
  (bind _returnvalue (Transformation|GetWorldLocation _capsulecomponent))
  (bind _returnvalue_2 (Effects|SpawnEmitteratLocation "/Game/Art/FX/BloodSplatter/splatter_P.splatter_P" _returnvalue))
  (Niagara|SpawnSystematLocation "/Game/Art/FX/EnemyDeath/NE_EnemyDeath_System.NE_EnemyDeath_System" _returnvalue)
  (EventDispatchers|BindEventtoOnParticleCollide _returnvalue_2 (delegate Custom|On%20Colide%20Event))
  (Class|GruntCharacter|UpdateStatusWidget)
  (Rendering|Material|SetMaterial _mesh 0 "/Game/BPs/AI/M_EnemyHit.M_EnemyHit")
  (Utilities|FlowControl|Delay 0.05)
  (Rendering|Material|SetMaterial _mesh 0 "/Game/Art/Materials/Enemies/M_Flier_base.M_Flier_Base"))

(event EventBeginPlay
  (bind _self self)
  (bind _self_2 self)
  (bind _maxheightaboveplayer (Variables|Default|GetMaxHeightAbovePlayer))
  (bind _attackrangevariation (Variables|Default|GetAttackRangeVariation))
  (bind _healthcomponent (Variables|Default|GetHealthComponent))
  (bind _healthcomponent_2 (Variables|Default|GetHealthComponent))
  (bind _returnvalue (Transformation|GetActorLocation _self))
  (bind _returnvalue_2 (AI|GetBlackboard _self_2))
  (|CallParentFunction)
  (bind _asbp_fpsplayer (Utilities|Casting|CastToBP_FPSPlayer (Game|Player|GetPlayerPawn 0)))
  (bind _asbp_gun (Utilities|Casting|CastToBP_Gun (Variables|/Script/Engine.ChildActorComponent|GetChildActor (Variables|/Game/BPs/BP_FPSPlayer.BP_FPSPlayer_C|GetGun _asbp_fpsplayer))))
  (bind (_newhealth _newdamage) (CallFunction|UpdateStats 1.0 (Variables|/Script/RLFPS.HealthComponent|GetcurrentHealth _healthcomponent_2) (Variables|Default|GetRangedAttackDamage) _asbp_gun))
  (Variables|/Script/RLFPS.HealthComponent|SetcurrentHealth _healthcomponent_2 _newhealth)
  (Variables|Default|SetRangedAttackDamage _newdamage)
  ;[1 1 1] Easy Mode Changes
  (bind _aswbp_settings_controller (Utilities|Casting|CastToWBP_SettingsController (Game|GetGameInstance)))
  (if (Variables|/Game/Widgets/3D_Menu/WBP_SettingsController.WBP_SettingsController_C|GetEasyMode _aswbp_settings_controller)
    (Development|PrintString "On" true true "(R=0.000000,G=1.000000,B=0.157874,A=1.000000)")
    (Variables|/Script/RLFPS.HealthComponent|SetcurrentHealth _healthcomponent (* (Variables|/Script/RLFPS.HealthComponent|GetcurrentHealth _healthcomponent) (Variables|Default|GeteasyModeMultiplier)))
    (Variables|Default|SetRangedAttackDamage (* (Variables|Default|GetRangedAttackDamage) (Variables|Default|GeteasyModeMultiplier))))
  (Variables|/Script/Engine.CharacterMovementComponent|SetGravityScale (Variables|/Script/Engine.Character|GetCharacterMovement _self) 0.0)
  (Transformation|SetActorLocation _self (Math|Vector|MakeVector (.x _returnvalue) (.y _returnvalue) (+ (.Z (Math|Vector|BreakVector (Transformation|GetActorLocation (Game|Player|GetPlayerPawn 0)))) (Math|Random|RandomFloatinRange (* _maxheightaboveplayer 0.8) _maxheightaboveplayer))) false true)
  (EventDispatchers|AssignOnTakeAnyDamage (delegate Custom|OnTakeAnyDamage_Event_0))
  (Class|SkeletalMeshComponent|SetAnimClass (Variables|Character|GetMesh) "/Game/Art/Meshes/Enemy/Flier/FlierAnim.FlierAnim_C")
  (AI|RunBehaviorTree (AI|GetAIController self) "/Game/BPs/AI/Flying/FlyingMiniboss/BT_FlyingMiniboss.BT_FlyingMiniboss")
  (AI|Components|Blackboard|SetValueasFloat _returnvalue_2 (Utilities|String|StringToName "FlySpeed") (Variables|Default|GetFlySpeed))
  (AI|Components|Blackboard|SetValueasBool _returnvalue_2 (Utilities|String|StringToName "DoesChargeShot") true)
  (AI|Components|Blackboard|SetValueasFloat (AI|GetBlackboard self) (Utilities|String|StringToName "RangeToAttack") (+ (Variables|Default|GetBaseAttackRange) (Math|Random|RandomFloatinRange (* -1 _attackrangevariation) _attackrangevariation)))
  (bind _asbp_fpsplayer_2 (Utilities|Casting|CastToBP_FPSPlayer (Game|Player|GetPlayerPawn 0)))
  (AI|Components|Blackboard|SetValueasVector (AI|GetBlackboard self) (Utilities|Name|MakeLiteralName "TargetDestination") (Math|Vector|MakeVector (.X (Math|Vector|BreakVector (Transformation|GetActorLocation _asbp_fpsplayer_2))) (.Y (Math|Vector|BreakVector (Transformation|GetActorLocation _asbp_fpsplayer_2))) (+ (.Z (Math|Vector|BreakVector (Transformation|GetActorLocation _asbp_fpsplayer_2))) 15.0)))
  (AI|Components|Blackboard|SetValueasFloat (AI|GetBlackboard self) (Utilities|Name|MakeLiteralName "DistanceFromPlayer") (Transformation|GetDistanceTo (Game|Player|GetPlayerPawn 0)))
  (if (<= (Variables|/Script/RLFPS.HealthComponent|GetcurrentHealth (Variables|Default|GetHealthComponent)) 0.0)
    (bind _asbp_fpsplayer_3 (Utilities|Casting|CastToBP_FPSPlayer (Game|Player|GetPlayerPawn 0)))
    (bind _asbp_gun_2 (Utilities|Casting|CastToBP_Gun (Variables|/Script/Engine.ChildActorComponent|GetChildActor (Variables|/Game/BPs/BP_FPSPlayer.BP_FPSPlayer_C|GetGun _asbp_fpsplayer_3))))
    (Class|Gun|GainEXP _asbp_gun_2 2)
    (bind _asgm_sym (Utilities|Casting|CastToGM_Sym (Game|GetGameMode)))
    (Variables|/Script/RLFPS.SymbioticGameMode|SetenemiesLeftToSpawn _asgm_sym (+ (Variables|/Script/RLFPS.SymbioticGameMode|GetenemiesLeftToSpawn _asgm_sym) 1))
    (Class|GruntCharacter|OnDeath)
    (CallFunction|PlayDeathSound)
    (Actor|DestroyActor)))

(event EventTick
  (params (DeltaSeconds :type Float%20%28single-precision%29))
  (bind _returnvalue (Game|Player|GetPlayerPawn 0))
  (bind _returnvalue_2 (Game|Player|GetPlayerPawn 0))
  (bind _self self)
  (bind _self_2 self)
  (bind _maxheightaboveplayer (Variables|Default|GetMaxHeightAbovePlayer))
  (bind _minheightaboveplayer (Variables|Default|GetMinHeightAbovePlayer))
  (bind _returnvalue_3 (Transformation|GetActorLocation _self))
  (bind _returnvalue_4 (Transformation|GetActorLocation _returnvalue))
  (bind _returnvalue_5 (Transformation|GetActorLocation _returnvalue_2))
  (bind _returnvalue_6 (Transformation|GetActorLocation _self_2))
  (bind _z (Math|Vector|BreakVector _returnvalue_4))
  (bind _z_2 (Math|Vector|BreakVector _returnvalue_5))
  (bind _returnvalue_7 (+ _minheightaboveplayer _z))
  (bind _returnvalue_8 (+ _maxheightaboveplayer _z_2))
  (bind _asflier_anim (Utilities|Casting|CastToFlierAnim (Components|SkeletalMesh|GetAnimInstance (Variables|Character|GetMesh))))
  (Variables|/Game/Art/Meshes/Enemy/Flier/FlierAnim.FlierAnim_C|SetHit _asflier_anim (Variables|Default|GetHit))
  (bind (_outhit _returnvalue_9) (Collision|LineTraceByChannel (+ _returnvalue_3 "0, 0,5.000000") (+ _returnvalue_3 (Math|Vector|MakeVector 0.0 0.0 (Variables|Default|GetMaxHeightAbovePlayer))) "TraceTypeQuery2" false 0 "None" true "(R=1.000000,G=0.000000,B=0.000000,A=0.000000)" "(R=0.000000,G=1.000000,B=0.000000,A=0.000000)" 0.0))
  (if _returnvalue_9
    (AI|Components|Blackboard|SetValueasFloat (AI|GetBlackboard self) (Utilities|String|StringToName "CeilingDist") (+ (Math|Float|Min(Float) (.Distance (Collision|BreakHitResult _outhit)) _returnvalue_8) _z_2))
    (else
      (AI|Components|Blackboard|SetValueasFloat (AI|GetBlackboard self) (Utilities|String|StringToName "CeilingDist") _returnvalue_8)))
  (bind (_outhit_2 _returnvalue_10) (Collision|LineTraceByChannel (+ _returnvalue_6 "0, 0,-5.000000") (+ _returnvalue_6 (Math|Vector|MakeVector 0.0 0.0 (* (Variables|Default|GetMinHeightAbovePlayer) -1.0))) "TraceTypeQuery2" false 0 "None" true "(R=1.000000,G=0.000000,B=0.000000,A=0.000000)" "(R=0.000000,G=1.000000,B=0.000000,A=0.000000)" 0.0))
  (if _returnvalue_10
    (AI|Components|Blackboard|SetValueasFloat (AI|GetBlackboard self) (Utilities|String|StringToName "FloorDist") (+ (Math|Float|Max(Float) (.Distance (Collision|BreakHitResult _outhit_2)) _returnvalue_7) _z))
    (else
      (AI|Components|Blackboard|SetValueasFloat (AI|GetBlackboard self) (Utilities|String|StringToName "FloorDist") _returnvalue_7)))
  (bind _asbp_fpsplayer (Utilities|Casting|CastToBP_FPSPlayer (Game|Player|GetPlayerPawn 0)))
  (AI|Components|Blackboard|SetValueasVector (AI|GetBlackboard self) (Utilities|Name|MakeLiteralName "TargetDestination") (Math|Vector|MakeVector (.X (Math|Vector|BreakVector (Transformation|GetActorLocation _asbp_fpsplayer))) (.Y (Math|Vector|BreakVector (Transformation|GetActorLocation _asbp_fpsplayer))) (+ (.Z (Math|Vector|BreakVector (Transformation|GetActorLocation _asbp_fpsplayer))) 15.0)))
  (AI|Components|Blackboard|SetValueasFloat (AI|GetBlackboard self) (Utilities|Name|MakeLiteralName "DistanceFromPlayer") (Transformation|GetDistanceTo (Game|Player|GetPlayerPawn 0)))
  (if (<= (Variables|/Script/RLFPS.HealthComponent|GetcurrentHealth (Variables|Default|GetHealthComponent)) 0.0)
    (bind _asbp_fpsplayer_2 (Utilities|Casting|CastToBP_FPSPlayer (Game|Player|GetPlayerPawn 0)))
    (bind _asbp_gun (Utilities|Casting|CastToBP_Gun (Variables|/Script/Engine.ChildActorComponent|GetChildActor (Variables|/Game/BPs/BP_FPSPlayer.BP_FPSPlayer_C|GetGun _asbp_fpsplayer_2))))
    (Class|Gun|GainEXP _asbp_gun 2)
    (bind _asgm_sym (Utilities|Casting|CastToGM_Sym (Game|GetGameMode)))
    (Variables|/Script/RLFPS.SymbioticGameMode|SetenemiesLeftToSpawn _asgm_sym (+ (Variables|/Script/RLFPS.SymbioticGameMode|GetenemiesLeftToSpawn _asgm_sym) 1))
    (Class|GruntCharacter|OnDeath)
    (CallFunction|PlayDeathSound)
    (Actor|DestroyActor)))

(fn ConstructionScript)

(fn PlayDeathSound
  (Audio|PlaySoundatLocation "/Game/Audio/EnemyAudio/Flier/Flier_Death.Flier_Death" (Transformation|GetActorLocation self) "0, 0, 0" 1.0 1.0 0.0 0 0 0))