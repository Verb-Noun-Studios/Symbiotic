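; BP_BossShot is a boss projectile actor that damages the player on overlap.
; On overlap with BP_FPSPlayer it applies its Damage value and destroys itself.
; Other actors stop it only if their root component carries the BulletBlocking tag, which destroys the shot without dealing damage.
; A timer started on BeginPlay destroys any shot that hits neither.
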(event EventBeginPlay
  (Utilities|FlowControl|Delay 1e+01)
  (Actor|DestroyActor))

(event EventTick
  (params (DeltaSeconds :type Float%20%28single-precision%29)))

(event Collision|EventActorBeginOverlap
  (params (OtherActor :type Actor%20Object%20Reference))
  (bind _asbp_fpsplayer (Utilities|Casting|CastToBP_FPSPlayer OtherActor)
    (:then
      (Game|Damage|ApplyDamage _asbp_fpsplayer (Variables|Default|GetDamage) 0 self)
      (Actor|DestroyActor :!label _label))
    (:CastFailed
      (if (Components|ComponentHasTag (Variables|/Script/Engine.Actor|GetRootComponent OtherActor) "BulletBlocking")
        (goto _label)))))

(fn ConstructionScript)