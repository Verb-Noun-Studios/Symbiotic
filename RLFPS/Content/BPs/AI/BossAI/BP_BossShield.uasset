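; BP_BossShield is a boss AI shield actor built around a Wall component that rises by scaling vertically.
; While the Growing flag is set, Tick increases the Wall's world Z scale by GrowSpeed times delta time until it reaches its height limit.
; The file only reads the Growing flag and contains no logic to set it, shrink the wall or handle hits.
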(event EventBeginPlay)

(event Collision|EventActorBeginOverlap
  (params (OtherActor :type Actor%20Object%20Reference)))

(event EventTick
  (params (DeltaSeconds :type Float%20%28single-precision%29))
  (bind _wall (Variables|Default|GetWall))
  (bind _returnvalue (Transformation|GetWorldScale _wall))
  (if (and (Variables|Default|GetGrowing) (< (.z _returnvalue) 2.0))
    (Transformation|SetWorldScale3D (Variables|Default|GetWall) (Math|Vector|MakeVector (.x _returnvalue) (.y _returnvalue) (+ (.z _returnvalue) (* DeltaSeconds (Variables|Default|GetGrowSpeed)))))))

(fn ConstructionScript)