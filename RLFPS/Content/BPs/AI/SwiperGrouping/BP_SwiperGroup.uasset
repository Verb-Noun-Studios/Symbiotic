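; BP_SwiperGroup is an actor representing a group of Swiper AI units, tracking its members and a size-dependent radius.
; AddUnit stores each unit in a map by UnitID and stamps it with the GroupID, while RemoveUnit deletes dead units' entries.
; CurrentRadius starts at BaseRadius on construction, then every Tick recomputes it as base times scale times member count.
; SetGroupPathTarget is an empty stub.
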(event EventBeginPlay)

(event Collision|EventActorBeginOverlap
  (params (OtherActor :type Actor%20Object%20Reference)))

(event EventTick
  (params (DeltaSeconds :type Float%20%28single-precision%29))
  (Variables|Default|SetCurrentRadius (* (Variables|Default|GetBaseRadius) (* (Variables|Default|GetRadiusScale) (Math|Conversions|ToFloat(Integer) (Utilities|Map|Length (Variables|Default|GetUnitsInGroup)))))))

(fn ConstructionScript
  (Variables|Default|SetCurrentRadius (Variables|Default|GetBaseRadius)))

(fn AddUnit
  (params (NewUnit :type BP%20Grunt%20Object%20Reference))
  (Utilities|Map|Add (Variables|Default|GetUnitsInGroup) (Variables|/Game/BPs/AI/Grunt/BP_Grunt.BP_Grunt_C|GetUnitID NewUnit) NewUnit)
  (Variables|/Game/BPs/AI/Grunt/BP_Grunt.BP_Grunt_C|SetGroupID NewUnit (Variables|Default|GetGroupID)))

(fn RemoveUnit
  (params (DeadUnit :type Integer))
  (Utilities|Map|Remove (Variables|Default|GetUnitsInGroup) DeadUnit))

(fn SetGroupPathTarget)