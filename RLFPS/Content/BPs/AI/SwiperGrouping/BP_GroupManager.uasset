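; Manager that tracks Swiper AI units and organizes them into groups that merge and attack the player.
; At a set interval on Tick, it has ungrouped Swipers seek nearby units and, when several groups exist, tells large groups to attack and others to seek the closest group.
; ID-keyed maps track membership as units and groups are created, joined or combined.
; Group destruction is deferred through a pending-delete list that Cleanup processes.
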(event EventBeginPlay)

(event Collision|EventActorBeginOverlap
  (params (OtherActor :type Actor%20Object%20Reference)))

(event EventTick
  (params (DeltaSeconds :type Float%20%28single-precision%29))
  (bind _swipers (Variables|Default|GetSwipers))
  (bind _grouplessunits (Variables|Default|GetGrouplessUnits))
  (bind _groups (Variables|Default|GetGroups))
  (bind _output_get (Variables|Default|SetTimer (+ (Variables|Default|GetTimer) DeltaSeconds)))
  ;[1 1 1] If there are no groups but at least 2 swipers
  (if (> _output_get (Variables|Default|GetUpdateInterval))
    (Variables|Default|SetTimer 0.0)
    (if (== (Utilities|Map|Length (Variables|Default|GetGroups)) 0)
      (if (>= (Utilities|Array|Length _swipers) 2)
        (for _array_element _swipers
          (if (Utilities|IsValid _array_element)
            (Default|FindClosestUnit _array_element _swipers)
            (CallFunction|Cleanup))))
      (else
        ;[1 1 1] If there are groups but solo swipers
        (if (!= (Utilities|Map|Length _grouplessunits) 0)
          (bind _values (Utilities|Map|Values _grouplessunits))
          (for _array_element_2 _values
            (if (Utilities|IsValid _array_element_2)
              (Default|FindClosestUnit _array_element_2 (Variables|Default|GetSwipers))
              (if (>= (Utilities|Map|Length _groups) 2)
                (bind _values_2 (Utilities|Map|Values _groups))
                (for _array_element_3 _values_2
                  (Utilities|IsValid _array_element_3
                    (:Is%20Valid
                      (if (Variables|/Game/BPs/AI/SwiperGrouping/BP_SwiperGroup.BP_SwiperGroup_C|GetIsLargeGroup _array_element_3)
                        (Default|AttackPlayer _array_element_3)
                        (else
                          (Default|FindClosestGroup _array_element_3 _groups)))
                      (CallFunction|Cleanup)))))))
          (else
            (if (>= (Utilities|Map|Length _groups) 2)
              (bind _values_3 (Utilities|Map|Values _groups))
              (for _array_element_4 _values_3
                (Utilities|IsValid _array_element_4
                  (:Is%20Valid
                    (if (Variables|/Game/BPs/AI/SwiperGrouping/BP_SwiperGroup.BP_SwiperGroup_C|GetIsLargeGroup _array_element_4)
                      (Default|AttackPlayer _array_element_4)
                      (else
                        (Default|FindClosestGroup _array_element_4 _groups)))
                    (CallFunction|Cleanup)))))))))
    (else
      (CallFunction|Cleanup))))

(fn ConstructionScript)

(fn CreateGroup
  (params (Unit1 :type BP%20Grunt%20Object%20Reference) (Unit2 :type BP%20Grunt%20Object%20Reference))
  (bind _unitid (Variables|/Game/BPs/AI/Grunt/BP_Grunt.BP_Grunt_C|GetUnitID Unit1))
  (bind _nextgroupid (Variables|Default|GetNextGroupID))
  (bind _unitid_2 (Variables|/Game/BPs/AI/Grunt/BP_Grunt.BP_Grunt_C|GetUnitID Unit2))
  (bind _grouplessunits (Variables|Default|GetGrouplessUnits))
  (bind _grouplessunits_2 (Variables|Default|GetGrouplessUnits))
  (if (and (Utilities|Map|Contains _grouplessunits _unitid) (Utilities|Map|Contains _grouplessunits _unitid_2))
    (bind _returnvalue (Game|SpawnActorfromClass "/Game/BPs/AI/SwiperGrouping/BP_SwiperGroup.BP_SwiperGroup_C" (Transformation|GetActorTransform Unit1) "Undefined" Unit1 0))
    (bind _output_get (Variables|/Game/BPs/AI/SwiperGrouping/BP_SwiperGroup.BP_SwiperGroup_C|SetGroupID _returnvalue _nextgroupid))
    (Math|Integer|IncrementInt _nextgroupid
      (:%20%20
        (Default|AddUnit _returnvalue Unit1)
        (Default|AddUnit _returnvalue Unit2)
        (Utilities|Map|Add (Variables|Default|GetGroups) _output_get _returnvalue)
        (Utilities|Map|Remove _grouplessunits_2 _unitid)
        (Utilities|Map|Remove _grouplessunits_2 _unitid_2)))))

(fn DestroyGroup
  (params (DestroyID :type Integer))
  (Utilities|Array|Add (Variables|Default|GetToBeDeleted) DestroyID))

(fn AddSwiper
  (params (NewUnit :type BP%20Grunt%20Object%20Reference))
  (bind _nextunitid (Variables|Default|GetNextUnitID))
  (bind _output_get (Variables|/Game/BPs/AI/Grunt/BP_Grunt.BP_Grunt_C|SetUnitID NewUnit _nextunitid))
  (Utilities|Array|AddUnique (Variables|Default|GetSwipers) NewUnit)
  (Utilities|Map|Add (Variables|Default|GetGrouplessUnits) _nextunitid NewUnit)
  (Math|Integer|IncrementInt _nextunitid
    (:%20%20
      (Development|PrintString "Swiper Added")
      (Development|PrintString (Utilities|String|ToString(Integer) _output_get)))))

(fn RemoveSwiper
  (params (DeadUnit :type BP%20Grunt%20Object%20Reference) (UnitsGroupID :type Integer))
  (Utilities|Array|RemoveItem (Variables|Default|GetSwipers) DeadUnit)
  (if (!= UnitsGroupID -1)
    (Default|RemoveUnit (.Value (Utilities|Map|Find (Variables|Default|GetGroups) UnitsGroupID)) (Variables|/Game/BPs/AI/Grunt/BP_Grunt.BP_Grunt_C|GetUnitID DeadUnit))))

(fn AddtoGroup
  (params (GroupToAdd :type Integer) (UnitToAdd :type BP%20Grunt%20Object%20Reference))
  (bind _unitid (Variables|/Game/BPs/AI/Grunt/BP_Grunt.BP_Grunt_C|GetUnitID UnitToAdd))
  (if (Utilities|Map|Contains (Variables|Default|GetGrouplessUnits) _unitid)
    (Variables|/Game/BPs/AI/Grunt/BP_Grunt.BP_Grunt_C|SetGroupID UnitToAdd GroupToAdd)
    (Default|AddUnit (.Value (Utilities|Map|Find (Variables|Default|GetGroups) GroupToAdd)) UnitToAdd)
    (Utilities|Map|Remove (Variables|Default|GetGrouplessUnits) _unitid)))

(fn RemovefromGroup
  (params (gID :type Integer) (uID :type Integer))
  (Default|RemoveUnit (.Value (Utilities|Map|Find (Variables|Default|GetGroups) gID)) uID))

(fn CalculateGroupPath)

(fn MakeLargeGroup
  (params (ID :type Integer))
  (bind _returnvalue (Utilities|Array|AddUnique (Variables|Default|GetBigGroups) ID))
  (Variables|/Game/BPs/AI/SwiperGrouping/BP_SwiperGroup.BP_SwiperGroup_C|SetIsLargeGroup (.Value (Utilities|Map|Find (Variables|Default|GetGroups) _returnvalue)) true))

(fn CombineGroups
  (params (ID1 :type Integer) (ID2 :type Integer))
  (bind _groups (Variables|Default|GetGroups))
  (if (not (Utilities|Array|ContainsItem (Variables|Default|GetToBeDeleted) ID1))
    (bind _values (Utilities|Map|Values (Variables|/Game/BPs/AI/SwiperGrouping/BP_SwiperGroup.BP_SwiperGroup_C|GetUnitsInGroup (.Value (Utilities|Map|Find _groups ID2)))))
    (for _array_element _values
      (if (Utilities|IsValid _array_element)
        (Utilities|Map|Add (Variables|/Game/BPs/AI/SwiperGrouping/BP_SwiperGroup.BP_SwiperGroup_C|GetUnitsInGroup (.Value (Utilities|Map|Find _groups ID1))) (Variables|/Game/BPs/AI/Grunt/BP_Grunt.BP_Grunt_C|GetUnitID _array_element) _array_element)
        (Variables|/Game/BPs/AI/Grunt/BP_Grunt.BP_Grunt_C|SetGroupID _array_element ID1)))
    (Utilities|Array|Add (Variables|Default|GetToBeDeleted) ID2)))

(fn Cleanup
  (bind _groups (Variables|Default|GetGroups))
  (for _array_element (Variables|Default|GetToBeDeleted)
    (Utilities|IsValid (.Value (Utilities|Map|Find _groups _array_element))
      (:Is%20Valid
        (bind _output_get (LocalVariables|SetTempGroupRef (.Value (Utilities|Map|Find _groups _array_element))))
        (Utilities|Map|Remove _groups _array_element)
        (Actor|DestroyActor _output_get)
        (Utilities|Array|RemoveItem (Variables|Default|GetBigGroups) _array_element))))
  (Utilities|Array|Clear (Variables|Default|GetToBeDeleted)))