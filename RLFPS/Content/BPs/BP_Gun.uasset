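; BP_Gun is the player's gun actor, handling weapon feedback and also triggering the boss sequence.
; On Tick, reloading plays a DoOnce-guarded timeline that rolls the mesh; otherwise it updates level percentage and starts the GM_Sym boss sequence once total EXP reaches the threshold.
; Callable events play muzzle flash with gunshot audio, play a first-upgrade sound and store handedness, while ToggleHat toggles the hat's visibility.
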(event Custom|UpdateControls
  (params (LeftHanded :type Boolean))
  (Variables|Default|SetLeftHanded LeftHanded))

(event Custom|Spread)

(event EventBeginPlay
  (bind _returnvalue (Actor|GetActorOfClass "/Game/BPs/BP_FPSPlayer.BP_FPSPlayer_C"))
  (Variables|Default|Setcamera (Variables|/Script/RLFPS.FragPlayer|GetFirstPersonCameraComponent _returnvalue))
  (bind _asgm_sym (Utilities|Casting|CastToGM_Sym (Game|GetGameMode)))
  (Variables|Default|SetGameMode _asgm_sym))

(event Collision|EventActorBeginOverlap
  (params (OtherActor :type Actor%20Object%20Reference)))

(event EventTick
  (params (DeltaSeconds :type Float%20%28single-precision%29))
  (bind _gamemode (Variables|Default|GetGameMode))
  (if (Variables|Default|Getreloading)
    (Utilities|FlowControl|DoOnce false :!label _label
      (:Completed
        (bind _newtrack_0 (Timeline|Timeline_0 PlayFromStart)
          (:Update
            (Transformation|SetRelativeRotation (Variables|Default|GetStaticMesh) (Math|Rotator|MakeRotator _newtrack_0 0.0 -9e+01) false false))
          (:Finished
            (goto _label Reset)))))
    (else
      (bind _asbp_fpsplayer (Utilities|Casting|CastToBP_FPSPlayer (Game|Player|GetPlayerPawn 0)))
      (Class|Gun|GetLevelPercentage)
      (if (and (>= (Variables|Default|GettotalEXP) (Variables|/Script/RLFPS.SymbioticGameMode|GetEXPRequiredForBoss _gamemode)) (not (Variables|/Script/RLFPS.SymbioticGameMode|GetbossSequenceStarted _gamemode)))
        (Class|SymbioticGameMode|StartBossSequence (Variables|Default|GetGameMode))))))

(event EventOnFirstUpgrade
  (Audio|PlaySound2D "/Game/Audio/FergusonVoiceLines/A_FirstUpgrade.A_FirstUpgrade" 1.0 1.0 0.0 0 0))

(event EventPlayMuzzleFlashFX
  (bind _returnvalue (Transformation|GetActorLocation))
  (bind _returnvalue_2 (Transformation|GetActorRotation))
  (bind _muzzlelocation (Variables|Default|GetMuzzleLocation))
  (bind _returnvalue_3 (Math|Vector|GetForwardVector _returnvalue_2))
  (bind _returnvalue_4 (* _returnvalue_3 _muzzlelocation))
  (bind _returnvalue_5 (+ _returnvalue_4 _returnvalue))
  (Niagara|SpawnSystemAttached "/Game/Art/FX/MuzzleFlash/NS_MuzzleFlash.NS_MuzzleFlash" (Variables|Transformation|GetRootComponent) "point" _returnvalue_5 (Transformation|GetActorRotation) "KeepWorldPosition" false)
  (Components|Activation|Activate (Variables|Default|GetNiagara) true)
  (Audio|PlaySoundatLocation "/Game/Audio/GunSFX/A_Gunshot.A_Gunshot" _returnvalue_5 "0, 0, 0" 0.2 1.0 0.0 0 0 0))

(fn ConstructionScript)

(fn ToggleHat
  (Rendering|ToggleVisibility (Variables|Default|GetBP_Hat) false))