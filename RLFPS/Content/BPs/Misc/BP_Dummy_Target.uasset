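; BP_Dummy_Target is a target dummy that rewards the player's gun with experience when its health runs out.
; Tick polls the Health component, and when current health equals exactly zero it casts to the player pawn and its Gun child actor.
; It then grants that BP_Gun a fixed amount of EXP and destroys itself, which only happens if both casts succeed.
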(event EventBeginPlay)

(event Collision|EventActorBeginOverlap
  (params (OtherActor :type Actor%20Object%20Reference)))

(event EventTick
  (params (DeltaSeconds :type Float%20%28single-precision%29))
  (if (== (Variables|/Script/RLFPS.HealthComponent|GetcurrentHealth (Variables|Default|GetHealth)) 0.0)
    (bind _asfps_player (Utilities|Casting|CastToBP_FPS_Player (Game|Player|GetPlayerPawn 0)))
    (bind _asgun_bp (Utilities|Casting|CastToBP_Gun (Variables|/Script/Engine.ChildActorComponent|GetChildActor (Variables|/Game/BPs/Player/BP_FPS_Player.BP_FPS_Player_C|GetGun _asfps_player))))
    (Class|Gun|GainEXP _asgun_bp 2)
    (Actor|DestroyActor)))

(fn ConstructionScript)