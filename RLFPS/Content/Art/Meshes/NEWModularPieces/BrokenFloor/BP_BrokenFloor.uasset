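; BP_BrokenFloor is a broken floor piece that can launch two of its fragments as debris when play begins.
; If AddImpulse is set, BeginPlay applies a randomized, mass-independent impulse to two shard components, with a strong upward bias and random horizontal spread.
; After a short delay, it destroys both fragments, leaving the rest of the actor in place.
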(event EventBeginPlay
  (bind _returnvalue (Math|Random|RandomUnitVector))
  (bind _returnvalue_2 (Math|Random|RandomFloatinRange 5e+02 1e+03))
  (bind _floor_brocken_polysurface4 (Variables|Default|Getfloor_brocken_polySurface4))
  (bind _returnvalue_3 (* _returnvalue 2.5e+02))
  (bind (_x _y) (Math|Vector|BreakVector _returnvalue_3))
  (if (Variables|Default|GetaddImpulse)
    (Physics|AddImpulse (Variables|Default|Getfloor_brocken_shard1) (Math|Vector|MakeVector _x _y _returnvalue_2) "None" true)
    (Physics|AddImpulse _floor_brocken_polysurface4 (Math|Vector|MakeVector _x _y _returnvalue_2) "None" true)
    (Utilities|FlowControl|Delay 5.0)
    (Components|DestroyComponent _floor_brocken_polysurface4)))

(event Collision|EventActorBeginOverlap
  (params (OtherActor :type Actor%20Object%20Reference)))

(event EventTick
  (params (DeltaSeconds :type Float%20%28single-precision%29)))

(fn ConstructionScript)