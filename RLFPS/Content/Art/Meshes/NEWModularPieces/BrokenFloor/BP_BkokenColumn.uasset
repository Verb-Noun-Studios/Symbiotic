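; BP_BkokenColumn is a broken column actor whose five mesh pieces burst apart when it begins play.
; Each piece gets a velocity-change impulse with random horizontal direction and a strong random upward push.
; After a five-second delay the piece components are destroyed, while the actor itself is not explicitly destroyed.
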(event EventBeginPlay
  (bind _returnvalue (Math|Random|RandomUnitVector))
  (bind _returnvalue_2 (* _returnvalue 2.5e+02))
  (bind (_x _y) (Math|Vector|BreakVector _returnvalue_2))
  (Physics|AddImpulse (Variables|Default|Getcolumn_broke_polySurface1) (Math|Vector|MakeVector _x _y (Math|Random|RandomFloatinRange 5e+02 1e+03)) "None" true)
  (Utilities|FlowControl|Delay 5.0)
  (Components|DestroyComponent (Variables|Default|Getcolumn_broke_polySurface5)))

(event Collision|EventActorBeginOverlap
  (params (OtherActor :type Actor%20Object%20Reference)))

(event EventTick
  (params (DeltaSeconds :type Float%20%28single-precision%29)))

(fn ConstructionScript)