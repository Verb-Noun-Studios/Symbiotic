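; Boss room elevator event controller that drops debris and can halt the moving walls.
; Tick runs through a latent Delay to fire DropDebris about every five seconds, printing a debug string.
; DropDebris spawns a BP_DebrisBroken at every BP_DebrisSpawner, with random scale per axis.
; StopElevator deactivates the Movement component on every BP_MovingWall but is not called within this Blueprint.
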(event EventTick
  (params (DeltaSeconds :type Float%20%28single-precision%29))
  (Utilities|FlowControl|Delay 5.0)
  (CallFunction|DropDebris))

(fn ConstructionScript)

(fn StopElevator
  (bind _outactors (Actor|GetAllActorsOfClass "/Game/Art/Meshes/LevelProps/BossRoom/BP_MovingWall.BP_MovingWall_C"))
  (for _array_element _outactors
    (Components|Activation|SetActive (Variables|/Game/Art/Meshes/LevelProps/BossRoom/BP_MovingWall.BP_MovingWall_C|Getmovement _array_element) false false)))

(fn DropDebris
  (bind _returnvalue (Math|Random|RandomFloatinRange 0.5 2.0))
  (Development|PrintString "Hello")
  (bind _outactors (Actor|GetAllActorsOfClass "/Game/Art/Meshes/LevelProps/BossRoom/BP_DebrisSpawner.BP_DebrisSpawner_C"))
  (for _array_element _outactors
    (bind _returnvalue_2 (Game|SpawnActorfromClass "/Game/Art/Meshes/LevelProps/BossRoom/BP_DebrisBroken.BP_DebrisBroken_C" (Transformation|GetActorTransform _array_element) "Undefined" 0 0))
    (Transformation|SetActorScale3D _returnvalue_2 (Math|Vector|MakeVector _returnvalue _returnvalue _returnvalue))))