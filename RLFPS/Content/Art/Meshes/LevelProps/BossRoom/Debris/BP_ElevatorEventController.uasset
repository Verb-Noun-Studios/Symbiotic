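; Event controller for the boss room elevator that drops debris and stops the moving walls.
; DropObjects spawns a debris actor at each BP_DebrisSpawner with a short stagger between spawns, then gives it a random rotation.
; StopElevator halts the elevator by deactivating the Movement component on every BP_MovingWall.
; The actor enables player input on BeginPlay so the B key can trigger the debris drop directly.
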(event Custom|DropObjects
  (bind _returnvalue (Math|Random|RandomFloatinRange 0.0 1.8e+02))
  (bind _outactors (Actor|GetAllActorsOfClass "/Game/Art/Meshes/LevelProps/BossRoom/Debris/BP_DebrisSpawner.BP_DebrisSpawner_C"))
  (bind _array_element (Utilities|ForEachLoopwithDelay _outactors 0.1)
    (:Loop%20Body
      (bind _returnvalue_2 (Game|SpawnActorfromClass "/Game/Art/Meshes/LevelProps/BossRoom/Debris/BP_DebrisFull.BP_DebrisFull_C" (Transformation|GetActorTransform _array_element) "Undefined" 0 0))
      (Transformation|SetActorRotation _returnvalue_2 (Math|Rotator|MakeRotator _returnvalue _returnvalue _returnvalue)))))

(event Custom|StopElevator
  (bind _outactors (Actor|GetAllActorsOfClass "/Game/Art/Meshes/LevelProps/BossRoom/BP_MovingWall.BP_MovingWall_C"))
  (for _array_element _outactors
    (Components|Activation|SetActive (Variables|/Game/Art/Meshes/LevelProps/BossRoom/BP_MovingWall.BP_MovingWall_C|Getmovement _array_element) false false)))

(event EventBeginPlay
  (Input|EnableInput (Game|GetPlayerController 0)))

(event Input|KeyboardEvents|B
  (params (Key :type Key%20Structure :default "None"))
  (:Pressed
    (CallFunction|DropObjects)))

(fn ConstructionScript)