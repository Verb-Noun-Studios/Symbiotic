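; BP_DebrisFull is an intact boss-room rock debris piece that shatters when its Rock3 component hits something.
; A hit on BP_FPSPlayer applies damage, while any other hit spawns the NE_ReloadBomb Niagara effect at the rock's location.
; Either way it destroys the rock component, leaving the actor itself alive, and spawns a randomly rotated BP_DebrisBroken using the rock's relative, not world, transform.
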(event OnComponentHit(rock3)
  (params (HitComponent :type Primitive%20Component%20Object%20Reference) (OtherActor :type Actor%20Object%20Reference) (OtherComp :type Primitive%20Component%20Object%20Reference) (NormalImpulse :type Vector :default "0, 0, 0") (Hit :type Hit%20Result%20Structure%20%28by%20ref%29))
  (bind _returnvalue (Math|Random|RandomFloatinRange 0.0 3.6e+02))
  (bind _rock3 (Variables|Default|Getrock3))
  (bind _asbp_fpsplayer (Utilities|Casting|CastToBP_FPSPlayer OtherActor)
    (:then
      (Game|Damage|ApplyDamage _asbp_fpsplayer 1e+01 0 0))
    (:CastFailed
      (Niagara|SpawnSystematLocation "/Game/Art/FX/Explosion/NE_ReloadBomb.NE_ReloadBomb" (Transformation|GetWorldLocation (Variables|Default|Getrock3)))))
  (bind _output_get (Variables|Default|SetrockTransform (Transformation|GetRelativeTransform _rock3)))
  (Components|DestroyComponent _rock3)
  (bind _returnvalue_2 (Game|SpawnActorfromClass "/Game/Art/Meshes/LevelProps/BossRoom/Debris/BP_DebrisBroken.BP_DebrisBroken_C" _output_get "Undefined" 0 0))
  (Transformation|SetActorRotation _returnvalue_2 (Math|Rotator|MakeRotator _returnvalue _returnvalue _returnvalue)))

(fn ConstructionScript)