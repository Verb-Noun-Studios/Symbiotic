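; BP_MovingWall is a boss room level prop that wraps its height back to a bottom point once it reaches a top limit.
; Each Tick compares the root's relative Z to TopTransform and, at or above it, sets Z to BotTransform's while feeding world X/Y into the relative location.
; The graph contains no upward movement, only this reset, plus an unconnected SetRelativeLocation node that never runs.
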(event Collision|EventActorBeginOverlap
  (params (OtherActor :type Actor%20Object%20Reference)))

(event EventTick
  (params (DeltaSeconds :type Float%20%28single-precision%29))
  (bind _defaultsceneroot (Variables|Default|GetDefaultSceneRoot))
  (bind _returnvalue (Transformation|GetWorldLocation _defaultsceneroot))
  (Variables|Default|SetCurrentTransform (.location (Transformation|GetRelativeTransform (Variables|Default|GetDefaultSceneRoot))))
  (if (>= (.z (Variables|Default|GetCurrentTransform)) (.z (Variables|Default|GetTopTransform)))
    (Transformation|SetRelativeLocation _defaultsceneroot (Math|Vector|MakeVector (.x _returnvalue) (.y _returnvalue) (.z (Variables|Default|GetBotTransform))) false false)))

(fn ConstructionScript)