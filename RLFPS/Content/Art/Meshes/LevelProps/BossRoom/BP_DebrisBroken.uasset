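; Boss room debris prop that bursts into three broken rock shards when it begins play.
; Each shard component gets a random velocity-change impulse with a strong upward bias, and the shards are destroyed after a short delay, leaving the actor itself in place.
; Any actor overlap prints a debug hit message and spawns a Niagara explosion at the other actor's location.
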(event EventBeginPlay
  (bind _returnvalue (Math|Random|RandomUnitVector))
  (bind _rock3_broken_shard1 (Variables|Default|Getrock3_broken_shard1))
  (bind _returnvalue_2 (* _returnvalue 2.5e+02))
  (bind (_x _y) (Math|Vector|BreakVector _returnvalue_2))
  (Physics|AddImpulse _rock3_broken_shard1 (Math|Vector|MakeVector _x _y (Math|Random|RandomFloatinRange 5e+02 1e+03)) "None" true)
  (Utilities|FlowControl|Delay 5.0)
  (Components|DestroyComponent _rock3_broken_shard1))

(event Collision|EventActorBeginOverlap
  (params (OtherActor :type Actor%20Object%20Reference))
  (Development|PrintString "HIT OBJECT")
  (Niagara|SpawnSystematLocation "/Game/Art/FX/CrawlerExplosion/Explosion_V2/NE_ExplosionCentre_System.NE_ExplosionCentre_System" (Transformation|GetActorLocation OtherActor)))

(fn ConstructionScript)