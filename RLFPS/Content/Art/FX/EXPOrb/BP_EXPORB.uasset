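; BP_EXPORB is an experience pickup that homes in on the player and grants EXP to their gun.
; Overlapping the Sphere sets FoundPlayer, after which Tick plays the Alpha timeline to lerp the actor toward the player's location.
; Overlapping PartCol stops the Niagara trail, hides the orb and awards a fixed EXP amount to the player's BP_Gun once.
; Tick then destroys the found, collected orb after a short delay.
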(event OnComponentBeginOverlap(Sphere)
  (params (OverlappedComponent :type Primitive%20Component%20Object%20Reference) (OtherActor :type Actor%20Object%20Reference) (OtherComp :type Primitive%20Component%20Object%20Reference) (OtherBodyIndex :type Integer) (bFromSweep :type Boolean) (SweepResult :type Hit%20Result%20Structure%20%28by%20ref%29))
  (Utilities|Casting|CastToBP_FPSPlayer OtherActor)
  (Development|PrintString "OOOOO")
  (Variables|Default|SetfoundPlayer true))

(event OnComponentBeginOverlap(partCol)
  (params (OverlappedComponent :type Primitive%20Component%20Object%20Reference) (OtherActor :type Actor%20Object%20Reference) (OtherComp :type Primitive%20Component%20Object%20Reference) (OtherBodyIndex :type Integer) (bFromSweep :type Boolean) (SweepResult :type Hit%20Result%20Structure%20%28by%20ref%29))
  (bind _ns_healingtrail_system (Variables|Default|GetNS_HealingTrail_System))
  (bind _asbp_fpsplayer (Utilities|Casting|CastToBP_FPSPlayer OtherActor))
  (if (not (Variables|Default|Getcolided))
    (Transformation|DetachFromComponent _ns_healingtrail_system "KeepRelative" "KeepRelative" "KeepRelative" true)
    (Components|Activation|Deactivate _ns_healingtrail_system)
    (Rendering|SetVisibility (Variables|Default|Getorb) false false)
    (bind _asbp_gun (Utilities|Casting|CastToBP_Gun (Variables|/Script/Engine.ChildActorComponent|GetChildActor (Variables|/Game/BPs/BP_FPSPlayer.BP_FPSPlayer_C|GetGun _asbp_fpsplayer))))
    (Class|Gun|GainEXP _asbp_gun 20)
    (Variables|Default|Setcolided true)))

(event EventTick
  (params (DeltaSeconds :type Float%20%28single-precision%29))
  (if (Variables|Default|GetfoundPlayer)
    (if (Variables|Default|Getcolided)
      (Utilities|FlowControl|Delay 3.0)
      (Actor|DestroyActor)
      (else
        (bind _returnvalue (Actor|GetActorOfClass "/Game/BPs/BP_FPSPlayer.BP_FPSPlayer_C"))
        (Variables|Default|SetPlayerPos (Transformation|GetActorLocation _returnvalue))
        (bind _alpha (Timeline|Alpha Play)
          (:Update
            (Transformation|SetActorLocation (Math|Vector|Lerp(Vector) (Transformation|GetWorldLocation (Variables|Default|GetSphere)) (Variables|Default|GetPlayerPos) _alpha) false false)))))))

(fn ConstructionScript)