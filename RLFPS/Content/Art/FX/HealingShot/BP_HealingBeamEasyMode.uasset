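; Easy-mode-only healing pickup that homes in on the player and restores health on contact.
; It destroys itself at BeginPlay unless the game instance's EasyMode flag is set.
; Overlapping the Sphere starts a Tick-driven timeline that lerps the actor toward the player.
; PartCol overlap heals once, detaches the Niagara trail, hides the plus and plays a sound, then Tick destroys it after a delay.
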(event OnComponentBeginOverlap(Sphere)
  (params (OverlappedComponent :type Primitive%20Component%20Object%20Reference) (OtherActor :type Actor%20Object%20Reference) (OtherComp :type Primitive%20Component%20Object%20Reference) (OtherBodyIndex :type Integer) (bFromSweep :type Boolean) (SweepResult :type Hit%20Result%20Structure%20%28by%20ref%29))
  (Utilities|Casting|CastToBP_FPSPlayer OtherActor)
  (Development|PrintString "OOOOO")
  (Variables|Default|SetfoundPlayer true))

(event OnComponentBeginOverlap(partCol)
  (params (OverlappedComponent :type Primitive%20Component%20Object%20Reference) (OtherActor :type Actor%20Object%20Reference) (OtherComp :type Primitive%20Component%20Object%20Reference) (OtherBodyIndex :type Integer) (bFromSweep :type Boolean) (SweepResult :type Hit%20Result%20Structure%20%28by%20ref%29))
  (bind _ns_healingtrail_system (Variables|Default|GetNS_HealingTrail_System))
  (bind _asbp_fpsplayer (Utilities|Casting|CastToBP_FPSPlayer OtherActor))
  (if (not (Variables|Default|Getcolided))
    (Transformation|DetachFromComponent _ns_healingtrail_system "KeepRelative" "KeepRelative" "KeepRelative" true)
    (Components|Activation|Deactivate _ns_healingtrail_system)
    (Rendering|SetVisibility (Variables|Default|Getplus) false false)
    (Class|HealthComponent|Heal (Variables|/Script/RLFPS.FragPlayer|GetHealthComponent _asbp_fpsplayer) 1e+01)
    (Variables|Default|Setcolided true)
    (Audio|PlaySoundatLocation "/Game/Audio/GunSFX/Upgrades_SFX-20220419T053714Z-001/Upgrades_SFX/Heal_Shots_Temp.Heal_Shots_Temp" "0, 0, 0" "0, 0, 0" 1.0 1.0 0.0 0 0 0)))

(event EventBeginPlay
  (bind _aswbp_settings_controller (Utilities|Casting|CastToWBP_SettingsController (Game|GetGameInstance)))
  (if (not (Variables|/Game/Widgets/3D_Menu/WBP_SettingsController.WBP_SettingsController_C|GetEasyMode _aswbp_settings_controller))
    (Actor|DestroyActor)))

(event EventTick
  (params (DeltaSeconds :type Float%20%28single-precision%29))
  (if (Variables|Default|GetfoundPlayer)
    (if (Variables|Default|Getcolided)
      (Utilities|FlowControl|Delay 3.0)
      (Actor|DestroyActor)
      (else
        (bind _returnvalue (Actor|GetActorOfClass "/Game/BPs/BP_FPSPlayer.BP_FPSPlayer_C"))
        (Variables|Default|SetPlayerPos (Transformation|GetActorLocation _returnvalue))
        (bind _alpha (Timeline|Alpha Play)
          (:Update
            (Transformation|SetActorLocation (Math|Vector|Lerp(Vector) (Transformation|GetWorldLocation (Variables|Default|GetSphere)) (Variables|Default|GetPlayerPos) _alpha) false false)))))))

(fn ConstructionScript)